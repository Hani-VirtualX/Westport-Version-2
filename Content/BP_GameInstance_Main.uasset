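; Main GameInstance for what appears to be a chapter-based VR experience, holding progress and mode state.
; CurrentChapterCompleted sets one of ten chapter completion flags based on ChapterNumber, while ResetAllVariable clears only some trackers and flags.
; Simple events toggle manual VR and snapping-ghost conditions.
; The per-chapter completion events are empty, and IsInSession and IsLoggedIn are stubs returning false.
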(event `self.ReceiveInit`
  ;[1 1 1] Init
  (`parent.ReceiveInit`))

(event `self.ReceiveShutdown`
  ;[1 1 1] Shutdown
  (`parent.ReceiveShutdown`))

(event `Start ManualVR`
  (set `self.ManualVR` true))

(event `Chapter 1 Completed`)

(event `Reset All Variable`
  (set `self.Chapter 1 Completed Tick` false)
  (set `self.Chapter 1 Tracker Current Integer` 0)
  (set `self.Chapter 3 Tracker Current Interger` 0)
  (set `self.Chapter 4 Tracker Current Interger` 0)
  (set `self.Restart Chapter Condition` false)
  (set `self.Next Step` false))

(event `Chapter 2 Completed`)

(event `Enable Snapping Ghost`
  ;[1 1 1] NOT SURE USING OR NOT
  (set `self.Snapping Ghost Condition` true))

(event `Chapter 3 Completed`)

(event `Disable Snapping Ghost`
  ;[1 1 1] NOT SURE USING OR NOT
  (set `self.Snapping Ghost Condition` false))

(event `Chapter 4 Completed`)

(event `Chapter 5 Completed`)

(event `Chapter 6 Completed`)

(event `Chapter 7 Completed`)

(event `Chapter 8 Completed`)

(event `Current Chapter Completed`
  (switch `int` (`self.Chapter Number`)
    (:`1`
      (set `self.Chapter 1 Completed Tick` true))
    (:`2`
      (set `self.Chapter 2 Completed Tick` true))
    (:`3`
      (set `self.Chapter 3 Completed Tick` true))
    (:`4`
      (set `self.Chapter 4 Completed Tick` true))
    (:`5`
      (set `self.Chapter 5 Completed Tick` true))
    (:`6`
      (set `self.Chapter 6 Completed Tick` true))
    (:`7`
      (set `self.Chapter 7 Completed Tick` true))
    (:`8`
      (set `self.Chapter 8 Completed Tick` true))
    (:`9`
      (set `self.Chapter 9 Completed Tick` true))
    (:`10`
      (set `self.Chapter 10 Completed Tick` true))))

(fn `IsInSession`
  (returns (InSession :type Boolean))
  (return false))

(fn `IsLoggedIn`
  (returns (LoggedIn :type Boolean))
  (return false))
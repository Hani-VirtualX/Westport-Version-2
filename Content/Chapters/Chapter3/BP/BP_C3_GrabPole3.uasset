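; BP_C3_GrabPole3 is a Chapter 3 VR grab pole that reports the first latch on it to the chapter game mode.
; Enable and disable events configure the latch, hand indicator and label widget through the VX latch-drag and label components.
; Latching sets IsGrabbing and calls Sub216 on GM_C3 through a DoOnce, re-armed by ResetPole3.
; BeginPlay caches pawn, right hook and GM_C3 references after a short delay.
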(event `self.ReceiveBeginPlay`
  (`KismetSystemLibrary.Delay` 0.2)
  (bind _returnvalue (`GameplayStatics.GetActorOfClass` "/Game/Azureal_Template/VXTemplate/0-Map/Setting/BP_Pawn_VR_VX.BP_Pawn_VR_VX_C"))
  (set `self.BP Pawn VR VX` _returnvalue)
  (bind _returnvalue_2 (`GameplayStatics.GetActorOfClass` "/Game/Chapters/Chapter2/Blueprint/BP_ClimbLadder/BP_RightHook.BP_RightHook_C"))
  (set `self.BP Right Hook` _returnvalue_2)
  (bind _returnvalue_3 (`GameplayStatics.GetActorOfClass` "/Game/Chapters/Chapter3/GM_C3.GM_C3_C"))
  (set `self.GM_C3` _returnvalue_3))

(event `Enable Latch Pole 3`
  (`/Game/Azureal_Template/VX_LatchDrag/VX_Latch_Drag.Set Latch` (`self.VX_Latch_Drag`) (`self.Cube`) (`self.BP_Hand_Indicator`) null true "NewEnumerator0" "NewEnumerator7" "NewEnumerator9")
  (`/Game/Azureal_Template/VX_Label/VX_Label.Set [ Label + ]` (`self.VX_Label`) (`self.Cube`) (`self.Widget`) true "NewEnumerator0" "NewEnumerator9" "NewEnumerator1" "NewEnumerator0"))

(event `self.VX_Latch_Drag.Latch_ActorGotLatched`
  (params (LatchingPawn :type "/Game/AFCore/Blueprints/Pawn/BP_Pawn_Base Object Reference") (LatchingActor :type "Actor Object Reference"))
  (`/Engine/EditorBlueprintResources/StandardMacros.DoOnce` false :!label _label
    (:`Completed`
      (set `self.IsGrabbing` true)
      (`/Game/Chapters/Chapter3/GM_C3.Sub 2-1-6` (`self.GM_C3`)))))

(event `Reset Pole 3`
  (goto _label :!via `Reset`))

(event `Disable Latch Pole 3`
  (`/Game/Azureal_Template/VX_LatchDrag/VX_Latch_Drag.Set Latch` (`self.VX_Latch_Drag`) (`self.Cube`) (`self.BP_Hand_Indicator`) null false "NewEnumerator4" "NewEnumerator9" "NewEnumerator9")
  (`/Game/Azureal_Template/VX_Label/VX_Label.Set [ Label + ]` (`self.VX_Label`) (`self.Cube`) (`self.Widget`) false "NewEnumerator4" "NewEnumerator6" "NewEnumerator4" "NewEnumerator4"))

(event `self.VX_Latch_Drag.Latch_ActorLatchReleased`
  (params (ReleasingPawn :type "/Game/AFCore/Blueprints/Pawn/BP_Pawn_Base Object Reference") (ReleasingActor :type "Actor Object Reference")))

(fn `UserConstructionScript`)
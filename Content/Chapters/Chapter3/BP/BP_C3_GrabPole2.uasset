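; BP_C3_GrabPole2 is a Chapter 3 grab pole Blueprint with no grab logic in its graphs.
; On BeginPlay it waits briefly, then finds the GM_C3 actor by class and caches the reference.
; Similar lookups for the left and right hooks, BP_C3_GrabPole3 and GM_C2 are left disconnected and never run.
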(event `self.ReceiveBeginPlay`
  (`KismetSystemLibrary.Delay` 0.2)
  (bind _returnvalue (`GameplayStatics.GetActorOfClass` "/Game/Chapters/Chapter3/GM_C3.GM_C3_C"))
  (set `self.GM_C3` _returnvalue))

(fn `UserConstructionScript`)
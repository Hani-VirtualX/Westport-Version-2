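; VR right safety-lanyard hook for Chapter 3, which the player grabs and attaches to attach point 2.
; After a short delay on BeginPlay it caches scene references, hides the hook and tethers its cable to the player pawn's lanyard.
; Events toggle hook visibility and configure the VXGrab component, using the attach point's hook as ghost target.
; The first completed attach calls Sub213 on GM_C3 to advance the chapter.
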(event `self.ReceiveBeginPlay`
  (`KismetSystemLibrary.Delay` 0.2)
  (`|ExecutionSequence`
    (:`then_0`
      (bind _returnvalue (`GameplayStatics.GetActorOfClass` "/Game/Chapters/Chapter3/BP/BP_C3_Hook_AttachPoint_2.BP_C3_Hook_AttachPoint_2_C"))
      (set `self.BP_C3_HookAttachPoint2` _returnvalue)
      (bind _returnvalue_2 (`GameplayStatics.GetActorOfClass` "/Game/Chapters/Chapter2/Blueprint/BP_ClimbLadder/BP_GrabPole2.BP_GrabPole2_C"))
      (set `self.BP Grab Pole 2` _returnvalue_2)
      (bind _returnvalue_3 (`GameplayStatics.GetActorOfClass` "/Game/AFCore/Blueprints/Pawn/VR/BP_Pawn_VR.BP_Pawn_VR_C"))
      (set `self.BP Pawn VR` _returnvalue_3)
      (bind _returnvalue_4 (`GameplayStatics.GetActorOfClass` "/Game/Chapters/Chapter3/GM_C3.GM_C3_C"))
      (set `self.GM_C3` _returnvalue_4)
      (`self.Set Hidden Hook`))
    (:`then_1`
      (`CableComponent.SetAttachEndTo` (`self.Cable`) (`GameplayStatics.GetPlayerPawn` 0) "WP_SafetyLanyard" "None"))))

(event `Enable Grab Attach`
  (`/Game/Azureal_Template/VX_Grab/VX_Grab.Set Grab Attach` (`self.VX_Grab`) (`self.Hook`) (`self.BP_Grab_Indicator`) (`self.Widget`) (`/Game/Chapters/Chapter3/BP/BP_C3_Hook_AttachPoint_2.Hook` (`self.BP_C3_HookAttachPoint2`)) "AttachWidget" true "NewEnumerator0" "NewEnumerator7" "NewEnumerator1" "NewEnumerator0")
  (set `/Game/AFCore/Blueprints/Pawn/VR/BP_Pawn_VR.Force Release` false (`self.BP Pawn VR`)))

(event `Disable Grab Attach`
  (`/Game/Azureal_Template/VX_Grab/VX_Grab.Set Grab Attach` (`self.VX_Grab`) (`self.Hook`) (`self.BP_Grab_Indicator`) (`self.Widget`) (`/Game/Chapters/Chapter3/BP/BP_C3_Hook_AttachPoint_2.Hook` (`self.BP_C3_HookAttachPoint2`)) "AttachWidget" false "NewEnumerator4" "NewEnumerator6" "NewEnumerator4" "NewEnumerator4")
  (set `/Game/AFCore/Blueprints/Pawn/VR/BP_Pawn_VR.Force Release` false (`self.BP Pawn VR`)))

(event `Set Hidden Hook`
  (`SceneComponent.SetHiddenInGame` (`self.Hook`) true true))

(event `Set Visible Hook`
  (`SceneComponent.SetHiddenInGame` (`self.Hook`) false true))

(event `self.VX_Grab.Grab Object - Attached`
  (params (`Comp Connector Achor` :type "/Game/AFCore/Blueprints/Components/Snapping/Comp_Connector_Anchor Object Reference"))
  (`/Engine/EditorBlueprintResources/StandardMacros.DoOnce` false
    (:`Completed`
      (`/Game/Chapters/Chapter3/GM_C3.Sub 2-1-3` (`self.GM_C3`)))))

(fn `UserConstructionScript`)
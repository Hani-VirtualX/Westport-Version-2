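; Chapter 3 Step 1 actor that shows and hides the explanation widgets for sub-steps 1-1-1 and 1-1-2.
; Paired Visible and Hidden custom events each call SetExplain on VXExplain, passing the widget along with settings such as arrow, highlight and cable positions.
; BeginPlay waits briefly, then caches the GM_C3 actor, which is not otherwise used in this graph.
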(event `self.ReceiveBeginPlay`
  (`KismetSystemLibrary.Delay` 0.2)
  (bind _returnvalue (`GameplayStatics.GetActorOfClass` "/Game/Chapters/Chapter3/GM_C3.GM_C3_C"))
  (set `self.GM_C3` _returnvalue))

(event `Set 1-1-1 Explain Visible`
  (`/Game/Azureal_Template/VX_Explain/VX_Explain.Set [ Explain + ]` (`self.VX_Explain`) null (`self.1-1-1_Explain`) true "NewEnumerator8" "NewEnumerator8" "NewEnumerator0" "NewEnumerator4" "NewEnumerator4"))

(event `Set 1-1-1 Explain Hidden`
  (`/Game/Azureal_Template/VX_Explain/VX_Explain.Set [ Explain + ]` (`self.VX_Explain`) null (`self.1-1-1_Explain`) false "NewEnumerator8" "NewEnumerator6" "NewEnumerator4" "NewEnumerator4" "NewEnumerator4"))

(event `Set 1-1-2 Explain Visible`
  (`/Game/Azureal_Template/VX_Explain/VX_Explain.Set [ Explain + ]` (`self.VX_Explain`) null (`self.1-1-2_Explain`) true "NewEnumerator9" "NewEnumerator8" "NewEnumerator0" "NewEnumerator4" "NewEnumerator4"))

(event `Set 1-1-2 Explain Hidden`
  (`/Game/Azureal_Template/VX_Explain/VX_Explain.Set [ Explain + ]` (`self.VX_Explain`) null (`self.1-1-2_Explain`) false "NewEnumerator9" "NewEnumerator6" "NewEnumerator4" "NewEnumerator4" "NewEnumerator4"))

(fn `UserConstructionScript`)
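; VR grab pole for Chapter 3 that toggles its latch, hand indicator, tag and label through enable and disable events.
; On BeginPlay it caches the VR pawn, both hooks, the second pole and GM_C3 after a short delay.
; The first latch triggers GM_C3's Sub212 step through a DoOnce that ResetPole1 re-arms.
; Latch release only checks the second pole without acting, and the climb-ending and hook-reset logic is disconnected.
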(event `self.ReceiveBeginPlay`
  (`KismetSystemLibrary.Delay` 0.2)
  (bind _returnvalue (`GameplayStatics.GetActorOfClass` "/Game/Azureal_Template/VXTemplate/0-Map/Setting/BP_Pawn_VR_VX.BP_Pawn_VR_VX_C"))
  (set `self.BP Pawn VR VX` _returnvalue)
  (bind _returnvalue_2 (`GameplayStatics.GetActorOfClass` "/Game/Chapters/Chapter3/BP/BP_C3_RightHook.BP_C3_RightHook_C"))
  (set `self.BP_C3_RightHook` _returnvalue_2)
  (bind _returnvalue_3 (`GameplayStatics.GetActorOfClass` "/Game/Chapters/Chapter3/BP/BP_C3_GrabPole2.BP_C3_GrabPole2_C"))
  (set `self.BP_C3_GrabPole2` _returnvalue_3)
  (bind _returnvalue_4 (`GameplayStatics.GetActorOfClass` "/Game/Chapters/Chapter3/GM_C3.GM_C3_C"))
  (set `self.GM_C3` _returnvalue_4)
  (bind _returnvalue_5 (`GameplayStatics.GetActorOfClass` "/Game/Chapters/Chapter3/BP/BP_C3_LeftHook.BP_C3_LeftHook_C"))
  (set `self.BP_C3_LeftHook` _returnvalue_5))

(event `Enable Latch Pole1`
  (bind _cube (`self.Cube`))
  (`/Game/Azureal_Template/VX_LatchDrag/VX_Latch_Drag.Set Latch` (`self.VX_Latch_Drag`) _cube (`self.BP_Hand_Indicator`) _cube true "NewEnumerator0" "NewEnumerator7" "NewEnumerator9")
  (set `/Game/AFCore/Blueprints/Pawn/VR/BP_Pawn_VR.Force Release` false (`self.BP Pawn VR VX`)))

(event `Enable Tag 2-1-2`
  (`/Game/Azureal_Template/VX_Label/VX_Label.Set [ Label + ]` (`self.VX_Label`) (`self.Cube`) (`self.tag`) true "NewEnumerator0" "NewEnumerator9" "NewEnumerator1" "NewEnumerator0"))

(event `Disable Latch Pole 1`
  (bind _cube (`self.Cube`))
  (`/Game/Azureal_Template/VX_LatchDrag/VX_Latch_Drag.Set Latch` (`self.VX_Latch_Drag`) _cube (`self.BP_Hand_Indicator`) _cube false "NewEnumerator4" "NewEnumerator6" "NewEnumerator9"))

(event `Disable Tag 2-1-2`
  (`/Game/Azureal_Template/VX_Label/VX_Label.Set [ Label + ]` (`self.VX_Label`) (`self.Cube`) (`self.tag`) false "NewEnumerator4" "NewEnumerator6" "NewEnumerator4" "NewEnumerator4"))

(event `self.VX_Latch_Drag.Latch_ActorGotLatched`
  (params (LatchingPawn :type "/Game/AFCore/Blueprints/Pawn/BP_Pawn_Base Object Reference") (LatchingActor :type "Actor Object Reference"))
  (`/Engine/EditorBlueprintResources/StandardMacros.DoOnce` false :!label _label
    (:`Completed`
      (`/Game/Chapters/Chapter3/GM_C3.Sub 2-1-2` (`self.GM_C3`)))))

(event `Enable Label 2-1-1`
  (`/Game/Azureal_Template/VX_Label/VX_Label.Set [ Label ]` (`self.VX_Label`) null (`self.Label`) true "NewEnumerator6" "NewEnumerator4" "NewEnumerator4"))

(event `Disable Label 2-1-1`
  (`/Game/Azureal_Template/VX_Label/VX_Label.Set [ Label ]` (`self.VX_Label`) null (`self.Label`) false "NewEnumerator6" "NewEnumerator4" "NewEnumerator4"))

(event `Reset Pole 1`
  (goto _label :!via `Reset`))

(event `self.VX_Latch_Drag.Latch_ActorLatchReleased`
  (params (ReleasingPawn :type "/Game/AFCore/Blueprints/Pawn/BP_Pawn_Base Object Reference") (ReleasingActor :type "Actor Object Reference"))
  (if (`/Game/Chapters/Chapter3/BP/BP_C3_GrabPole2.IsGrabbing` (`self.BP_C3_GrabPole2`))
    _))

(fn `UserConstructionScript`)
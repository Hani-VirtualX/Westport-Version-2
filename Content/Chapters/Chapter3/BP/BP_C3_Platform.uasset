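; BP_C3_Platform is the Chapter 3 platform actor, providing a switchable floor and preset teleports for the player pawn.
; On BeginPlay, after a short delay, it caches the GM_C3 actor and the BP_Pawn_Base pawn.
; Custom events toggle the Floor's collision or pass that pawn to CompTeleport with hardcoded high or side locations and rotations.
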(event `self.ReceiveBeginPlay`
  (`KismetSystemLibrary.Delay` 0.2)
  (bind _returnvalue (`GameplayStatics.GetActorOfClass` "/Game/Chapters/Chapter3/GM_C3.GM_C3_C"))
  (set `self.GM_C3` _returnvalue)
  (bind _returnvalue_2 (`GameplayStatics.GetActorOfClass` "/Game/AFCore/Blueprints/Pawn/BP_Pawn_Base.BP_Pawn_Base_C"))
  (set `self.BP_Pawn_Base` _returnvalue_2))

(event `Enable Floor`
  (`PrimitiveComponent.SetCollisionEnabled` (`self.Floor`) "QueryAndPhysics"))

(event `Disable Floor`
  (`PrimitiveComponent.SetCollisionEnabled` (`self.Floor`) "NoCollision"))

(event `Teleport To High`
  (`/Game/AFCore/Blueprints/Components/Interaction/Comp_Teleport.TeleportToLocation` (`self.Comp_Teleport`) (`self.BP_Pawn_Base`) (-2700.0 4090.0 400.0) (struct :`Yaw` -90.0)))

(event `Teleport To Side`
  (`/Game/AFCore/Blueprints/Components/Interaction/Comp_Teleport.TeleportToLocation` (`self.Comp_Teleport`) (`self.BP_Pawn_Base`) (-2540.0 4133.0 60.0) (struct :`Yaw` -175.0)))

(fn `UserConstructionScript`)
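; Chapter 3 actor that animates a pair of boots lifting like legs and exposes events to show, hide and reset them.
; Per-boot timelines drive relative location from FirstUp or SecondUp vector tracks, gated by boolean flags that separate Play and Pause events toggle.
; The right boot's SecondUp branch is hardwired off.
; BeginPlay only runs a short delay, so nothing here starts the motion itself.
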(event `self.ReceiveBeginPlay`
  (`KismetSystemLibrary.Delay` 0.2))

(event `Left Leg Up`
  (bind (_direction _first_up _second_up) (`Timeline|Move Up Left Leg` :!label _label)
    (:`Update`
      (`|ExecutionSequence`
        (:`then_0`
          (if (`self.Left 1 Up`)
            (`SceneComponent.K2_SetRelativeLocation` (`self.Boots_Left`) (`KismetMathLibrary.MakeVector` (.x _first_up) 25.801355 (.z _first_up)) false false)))
        (:`then_1`
          (if (`self.Left 2 Up`)
            (`SceneComponent.K2_SetRelativeLocation` (`self.Boots_Left`) (`KismetMathLibrary.MakeVector` (.x _second_up) 25.801355 (.z _second_up)) false false)))))))

(event `Play Left 1 Up`
  (set `self.Left 1 Up` true))

(event `Left Leg Up 2`
  (goto _label :!via `PlayFromStart`))

(event `Pause Left 1 Up`
  (set `self.Left 1 Up` false))

(event `Play Left 2 Up`
  (set `self.Left 2 Up` true))

(event `Pause Left 2 Up`
  (set `self.Left 2 Up` false))

(event `Set Hidden Boots`
  (`SceneComponent.SetHiddenInGame` (`self.Boots_Right`) true false)
  (`SceneComponent.SetHiddenInGame` (`self.Boots_Left`) true false))

(event `Play Right 1 Up`
  (set `self.Right 1 Up` true))

(event `Pause Right 1 Up`
  (set `self.Right 1 Up` false))

(event `Reset Anim R`
  (`SceneComponent.K2_SetRelativeLocation` (`self.Boots_Right`) (0.0 0.0 0.929941) false false)
  (`self.Pause Right 1 Up`))

(event `Reset Anim L`
  (`SceneComponent.K2_SetRelativeLocation` (`self.Boots_Left`) (-0.401155 25.801355 0.929941) false false)
  (`self.Pause Left 1 Up`)
  (`self.Pause Left 2 Up`))

(event `Set Visible Boots`
  (`SceneComponent.SetHiddenInGame` (`self.Boots_Right`) false false)
  (`SceneComponent.SetHiddenInGame` (`self.Boots_Left`) false false))

(event `Right Leg Up`
  (bind (_direction _first_up _second_up) (`Timeline|Move Up Right Leg` :!label _label_2)
    (:`Update`
      (`|ExecutionSequence`
        (:`then_0`
          (if (`self.Right 1 Up`)
            (`SceneComponent.K2_SetRelativeLocation` (`self.Boots_Right`) (`KismetMathLibrary.MakeVector` (.x _first_up) 0.0 (.z _first_up)) false false)))
        (:`then_1`
          (if false
            (`SceneComponent.K2_SetRelativeLocation` (`self.Boots_Right`) (`KismetMathLibrary.MakeVector` (.x _second_up) 0.0 (.z _second_up)) false false)))))))

(event `Right Leg Up 2`
  (goto _label_2 :!via `PlayFromStart`))

(fn `UserConstructionScript`)
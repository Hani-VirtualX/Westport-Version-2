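; Chapter 3 game mode that scripts a two-step VR training procedure on an RTG crane, centred on a harnessed ladder climb.
; BeginPlay caches scene actors and the step widget, and RunStepsOrder plays timed narration before starting each step.
; Chained Sub events alternate left/right hook grabs and pole latches, raising the player and animating boots.
; Completed steps update progress; ResetEverything resets the climb with fall and danger feedback.
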(event `Step 1`
  ;[1 1 1] STEP 1
  (`/Game/Chapters/Chapter3/NewBP/BP_C3_RTGCrane.Set 1-1-1 Explain Visible` (`self.BP_C3_RTGCrane`))
  (`ManualVRPluginBPLibrary.Start`))

(event `Sub 1-1-1`
  ;[1 1 1] SUB 1
  (`/Game/Chapters/Chapter3/NewBP/BP_C3_RTGCrane.Set 1-1-1 Explain Hidden` (`self.BP_C3_RTGCrane`))
  ;[1 0.04231 0] Instructions
  (`TrainingStepPage.AdvanceProgress` (`self.WBP_Step_Page`))
  ;[0.01405 0 1] ManualVR
  (`ManualVRPluginBPLibrary.Update` "3" "1" "1" 1)
  ;[1 1 1] Pointers
  (`/Game/Chapters/Chapter3/BP_C3_CSM.Enable Pointer` (`self.BP_C3_CSM`))
  (`GameplayStatics.SpawnSound2D` "/Game/Chapters/Steps_Completed/1Comp.1Comp" 1.0 1.0 0.0 null))

(event `self.ReceiveBeginPlay`
  (`KismetSystemLibrary.Delay` 0.2)
  (`|ExecutionSequence`
    (:`then_0`
      (bind _returnvalue (`GameplayStatics.GetActorOfClass` "/Game/Chapters/Chapter3/BP_C3_CSM.BP_C3_CSM_C"))
      (set `self.BP_C3_CSM` _returnvalue)
      (`/Game/Chapters/Chapter3/BP_C3_CSM.Enable Pointer` (`self.BP_C3_CSM`)))
    (:`then_1`
      (bind _foundwidgets (`WidgetBlueprintLibrary.GetAllWidgetsOfClass` "/Azureal_CSM/WBP_StepPage.WBP_StepPage_C" false))
      (set `self.WBP_Step_Page` (`|GetArrayItem` _foundwidgets)))
    (:`then_2`
      (bind _returnvalue_2 (`GameplayStatics.GetActorOfClass` "/Game/Chapters/Chapter3/NewBP/BP_C3_RTGCrane.BP_C3_RTGCrane_C"))
      (set `self.BP_C3_RTGCrane` _returnvalue_2)
      (bind _returnvalue_3 (`GameplayStatics.GetActorOfClass` "/Game/Chapters/Chapter3/NewBP/BP_C3_LeftHook.BP_C3_LeftHook_C"))
      (set `self.BP_C3_LeftHook` _returnvalue_3)
      (bind _returnvalue_4 (`GameplayStatics.GetActorOfClass` "/Game/Chapters/Chapter3/NewBP/BP_C3_GrabPole1.BP_C3_GrabPole1_C"))
      (set `self.BP_C3_GrabPole1` _returnvalue_4)
      (bind _returnvalue_5 (`GameplayStatics.GetActorOfClass` "/Game/Chapters/Chapter3/NewBP/BP_C3_RightHook.BP_C3_RightHook_C"))
      (set `self.BP_C3_RightHook` _returnvalue_5)
      (bind _returnvalue_6 (`GameplayStatics.GetActorOfClass` "/AzurealXR/Core/BP_Azr_Pawn.BP_Azr_Pawn_C"))
      (set `self.BP_Azr_Pawn` _returnvalue_6)
      (bind _returnvalue_7 (`GameplayStatics.GetActorOfClass` "/Game/Chapters/Chapter3/NewBP/BP_C3_Boots_Anim.BP_C3_Boots_Anim_C"))
      (set `self.BP_C3_Boots_Anim` _returnvalue_7)
      (bind _returnvalue_8 (`GameplayStatics.GetActorOfClass` "/Game/Chapters/Chapter3/NewBP/BP_C3_GrabPole2.BP_C3_GrabPole2_C"))
      (set `self.BP_C3_GrabPole2` _returnvalue_8)
      (bind _returnvalue_9 (`GameplayStatics.GetActorOfClass` "/Game/Chapters/Chapter3/NewBP/BP_C3_GrabPole3.BP_C3_GrabPole3_C"))
      (set `self.BP_C3_GrabPole3` _returnvalue_9)
      (bind _returnvalue_10 (`GameplayStatics.GetActorOfClass` "/Game/Chapters/Chapter3/NewBP/BP_C3_GrabPole4.BP_C3_GrabPole4_C"))
      (set `self.BP_C3_GrabPole4` _returnvalue_10)
      (bind _returnvalue_11 (`GameplayStatics.GetActorOfClass` "/Game/Chapters/Chapter3/NewBP/BP_C3_GrabPole5.BP_C3_GrabPole5_C"))
      (set `self.BP_C3_GrabPole5` _returnvalue_11)
      (bind _returnvalue_12 (`GameplayStatics.GetActorOfClass` "/Game/Chapters/Chapter3/NewBP/BP_C3_GrabPole6.BP_C3_GrabPole6_C"))
      (set `self.BP_C3_GrabPole6` _returnvalue_12))
    (:`then_3`
      (`KismetSystemLibrary.Delay` 3.0))
    (:`then_4`
      (`KismetSystemLibrary.Delay` 1.0)
      (`/AzurealXR/Core/BP_Azr_Pawn.Turn On Harness` (`self.BP_Azr_Pawn`)))
    (:`then_6`
      (bind _asazr_game_instance (cast `/AzurealXR/Core/Azr_GameInstance` (`GameplayStatics.GetGameInstance`)))
      (set `/AzurealXR/Core/Azr_GameInstance.Chapter Number` 3 _asazr_game_instance))))

(event `StepSequencerInterface.RunStepsOrder`
  (bind _result (`/Engine/EditorBlueprintResources/StandardMacros.IncrementInt` (`self.Steps Interger`))
    (:`  `
      (switch `int` _result
        (:`1`
          (bind _returnvalue (`GameplayStatics.SpawnSound2D` "/Game/Chapters/Steps_Num/1.1" 1.0 1.0 0.0 null))
          (`KismetSystemLibrary.Delay` (`SoundBase.Duration` (`AudioComponent.Sound` _returnvalue)))
          (bind _returnvalue_2 (`GameplayStatics.SpawnSound2D` "/Game/Chapters/Chapter3/Audio/Wes_C3/Steps_Intro/C3_Step1.C3_Step1" 1.0 1.0 0.0 null))
          (`KismetSystemLibrary.Delay` (`SoundBase.Duration` (`AudioComponent.Sound` _returnvalue_2)))
          (`self.Step 1`))
        (:`2`
          (bind _returnvalue_3 (`GameplayStatics.SpawnSound2D` "/Game/Chapters/Steps_Num/2.2" 1.0 1.0 0.0 null))
          (`KismetSystemLibrary.Delay` (`SoundBase.Duration` (`AudioComponent.Sound` _returnvalue_3)))
          (bind _returnvalue_4 (`GameplayStatics.SpawnSound2D` "/Game/Chapters/Chapter3/Audio/Wes_C3/Steps_Intro/C3_Step2.C3_Step2" 1.0 1.0 0.0 null))
          (`KismetSystemLibrary.Delay` (`SoundBase.Duration` (`AudioComponent.Sound` _returnvalue_4)))
          (`self.Step 2`))))))

(event `Step 2`
  ;[1 1 1] STEP 2
  (`/Game/Chapters/Chapter3/NewBP/BP_C3_LeftHook.Enable Grab Attach First Pos` (`self.BP_C3_LeftHook`))
  (`/Engine/EditorBlueprintResources/StandardMacros.DoOnce` false
    (:`Completed`
      (`/Game/Chapters/Chapter3/NewBP/BP_C3_LeftHook.Spawn LeftHook` (`self.BP_C3_LeftHook`))
      (`/Game/Chapters/Chapter3/NewBP/BP_C3_RightHook.Spawn RightHook` (`self.BP_C3_RightHook`))
      (`/Game/Chapters/Chapter3/NewBP/BP_C3_RTGCrane.Enable Label 2-1-1` (`self.BP_C3_RTGCrane`))
      (`/Game/Chapters/Chapter3/NewBP/BP_C3_Boots_Anim.Spawn Boots` (`self.BP_C3_Boots_Anim`))
      (`/Game/Chapters/Chapter3/NewBP/BP_C3_Boots_Anim.Teleport To Ladder` (`self.BP_C3_Boots_Anim`)))))

(event `Sub 2-1-1`
  ;[1 1 1] SUB 2
  (`/Game/Chapters/Chapter3/NewBP/BP_C3_LeftHook.Disable Grab Attach` (`self.BP_C3_LeftHook`))
  (`/Game/Chapters/Chapter3/NewBP/BP_C3_GrabPole1.Enable Latch Pole1` (`self.BP_C3_GrabPole1`)))

(event `Sub 2-1-2`
  ;[1 1 1] SUB 2
  (`/Game/Chapters/Chapter3/NewBP/BP_C3_GrabPole1.Disable Latch Pole1` (`self.BP_C3_GrabPole1`))
  (`/AzurealXR/Core/BP_Azr_Pawn.First MovePlayerUp` (`self.BP_Azr_Pawn`))
  (`/Game/Chapters/Chapter3/NewBP/BP_C3_RightHook.Enable Grab Attach First Pos` (`self.BP_C3_RightHook`))
  (`/Game/Chapters/Chapter3/NewBP/BP_C3_Boots_Anim.Left Leg Up` (`self.BP_C3_Boots_Anim`))
  (`/Game/Chapters/Chapter3/NewBP/BP_C3_Boots_Anim.Play Left 1 Up` (`self.BP_C3_Boots_Anim`))
  (`/AzurealXR/Core/BP_Azr_Pawn.Disable Teleport` (`self.BP_Azr_Pawn`)))

(event `Sub 2-1-3`
  ;[1 1 1] SUB 2
  (`/Game/Chapters/Chapter3/NewBP/BP_C3_RightHook.Disable Grab Attach` (`self.BP_C3_RightHook`))
  (`/Game/Chapters/Chapter3/NewBP/BP_C3_GrabPole2.Enable Latch Pole2` (`self.BP_C3_GrabPole2`)))

(event `Sub 2-1-4`
  ;[1 1 1] SUB 2
  (`/Game/Chapters/Chapter3/NewBP/BP_C3_GrabPole2.Disable Latch Pole2` (`self.BP_C3_GrabPole2`))
  (`/AzurealXR/Core/BP_Azr_Pawn.First MovePlayerUp` (`self.BP_Azr_Pawn`))
  (`/Game/Chapters/Chapter3/NewBP/BP_C3_Boots_Anim.Pause Left 1 Up` (`self.BP_C3_Boots_Anim`))
  (`/Game/Chapters/Chapter3/NewBP/BP_C3_Boots_Anim.Right Leg Up` (`self.BP_C3_Boots_Anim`))
  (`/Game/Chapters/Chapter3/NewBP/BP_C3_Boots_Anim.Play Right 1 Up` (`self.BP_C3_Boots_Anim`))
  (`KismetSystemLibrary.Delay` 0.2)
  (`/Game/Chapters/Chapter3/NewBP/BP_C3_LeftHook.Enable Grab Attach Second Pos` (`self.BP_C3_LeftHook`)))

(event `Sub 2-1-5`
  ;[1 1 1] SUB 2
  (`/Game/Chapters/Chapter3/NewBP/BP_C3_LeftHook.Disable Grab Attach` (`self.BP_C3_LeftHook`))
  (`/Game/Chapters/Chapter3/NewBP/BP_C3_GrabPole3.Enable Latch Pole3` (`self.BP_C3_GrabPole3`)))

(event `Sub 2-1-6`
  ;[1 1 1] SUB 2
  (`/Game/Chapters/Chapter3/NewBP/BP_C3_GrabPole3.Disable Latch Pole3` (`self.BP_C3_GrabPole3`))
  (`/AzurealXR/Core/BP_Azr_Pawn.First MovePlayerUp` (`self.BP_Azr_Pawn`))
  (`/Game/Chapters/Chapter3/NewBP/BP_C3_Boots_Anim.Pause Right 1 Up` (`self.BP_C3_Boots_Anim`))
  (`/Game/Chapters/Chapter3/NewBP/BP_C3_Boots_Anim.Left Leg Up Repeat` (`self.BP_C3_Boots_Anim`))
  (`/Game/Chapters/Chapter3/NewBP/BP_C3_Boots_Anim.Play Left 2 Up` (`self.BP_C3_Boots_Anim`))
  (`KismetSystemLibrary.Delay` 0.2)
  (`/Game/Chapters/Chapter3/NewBP/BP_C3_RightHook.Enable Grab Attach Second Pos` (`self.BP_C3_RightHook`)))

(event `Sub 2-1-7`
  ;[1 1 1] SUB 2
  (`/Game/Chapters/Chapter3/NewBP/BP_C3_RightHook.Disable Grab Attach` (`self.BP_C3_RightHook`))
  (`/Game/Chapters/Chapter3/NewBP/BP_C3_GrabPole4.Enable Latch Pole4` (`self.BP_C3_GrabPole4`)))

(event `Sub 2-1-8`
  ;[1 1 1] SUB 2
  (`/Game/Chapters/Chapter3/NewBP/BP_C3_GrabPole4.Disable Latch Pole4` (`self.BP_C3_GrabPole4`))
  (`/AzurealXR/Core/BP_Azr_Pawn.First MovePlayerUp` (`self.BP_Azr_Pawn`))
  (`/Game/Chapters/Chapter3/NewBP/BP_C3_Boots_Anim.Pause Left 2 Up` (`self.BP_C3_Boots_Anim`))
  (`/Game/Chapters/Chapter3/NewBP/BP_C3_Boots_Anim.Right Leg Up Repeat` (`self.BP_C3_Boots_Anim`))
  (`/Game/Chapters/Chapter3/NewBP/BP_C3_Boots_Anim.Play Right 2 Up` (`self.BP_C3_Boots_Anim`))
  (`KismetSystemLibrary.Delay` 0.2)
  (`/Game/Chapters/Chapter3/NewBP/BP_C3_LeftHook.Enable Grab Attach Third Pos` (`self.BP_C3_LeftHook`)))

(event `Sub 2-1-9`
  ;[1 1 1] SUB 2
  (`/Game/Chapters/Chapter3/NewBP/BP_C3_LeftHook.Disable Grab Attach` (`self.BP_C3_LeftHook`))
  (`/Game/Chapters/Chapter3/NewBP/BP_C3_GrabPole5.Enable Latch Pole5` (`self.BP_C3_GrabPole5`)))

(event `Sub 2-1-10`
  ;[1 1 1] SUB 2
  (`/Game/Chapters/Chapter3/NewBP/BP_C3_GrabPole5.Disable Latch Pole5` (`self.BP_C3_GrabPole5`))
  (`/AzurealXR/Core/BP_Azr_Pawn.First MovePlayerUp` (`self.BP_Azr_Pawn`))
  (`/Game/Chapters/Chapter3/NewBP/BP_C3_Boots_Anim.Pause Right 2 Up` (`self.BP_C3_Boots_Anim`))
  (`/Game/Chapters/Chapter3/NewBP/BP_C3_Boots_Anim.Left Leg Up Repeat` (`self.BP_C3_Boots_Anim`))
  (`/Game/Chapters/Chapter3/NewBP/BP_C3_Boots_Anim.Play Left 3 Up` (`self.BP_C3_Boots_Anim`))
  (`KismetSystemLibrary.Delay` 0.2)
  (`/Game/Chapters/Chapter3/NewBP/BP_C3_RightHook.Enable Grab Attach Third Pos` (`self.BP_C3_RightHook`)))

(event `Sub 2-1-11`
  ;[1 1 1] SUB 2
  (`/Game/Chapters/Chapter3/NewBP/BP_C3_RightHook.Disable Grab Attach` (`self.BP_C3_RightHook`))
  (`/Game/Chapters/Chapter3/NewBP/BP_C3_GrabPole6.Enable Latch Pole6` (`self.BP_C3_GrabPole6`)))

(event `Sub 2-1-12`
  ;[1 1 1] SUB 2
  (`/Game/Chapters/Chapter3/NewBP/BP_C3_GrabPole6.Disable Latch Pole6` (`self.BP_C3_GrabPole6`))
  (`/AzurealXR/Core/BP_Azr_Pawn.First MovePlayerUp` (`self.BP_Azr_Pawn`))
  (`/Game/Chapters/Chapter3/NewBP/BP_C3_Boots_Anim.Pause Left 3 Up` (`self.BP_C3_Boots_Anim`))
  (`/Game/Chapters/Chapter3/NewBP/BP_C3_Boots_Anim.Right Leg Up Repeat` (`self.BP_C3_Boots_Anim`))
  (`/Game/Chapters/Chapter3/NewBP/BP_C3_Boots_Anim.Play Right 3 Up` (`self.BP_C3_Boots_Anim`))
  (`/Game/Chapters/Chapter3/NewBP/BP_C3_RTGCrane.Disabel Label 2-1-1` (`self.BP_C3_RTGCrane`))
  (`KismetSystemLibrary.Delay` 3.0)
  (`/Game/Chapters/Chapter3/NewBP/BP_C3_Boots_Anim.Teleport To Stair` (`self.BP_C3_Boots_Anim`))
  (`/Game/Chapters/Chapter3/BP_C3_CSM.Teleport To Top Crane` (`self.BP_C3_CSM`))
  (`/Game/Chapters/Chapter3/NewBP/BP_C3_LeftHook.Hide LeftHook` (`self.BP_C3_LeftHook`))
  (`/Game/Chapters/Chapter3/NewBP/BP_C3_RightHook.Hide RightHook` (`self.BP_C3_RightHook`))
  ;[1 0.04231 0] Instructions
  (`TrainingStepPage.AdvanceProgress` (`self.WBP_Step_Page`))
  ;[0.01405 0 1] ManualVR
  (`ManualVRPluginBPLibrary.Update` "3" "2" "1" 1)
  ;[1 1 1] Pointers
  (`/Game/Chapters/Chapter3/BP_C3_CSM.Enable Pointer` (`self.BP_C3_CSM`))
  (`GameplayStatics.SpawnSound2D` "/Game/Chapters/Steps_Completed/2Comp.2Comp" 1.0 1.0 0.0 null)
  (`ManualVRPluginBPLibrary.End`))

(event `Reset Everything`
  ;[1 1 1] SUB 2
  (`/Game/Chapters/Chapter3/NewBP/BP_C3_GrabPole1.Reset Pole 1` (`self.BP_C3_GrabPole1`))
  (`/Game/Chapters/Chapter3/NewBP/BP_C3_GrabPole1.Disable Latch Pole1` (`self.BP_C3_GrabPole1`))
  (`/Game/Chapters/Chapter3/NewBP/BP_C3_GrabPole2.Reset Pole 2` (`self.BP_C3_GrabPole2`))
  (`/Game/Chapters/Chapter3/NewBP/BP_C3_GrabPole2.Disable Latch Pole2` (`self.BP_C3_GrabPole2`))
  (`/Game/Chapters/Chapter3/NewBP/BP_C3_GrabPole3.Reset Pole 3` (`self.BP_C3_GrabPole3`))
  (`/Game/Chapters/Chapter3/NewBP/BP_C3_GrabPole3.Disable Latch Pole3` (`self.BP_C3_GrabPole3`))
  (`/Game/Chapters/Chapter3/NewBP/BP_C3_GrabPole4.Reset Pole 4` (`self.BP_C3_GrabPole4`))
  (`/Game/Chapters/Chapter3/NewBP/BP_C3_GrabPole4.Disable Latch Pole4` (`self.BP_C3_GrabPole4`))
  (`/Game/Chapters/Chapter3/NewBP/BP_C3_GrabPole5.Reset Pole 5` (`self.BP_C3_GrabPole5`))
  (`/Game/Chapters/Chapter3/NewBP/BP_C3_GrabPole5.Disable Latch Pole5` (`self.BP_C3_GrabPole5`))
  (`/Game/Chapters/Chapter3/NewBP/BP_C3_GrabPole6.Disable Latch Pole6` (`self.BP_C3_GrabPole6`))
  (`/Game/Chapters/Chapter3/NewBP/BP_C3_LeftHook.Reset LeftHook` (`self.BP_C3_LeftHook`))
  (`/Game/Chapters/Chapter3/NewBP/BP_C3_RightHook.Reset RightHook` (`self.BP_C3_RightHook`))
  (`/Game/Chapters/Chapter3/NewBP/BP_C3_GrabPole1.Fall` (`self.BP_C3_GrabPole1`))
  (`/Game/Chapters/Chapter3/NewBP/BP_C3_Boots_Anim.Reset Anim R` (`self.BP_C3_Boots_Anim`))
  (`/Game/Chapters/Chapter3/NewBP/BP_C3_Boots_Anim.Reset Anim L` (`self.BP_C3_Boots_Anim`))
  (`/AzurealXR/Core/BP_Azr_Pawn.Enable Teleport` (`self.BP_Azr_Pawn`))
  (`/AzurealXR/Core/BP_Azr_Pawn.On Danger` (`self.BP_Azr_Pawn`))
  (`KismetSystemLibrary.Delay` 2.0)
  (`/AzurealXR/Core/BP_Azr_Pawn.Off Danger` (`self.BP_Azr_Pawn`)))

(fn `UserConstructionScript`)
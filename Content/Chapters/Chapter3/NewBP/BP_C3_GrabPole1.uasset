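; BP_C3_GrabPole1 is the first latchable grab pole in Chapter 3's climbing sequence.
; It enables or disables its Azr_Latch on demand and calls GM_C3's Sub212 on first latch, until reset.
; Releasing while GrabPole2 is not grabbed ends climbing, resets both hooks and restarts the game mode at Step2.
; PlayFallAnim fakes a fall on Tick, lowering the pawn and camera at fixed XY until a Z threshold.
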(event `self.ReceiveBeginPlay`
  (`KismetSystemLibrary.Delay` 0.2)
  (bind _returnvalue (`GameplayStatics.GetActorOfClass` "/Game/Chapters/Chapter3/GM_C3.GM_C3_C"))
  (set `self.GM_C3` _returnvalue)
  (bind _returnvalue_2 (`GameplayStatics.GetActorOfClass` "/AzurealXR/Core/BP_Azr_Pawn.BP_Azr_Pawn_C"))
  (set `self.BP_AZR_Pawn` _returnvalue_2)
  (bind _returnvalue_3 (`GameplayStatics.GetActorOfClass` "/Game/Chapters/Chapter3/NewBP/BP_C3_GrabPole2.BP_C3_GrabPole2_C"))
  (set `self.BP_C3_GrabPole2` _returnvalue_3)
  (bind _returnvalue_4 (`GameplayStatics.GetActorOfClass` "/Game/Chapters/Chapter3/NewBP/BP_C3_RightHook.BP_C3_RightHook_C"))
  (set `self.BP_C3_RightHook` _returnvalue_4)
  (bind _returnvalue_5 (`GameplayStatics.GetActorOfClass` "/Game/Chapters/Chapter3/NewBP/BP_C3_LeftHook.BP_C3_LeftHook_C"))
  (set `self.BP_C3_LeftHook` _returnvalue_5))

(event `Play Fall Anim`
  (`self.SetActorTickEnabled` true)
  (`KismetSystemLibrary.Delay` 0.5)
  (set `self.Fall Anim` true))

(event `Enable Latch Pole1`
  (`Azr_Latch.EnableLatch` (`self.Azr_Latch`)))

(event `Disable Latch Pole1`
  (`Azr_Latch.DisableLatch` (`self.Azr_Latch`)))

(event `self.Azr_Latch.OnLatched`
  (`/Engine/EditorBlueprintResources/StandardMacros.DoOnce` false :!label _label
    (:`Completed`
      (`/Game/Chapters/Chapter3/GM_C3.Sub 2-1-2` (`self.GM_C3`)))))

(event `Reset Pole 1`
  (goto _label :!via `Reset`))

(event `self.ReceiveTick`
  (params (DeltaSeconds :type "Float (single-precision)"))
  (bind _bp_azr_pawn (`self.BP_AZR_Pawn`))
  (bind (_returnvalue_x _returnvalue_y _returnvalue_z) (`KismetMathLibrary.BreakVector` (`self.K2_GetActorLocation` _bp_azr_pawn)))
  (bind _returnvalue (- _returnvalue_z 10.0))
  (`|ExecutionSequence`
    (:`then_0`
      (if (`self.Fall Anim`)
        (`SceneComponent.K2_SetWorldLocation` (`Azr_Pawn.Camera` _bp_azr_pawn) (`KismetMathLibrary.MakeVector` -2714.009257 4073.067759 _returnvalue) false false)
        (`self.K2_SetActorLocationAndRotation` _bp_azr_pawn (`KismetMathLibrary.MakeVector` -2714.009257 4073.067759 _returnvalue) (`self.New Rotation`) false false)
        (if (<= _returnvalue_z -20.0)
          (set `self.Fall Anim` false)
          (`self.SetActorTickEnabled` false))))))

(event `self.Azr_Latch.OnLatchReleased`
  (`KismetSystemLibrary.PrintString` "RELEASE")
  (if (not (`/Game/Chapters/Chapter3/NewBP/BP_C3_GrabPole2.IsGrabbing` (`self.BP_C3_GrabPole2`)))
    (`/AzurealXR/Core/BP_Azr_Pawn.Ending Climbing` (`self.BP_AZR_Pawn`))
    (`SceneComponent.K2_SetWorldLocation` (`Azr_Interactable.SceneRoot` (`self.BP_C3_RightHook`)) (`self.New Location_0`) false false)
    (`SceneComponent.K2_SetWorldLocation` (`Azr_Interactable.SceneRoot` (`self.BP_C3_LeftHook`)) (`self.New Location`) false false)
    (`/Game/Chapters/Chapter3/NewBP/BP_C3_LeftHook.Disable Grab Attach` (`self.BP_C3_LeftHook`))
    (`/Game/Chapters/Chapter3/NewBP/BP_C3_RightHook.Disable Grab Attach` (`self.BP_C3_RightHook`))
    (`KismetSystemLibrary.Delay` 0.5)
    (`/Game/Chapters/Chapter3/GM_C3.Reset Everything` (`self.GM_C3`))
    (`KismetSystemLibrary.Delay` 0.1)
    (`/Game/Chapters/Chapter3/GM_C3.Step 2` (`self.GM_C3`))))

(fn `UserConstructionScript`)
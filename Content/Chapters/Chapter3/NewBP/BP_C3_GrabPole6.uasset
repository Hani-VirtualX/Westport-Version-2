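; BP_C3_GrabPole6 is the sixth grab pole in Chapter 3, a latchable actor that reports when it is grabbed.
; After a short delay at BeginPlay it caches the GM_C3 game mode, the player pawn and both hook actors.
; The first latch on its AzrLatch component calls Sub2112 on GM_C3 and sets IsGrabbing, gated by a DoOnce.
; Two custom events enable and disable the latch.
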(event `self.ReceiveBeginPlay`
  (`KismetSystemLibrary.Delay` 0.2)
  (bind _returnvalue (`GameplayStatics.GetActorOfClass` "/Game/Chapters/Chapter3/GM_C3.GM_C3_C"))
  (set `self.GM_C3` _returnvalue)
  (bind _returnvalue_2 (`GameplayStatics.GetActorOfClass` "/AzurealXR/Core/BP_Azr_Pawn.BP_Azr_Pawn_C"))
  (set `self.BP_AZR_Pawn` _returnvalue_2)
  (bind _returnvalue_3 (`GameplayStatics.GetActorOfClass` "/Game/Chapters/Chapter3/NewBP/BP_C3_RightHook.BP_C3_RightHook_C"))
  (set `self.BP_C3_RightHook` _returnvalue_3)
  (bind _returnvalue_4 (`GameplayStatics.GetActorOfClass` "/Game/Chapters/Chapter3/NewBP/BP_C3_LeftHook.BP_C3_LeftHook_C"))
  (set `self.BP_C3_LeftHook` _returnvalue_4))

(event `Enable Latch Pole6`
  (`Azr_Latch.EnableLatch` (`self.Azr_Latch`)))

(event `Disable Latch Pole6`
  (`Azr_Latch.DisableLatch` (`self.Azr_Latch`)))

(event `self.Azr_Latch.OnLatched`
  (`/Engine/EditorBlueprintResources/StandardMacros.DoOnce` false
    (:`Completed`
      (`/Game/Chapters/Chapter3/GM_C3.Sub 2-1-12` (`self.GM_C3`))
      (set `self.IsGrabbing` true))))

(fn `UserConstructionScript`)
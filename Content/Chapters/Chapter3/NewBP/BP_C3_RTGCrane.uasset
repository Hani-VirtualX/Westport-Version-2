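; Chapter 3 RTG crane actor that exposes events for explanation steps, labels and a see-inside hole effect on the crane.
; It caches the GM_C3 reference shortly after BeginPlay and calls its Sub111 when the step 1 explanation completes.
; Events toggle the step 1 explanation and AzrLabel, and swap the crane's bottom material for a hole variant.
; The 2-1-1 explanation events are empty stubs, and leftover test chains are unconnected.
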(event `self.ReceiveBeginPlay`
  (`KismetSystemLibrary.Delay` 0.2)
  (bind _returnvalue (`GameplayStatics.GetActorOfClass` "/Game/Chapters/Chapter3/GM_C3.GM_C3_C"))
  (set `self.GM_C3` _returnvalue))

(event `Set 1-1-1 Explain Visible`
  (`Azr_Explain.EnableExplain` (`self.Step1_Explain`)))

(event `Set 1-1-1 Explain Hidden`
  (`Azr_Explain.DisableExplain` (`self.Step1_Explain`)))

(event `self.Step1_Explain.OnExplainCompleted`
  (`/Game/Chapters/Chapter3/GM_C3.Sub 1-1-1` (`self.GM_C3`)))

(event `Enable Label 2-1-1`
  (`Azr_Label.EnableLabel` (`self.Azr_Label`)))

(event `Disabel Label 2-1-1`
  (`Azr_Label.DisableLabel` (`self.Azr_Label`)))

(event `Set 2-1-1 Explain Visible`)

(event `Set 2-1-1 Explain Hidden`)

(event `Show Crane Hole`
  (`PrimitiveComponent.SetMaterial` (`self.WP_RTGCrane_Joined`) 0 "/Game/wesport_Stuff/Assets/RTGCrane/Materials/RTG_Bottom_Inst_Hole.RTG_Bottom_Inst_Hole"))

(event `Hide Crane Hole`
  (`PrimitiveComponent.SetMaterial` (`self.WP_RTGCrane_Joined`) 0 "/Game/wesport_Stuff/Assets/RTGCrane/Materials/RTG_Bottom_Inst.RTG_Bottom_Inst"))

(fn `UserConstructionScript`)
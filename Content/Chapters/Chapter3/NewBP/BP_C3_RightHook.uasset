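; Right-hand safety lanyard hook for Chapter 3, with a cable whose end attaches to the player pawn's lanyard component.
; After a short startup delay it caches GM_C3 and hides the hook and cable, with events to show, hide or reposition them.
; Events toggle grab-attach at three positions on the AzrGrab component, and each successful attach calls the matching GM_C3 sub-step to advance the sequence.
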(event `self.ReceiveBeginPlay`
  (`KismetSystemLibrary.Delay` 0.2)
  (`|ExecutionSequence`
    (:`then_0`
      (bind _returnvalue (`GameplayStatics.GetActorOfClass` "/Game/Chapters/Chapter3/GM_C3.GM_C3_C"))
      (set `self.GM_C3` _returnvalue)
      (`self.Hide RightHook`))
    (:`then_1`
      (`CableComponent.SetAttachEndTo` (`self.Cable`) (`GameplayStatics.GetPlayerPawn` 0) "WP_SafetyLanyard" "None"))))

(event `Enable Grab Attach First Pos`
  (`Azr_Grab.EnableGrabAttach` (`self.Azr_Grab`) 1))

(event `Disable Grab Attach`
  (`Azr_Grab.DisableGrabAttach` (`self.Azr_Grab`)))

(event `Enable Grab Attach Second Pos`
  (`Azr_Grab.EnableGrabAttach` (`self.Azr_Grab`) 2))

(event `Enable Grab Attach Third Pos`
  (`Azr_Grab.EnableGrabAttach` (`self.Azr_Grab`) 3))

(event `Reset RightHook`
  (`SceneComponent.K2_SetWorldLocationAndRotation` (`self.SceneRoot`) (`self.New Location`) (`self.New Rotation`) false false))

(event `Hide RightHook`
  (`SceneComponent.SetHiddenInGame` (`self.SM_Metal_Hook01`) true false)
  (`SceneComponent.SetHiddenInGame` (`self.Cable`) true false))

(event `Spawn RightHook`
  (`SceneComponent.SetHiddenInGame` (`self.SM_Metal_Hook01`) false false)
  (`SceneComponent.SetHiddenInGame` (`self.Cable`) false false))

(event `self.Azr_Grab.OnGrabAttached`
  (params (SequenceID :type Integer) (Target :type "Azr_AttachTarget Object Reference"))
  (switch `int` SequenceID
    (:`1`
      (`/Game/Chapters/Chapter3/GM_C3.Sub 2-1-3` (`self.GM_C3`)))
    (:`2`
      (`/Game/Chapters/Chapter3/GM_C3.Sub 2-1-7` (`self.GM_C3`)))
    (:`3`
      (`/Game/Chapters/Chapter3/GM_C3.Sub 2-1-11` (`self.GM_C3`)))))

(fn `UserConstructionScript`)
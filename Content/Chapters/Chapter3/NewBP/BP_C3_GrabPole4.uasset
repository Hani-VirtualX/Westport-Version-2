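; BP_C3_GrabPole4 is the fourth grab pole in a Chapter 3 sequence, built around an Azr latch that other logic can enable, disable or reset.
; The first latch after each reset notifies GM_C3 via Sub218 and force-releases pole 3.
; Releasing it while pole 5 is not grabbed repositions both hooks, disables their grab attach, then resets the sequence through GM_C3 and calls Step2 after short delays.
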(event `self.ReceiveBeginPlay`
  (`KismetSystemLibrary.Delay` 0.2)
  (bind _returnvalue (`GameplayStatics.GetActorOfClass` "/Game/Chapters/Chapter3/GM_C3.GM_C3_C"))
  (set `self.GM_C3` _returnvalue)
  (bind _returnvalue_2 (`GameplayStatics.GetActorOfClass` "/AzurealXR/Core/BP_Azr_Pawn.BP_Azr_Pawn_C"))
  (set `self.BP_AZR_Pawn` _returnvalue_2)
  (bind _returnvalue_3 (`GameplayStatics.GetActorOfClass` "/Game/Chapters/Chapter3/NewBP/BP_C3_GrabPole5.BP_C3_GrabPole5_C"))
  (set `self.BP_C3_GrabPole5` _returnvalue_3)
  (bind _returnvalue_4 (`GameplayStatics.GetActorOfClass` "/Game/Chapters/Chapter3/NewBP/BP_C3_RightHook.BP_C3_RightHook_C"))
  (set `self.BP_C3_RightHook` _returnvalue_4)
  (bind _returnvalue_5 (`GameplayStatics.GetActorOfClass` "/Game/Chapters/Chapter3/NewBP/BP_C3_LeftHook.BP_C3_LeftHook_C"))
  (set `self.BP_C3_LeftHook` _returnvalue_5)
  (bind _returnvalue_6 (`GameplayStatics.GetActorOfClass` "/Game/Chapters/Chapter3/NewBP/BP_C3_GrabPole3.BP_C3_GrabPole3_C"))
  (set `self.BP_C3_GrabPole3` _returnvalue_6))

(event `Enable Latch Pole4`
  (`Azr_Latch.EnableLatch` (`self.Azr_Latch`)))

(event `Disable Latch Pole4`
  (`Azr_Latch.DisableLatch` (`self.Azr_Latch`)))

(event `self.Azr_Latch.OnLatched`
  (`/Engine/EditorBlueprintResources/StandardMacros.DoOnce` false :!label _label
    (:`Completed`
      (set `self.IsGrabbing` true)
      (`/Game/Chapters/Chapter3/GM_C3.Sub 2-1-8` (`self.GM_C3`))
      (`Azr_Latch.ForceLatchRelease` (`/Game/Chapters/Chapter3/NewBP/BP_C3_GrabPole3.Azr_Latch` (`self.BP_C3_GrabPole3`))))))

(event `Reset Pole 4`
  (goto _label :!via `Reset`))

(event `self.Azr_Latch.OnLatchReleased`
  (set `self.IsGrabbing` false)
  (if (not (`/Game/Chapters/Chapter3/NewBP/BP_C3_GrabPole5.IsGrabbing` (`self.BP_C3_GrabPole5`)))
    (`SceneComponent.K2_SetWorldLocation` (`Azr_Interactable.SceneRoot` (`self.BP_C3_RightHook`)) (`self.New Location_0`) false false)
    (`SceneComponent.K2_SetWorldLocation` (`Azr_Interactable.SceneRoot` (`self.BP_C3_LeftHook`)) (`self.New Location`) false false)
    (`/Game/Chapters/Chapter3/NewBP/BP_C3_LeftHook.Disable Grab Attach` (`self.BP_C3_LeftHook`))
    (`/Game/Chapters/Chapter3/NewBP/BP_C3_RightHook.Disable Grab Attach` (`self.BP_C3_RightHook`))
    (`KismetSystemLibrary.Delay` 0.5)
    (`/Game/Chapters/Chapter3/GM_C3.Reset Everything` (`self.GM_C3`))
    (`KismetSystemLibrary.Delay` 0.1)
    (`/Game/Chapters/Chapter3/GM_C3.Step 2` (`self.GM_C3`))))

(fn `UserConstructionScript`)
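; Test actor for the right safety-lanyard hook in a Chapter 2 task: a grabbable metal hook with a cable.
; After a short delay on BeginPlay it caches GM_TestC2, hides hook and cable, and attaches the cable end to the player pawn's WP_SafetyLanyard.
; Events show or hide the hook and enable or disable grab-attach at two positions.
; The first successful attach calls Sub233 on GM_TestC2 once.
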(event `self.ReceiveBeginPlay`
  (`KismetSystemLibrary.Delay` 0.2)
  (`|ExecutionSequence`
    (:`then_0`
      (bind _returnvalue (`GameplayStatics.GetActorOfClass` "/Game/Chapters/NEW_C2/BP/GM_TestC2.GM_TestC2_C"))
      (set `self.GM_TestC2` _returnvalue)
      (`self.Hide RightHook`))
    (:`then_1`
      (`CableComponent.SetAttachEndTo` (`self.Cable`) (`GameplayStatics.GetPlayerPawn` 0) "WP_SafetyLanyard" "None"))))

(event `Enable Grab Attach First Pos`
  (`Azr_Grab.EnableGrabAttach` (`self.Azr_Grab`) 1)
  (`KismetSystemLibrary.PrintString` "Hello"))

(event `Disable Grab Attach`
  (`Azr_Grab.DisableGrabAttach` (`self.Azr_Grab`)))

(event `Enable Gran Attach Second Pos`
  (`Azr_Grab.EnableGrabAttach` (`self.Azr_Grab`) 2))

(event `Reset RightHook`)

(event `Hide RightHook`
  (`SceneComponent.SetHiddenInGame` (`self.SM_Metal_Hook01`) true false)
  (`SceneComponent.SetHiddenInGame` (`self.Cable`) true false))

(event `Spawn RightHook`
  (`SceneComponent.SetHiddenInGame` (`self.SM_Metal_Hook01`) false false)
  (`SceneComponent.SetHiddenInGame` (`self.Cable`) false false))

(event `self.Azr_Grab.OnGrabAttached`
  (params (SequenceID :type Integer) (Target :type "Azr_AttachTarget Object Reference"))
  (`/Engine/EditorBlueprintResources/StandardMacros.DoOnce` false
    (:`Completed`
      (`/Game/Chapters/NEW_C2/BP/GM_TestC2.Sub 2-3-3` (`self.GM_TestC2`)))))

(fn `UserConstructionScript`)
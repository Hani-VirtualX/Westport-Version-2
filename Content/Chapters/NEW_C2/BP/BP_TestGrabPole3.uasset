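; BP_TestGrabPole3 is the third grabbable pole in the C2 test chapter, reporting to GM_TestC2 when the player latches onto it.
; Its Azr latch can be switched on and off through custom events.
; The first latch sets IsGrabbing and calls Sub236 on GM_TestC2, gated by a DoOnce that ResetPole3 re-arms.
; Releasing the latch does nothing, so IsGrabbing is never cleared.
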(event `self.ReceiveBeginPlay`
  (`KismetSystemLibrary.Delay` 0.2)
  (bind _returnvalue (`GameplayStatics.GetActorOfClass` "/Game/Chapters/NEW_C2/BP/GM_TestC2.GM_TestC2_C"))
  (set `self.GM_TestC2` _returnvalue)
  (bind _returnvalue_2 (`GameplayStatics.GetActorOfClass` "/AzurealXR/Core/BP_Azr_Pawn.BP_Azr_Pawn_C"))
  (set `self.BP_AZR_Pawn` _returnvalue_2))

(event `Enable Latch Pole3`
  (`Azr_Latch.EnableLatch` (`self.Azr_Latch`)))

(event `Disable Latch Pole3`
  (`Azr_Latch.DisableLatch` (`self.Azr_Latch`)))

(event `self.Azr_Latch.OnLatched`
  (`/Engine/EditorBlueprintResources/StandardMacros.DoOnce` false :!label _label
    (:`Completed`
      (set `self.IsGrabbing` true)
      (`/Game/Chapters/NEW_C2/BP/GM_TestC2.Sub 2-3-6` (`self.GM_TestC2`)))))

(event `Reset Pole 3`
  (goto _label :!via `Reset`))

(event `self.Azr_Latch.OnLatchReleased`)

(fn `UserConstructionScript`)
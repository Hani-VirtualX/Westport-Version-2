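; Game mode for the Chapter 2 test, an RTG crane safety training covering a hooked ladder climb and gaze-based walkway hazard spotting.
; BeginPlay caches the level's actors and step-page widget.
; RunStepsOrder plays narration before each of three steps, while externally triggered Sub events swap explanation panels, toggle interactions and advance progress.
; Step 4 is an empty stub, and part of the boot-climb logic is disconnected.
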(event `self.ReceiveBeginPlay`
  (`KismetSystemLibrary.Delay` 0.2)
  (`|ExecutionSequence`
    (:`then_1`
      (bind _returnvalue (`GameplayStatics.GetActorOfClass` "/Game/Chapters/NEW_C2/BP/BP_TestC2_CSM.BP_TestC2_CSM_C"))
      (set `self.BP_TestC2CSM` _returnvalue))
    (:`then_2`
      (bind _foundwidgets (`WidgetBlueprintLibrary.GetAllWidgetsOfClass` "/Game/Test_Chapter/CSM/WBP_StepPage.WBP_StepPage_C" false))
      (set `self.WBP_Step_Page` (`|GetArrayItem` _foundwidgets)))
    (:`then_3`
      (bind _returnvalue_2 (`GameplayStatics.GetActorOfClass` "/Game/Chapters/NEW_C2/BP/BP_TestRTGCrane.BP_TestRTGCrane_C"))
      (set `self.BP_TestRTGCrane` _returnvalue_2)
      (bind _returnvalue_3 (`GameplayStatics.GetActorOfClass` "/Game/Chapters/NEW_C2/BP/BP_TestCraneOperator.BP_TestCraneOperator_C"))
      (set `self.BP_TestCraneOperator` _returnvalue_3)
      (bind _returnvalue_4 (`GameplayStatics.GetActorOfClass` "/Game/Chapters/Chapter2/Blueprint/BP_PlayClimbAnimation.BP_PlayClimbAnimation_C"))
      (set `self.BP_PlayClimbAnimation` _returnvalue_4)
      (bind _returnvalue_5 (`GameplayStatics.GetActorOfClass` "/Game/Chapters/NEW_C2/BP/BP_TestBoots_Anim.BP_TestBoots_Anim_C"))
      (set `self.BP_TestBootsAnim` _returnvalue_5)
      (bind _returnvalue_6 (`GameplayStatics.GetActorOfClass` "/Game/Chapters/NEW_C2/BP/BP_TestLeftHook.BP_TestLeftHook_C"))
      (set `self.BP_TestLeftHook` _returnvalue_6)
      (bind _returnvalue_7 (`GameplayStatics.GetActorOfClass` "/Game/Chapters/NEW_C2/BP/BP_TestRightHook.BP_TestRightHook_C"))
      (set `self.BP_TestRightHook` _returnvalue_7)
      (bind _returnvalue_8 (`GameplayStatics.GetActorOfClass` "/Game/Chapters/NEW_C2/BP/BP_TestGrabPole.BP_TestGrabPole_C"))
      (set `self.BP_TestGrabPole` _returnvalue_8)
      (bind _returnvalue_9 (`GameplayStatics.GetActorOfClass` "/AzurealXR/Core/BP_Azr_Pawn.BP_Azr_Pawn_C"))
      (set `self.BP_Azr_Pawn` _returnvalue_9)
      (bind _returnvalue_10 (`GameplayStatics.GetActorOfClass` "/Game/Chapters/NEW_C2/BP/BP_TestGrabPole2.BP_TestGrabPole2_C"))
      (set `self.BP_TestGrabPole2` _returnvalue_10)
      (bind _returnvalue_11 (`GameplayStatics.GetActorOfClass` "/Game/Chapters/NEW_C2/BP/BP_TestGrabPole3.BP_TestGrabPole3_C"))
      (set `self.BP_TestGrabPole3` _returnvalue_11)
      (bind _returnvalue_12 (`GameplayStatics.GetActorOfClass` "/Game/Chapters/NEW_C2/BP/BP_Test_CubeWalkway.BP_Test_CubeWalkway_C"))
      (set `self.BP_Test_CubeWalkway` _returnvalue_12)
      (bind _returnvalue_13 (`GameplayStatics.GetActorOfClass` "/Game/Chapters/NEW_C2/BP/BP_TestToeBoard.BP_TestToeBoard_C"))
      (set `self.BP_TestToeBoard` _returnvalue_13)
      (bind _returnvalue_14 (`GameplayStatics.GetActorOfClass` "/Game/Chapters/NEW_C2/BP/BP_Test_Scattered_Tools.BP_Test_Scattered_Tools_C"))
      (set `self.BP_TestScatteredTools` _returnvalue_14)
      (bind _returnvalue_15 (`GameplayStatics.GetActorOfClass` "/Game/Chapters/NEW_C2/BP/BP_TestMud.BP_TestMud_C"))
      (set `self.BP_TestMud` _returnvalue_15)
      (bind _returnvalue_16 (`GameplayStatics.GetActorOfClass` "/Game/Chapters/NEW_C2/BP/BP_TestHole.BP_TestHole_C"))
      (set `self.BP_TestHole` _returnvalue_16))
    (:`then_4`
      ;[1 1 1] STEP 2
      (`KismetSystemLibrary.Delay` 3.0))))

(event `self.RunStepsOrder`
  (bind _result (`/Engine/EditorBlueprintResources/StandardMacros.IncrementInt` (`self.Steps Interger`))
    (:`  `
      (switch `int` _result
        (:`1`
          (bind _returnvalue (`GameplayStatics.SpawnSound2D` "/Game/Chapters/Steps_Num/1.1" 1.0 1.0 0.0 null))
          (`KismetSystemLibrary.Delay` (`SoundBase.Duration` (`AudioComponent.Sound` _returnvalue)))
          (bind _returnvalue_2 (`GameplayStatics.SpawnSound2D` "/Game/Chapters/Chapter2/Audio/Wes_C2/Step_Intro/C2_Step1.C2_Step1" 1.0 1.0 0.0 null))
          (`KismetSystemLibrary.Delay` (`SoundBase.Duration` (`AudioComponent.Sound` _returnvalue_2)))
          (`self.Step 1`))
        (:`2`
          (bind _returnvalue_3 (`GameplayStatics.SpawnSound2D` "/Game/Chapters/Steps_Num/2.2" 1.0 1.0 0.0 null))
          (`KismetSystemLibrary.Delay` (`SoundBase.Duration` (`AudioComponent.Sound` _returnvalue_3)))
          (bind _returnvalue_4 (`GameplayStatics.SpawnSound2D` "/Game/Chapters/Chapter2/Audio/Wes_C2/Step_Intro/C2_Step2.C2_Step2" 1.0 1.0 0.0 null))
          (`KismetSystemLibrary.Delay` (`SoundBase.Duration` (`AudioComponent.Sound` _returnvalue_4)))
          (`self.Step 2`))
        (:`3`
          (bind _returnvalue_5 (`GameplayStatics.SpawnSound2D` "/Game/Chapters/Steps_Num/3.3" 1.0 1.0 0.0 null))
          (`KismetSystemLibrary.Delay` (`SoundBase.Duration` (`AudioComponent.Sound` _returnvalue_5)))
          (bind _returnvalue_6 (`GameplayStatics.SpawnSound2D` "/Game/Chapters/Chapter2/Audio/Wes_C2/Step_Intro/C2_Step3.C2_Step3" 1.0 1.0 0.0 null))
          (`KismetSystemLibrary.Delay` (`SoundBase.Duration` (`AudioComponent.Sound` _returnvalue_6)))
          (`self.Step 3`))))))

(event `Step 1`
  ;[1 1 1] STEP 1
  (`/Game/Chapters/NEW_C2/BP/BP_TestRTGCrane.Set 1-1-1 Explain Visible` (`self.BP_TestRTGCrane`)))

(event `Sub 1-1-1`
  ;[1 1 1] SUB 1
  (`/Game/Chapters/NEW_C2/BP/BP_TestRTGCrane.Set 1-1-1 Explain Hidden` (`self.BP_TestRTGCrane`))
  ;[1 0.04231 0] Instructions
  (`TrainingStepPage.AdvanceProgress` (`self.WBP_Step_Page`)))

(event `Sub 2-1-1`
  ;[1 1 1] SUB 2
  (`/Game/Chapters/NEW_C2/BP/BP_TestRTGCrane.Set 2-1-1 Explain Hidden` (`self.BP_TestRTGCrane`))
  (`KismetSystemLibrary.Delay` 0.5)
  (`/Game/Chapters/NEW_C2/BP/BP_TestCraneOperator.Set 2-2-1 Explain Visible` (`self.BP_TestCraneOperator`))
  (`/Game/Chapters/NEW_C2/BP/BP_TestCraneOperator.Spawn Operator` (`self.BP_TestCraneOperator`))
  (`/Game/Chapters/Chapter2/Blueprint/BP_PlayClimbAnimation.Play Animation Climb` (`self.BP_PlayClimbAnimation`))
  (`KismetSystemLibrary.Delay` 0.1)
  (`/Game/Chapters/Chapter2/Blueprint/BP_PlayClimbAnimation.Pause Animation Climb` (`self.BP_PlayClimbAnimation`))
  (`/Game/Chapters/NEW_C2/BP/BP_TestBoots_Anim.Teleport Beside Ladder` (`self.BP_TestBootsAnim`))
  ;[1 0.04231 0] Instructions
  (`TrainingStepPage.AdvanceProgress` (`self.WBP_Step_Page`)))

(event `Step 2`
  ;[1 1 1] STEP 2
  (`/Game/Chapters/NEW_C2/BP/BP_TestRTGCrane.Set 2-1-1 Explain Visible` (`self.BP_TestRTGCrane`)))

(event `Sub 2-2-1`
  ;[1 1 1] SUB 2
  (`/Game/Chapters/NEW_C2/BP/BP_TestCraneOperator.Set 2-2-1 Explain Hidden` (`self.BP_TestCraneOperator`))
  (`KismetSystemLibrary.Delay` 0.5)
  (`/Game/Chapters/NEW_C2/BP/BP_TestCraneOperator.Set 2-2-2 Explain Visible` (`self.BP_TestCraneOperator`)))

(event `Sub 2-2-2`
  ;[1 1 1] SUB 2
  (`/Game/Chapters/NEW_C2/BP/BP_TestCraneOperator.Set 2-2-2 Explain Hidden` (`self.BP_TestCraneOperator`))
  (`KismetSystemLibrary.Delay` 0.5)
  (`/Game/Chapters/NEW_C2/BP/BP_TestCraneOperator.Set 2-2-3 Explain Visible` (`self.BP_TestCraneOperator`))
  (`/Game/Chapters/Chapter2/Blueprint/BP_PlayClimbAnimation.Play Animation Climb` (`self.BP_PlayClimbAnimation`))
  (`KismetSystemLibrary.Delay` 3.0)
  (`/Game/Chapters/Chapter2/Blueprint/BP_PlayClimbAnimation.Pause Animation Climb` (`self.BP_PlayClimbAnimation`)))

(event `Sub 2-2-3`
  ;[1 1 1] SUB 2
  (`/Game/Chapters/NEW_C2/BP/BP_TestCraneOperator.Set 2-2-3 Explain Hidden` (`self.BP_TestCraneOperator`))
  (`KismetSystemLibrary.Delay` 0.5)
  (`/Game/Chapters/NEW_C2/BP/BP_TestCraneOperator.Set 2-2-4 Explain Visible` (`self.BP_TestCraneOperator`))
  (`/Game/Chapters/Chapter2/Blueprint/BP_PlayClimbAnimation.Play Animation Climb` (`self.BP_PlayClimbAnimation`))
  (`KismetSystemLibrary.Delay` 4.0)
  (`/Game/Chapters/Chapter2/Blueprint/BP_PlayClimbAnimation.Pause Animation Climb` (`self.BP_PlayClimbAnimation`)))

(event `Sub 2-2-4`
  ;[1 1 1] SUB 2
  (`/Game/Chapters/NEW_C2/BP/BP_TestCraneOperator.Set 2-2-4 Explain Hidden` (`self.BP_TestCraneOperator`))
  (`KismetSystemLibrary.Delay` 0.5)
  (`/Game/Chapters/NEW_C2/BP/BP_TestCraneOperator.Set 2-2-5 Explain Visible` (`self.BP_TestCraneOperator`))
  (`/Game/Chapters/Chapter2/Blueprint/BP_PlayClimbAnimation.Play Animation Climb` (`self.BP_PlayClimbAnimation`))
  (`KismetSystemLibrary.Delay` 2.0)
  (`/Game/Chapters/Chapter2/Blueprint/BP_PlayClimbAnimation.Pause Animation Climb` (`self.BP_PlayClimbAnimation`)))

(event `Sub 2-2-5`
  ;[1 1 1] SUB 2
  (`/Game/Chapters/NEW_C2/BP/BP_TestCraneOperator.Set 2-2-5 Explain Hidden` (`self.BP_TestCraneOperator`))
  (`KismetSystemLibrary.Delay` 0.5)
  (`/Game/Chapters/NEW_C2/BP/BP_TestCraneOperator.Set 2-2-6 Explain Visible` (`self.BP_TestCraneOperator`))
  (`/Game/Chapters/Chapter2/Blueprint/BP_PlayClimbAnimation.Play Animation Climb` (`self.BP_PlayClimbAnimation`))
  (`KismetSystemLibrary.Delay` 15.0)
  (`/Game/Chapters/Chapter2/Blueprint/BP_PlayClimbAnimation.Pause Animation Climb` (`self.BP_PlayClimbAnimation`)))

(event `Sub 2-2-6`
  ;[1 1 1] SUB 2
  (`/Game/Chapters/NEW_C2/BP/BP_TestCraneOperator.Set 2-2-6 Explain Hidden` (`self.BP_TestCraneOperator`))
  (`KismetSystemLibrary.Delay` 0.5)
  (`/Game/Chapters/NEW_C2/BP/BP_TestCraneOperator.Set 2-2-7 Explain Visible` (`self.BP_TestCraneOperator`)))

(event `Sub 2-2-7-1`
  ;[1 1 1] SUB 2
  (`/Game/Chapters/NEW_C2/BP/BP_TestCraneOperator.Set 2-2-7 Explain Hidden` (`self.BP_TestCraneOperator`))
  (`/Game/Chapters/NEW_C2/BP/BP_TestLeftHook.Spawn LeftHook` (`self.BP_TestLeftHook`))
  (`/Game/Chapters/NEW_C2/BP/BP_TestRightHook.Spawn RightHook` (`self.BP_TestRightHook`))
  (`/Game/Chapters/NEW_C2/BP/BP_TestBoots_Anim.Spawn Boots` (`self.BP_TestBootsAnim`))
  (`/Game/Chapters/NEW_C2/BP/BP_TestCraneOperator.Hide Operator` (`self.BP_TestCraneOperator`))
  (`self.Sub 2-2-7-2`)
  ;[1 0.04231 0] Instructions
  (`TrainingStepPage.AdvanceProgress` (`self.WBP_Step_Page`)))

(event `Sub 2-2-7-2`
  ;[1 1 1] SUB 2
  (`/Game/Chapters/NEW_C2/BP/BP_TestLeftHook.Enable Grab Attach First Pos` (`self.BP_TestLeftHook`))
  (`/Engine/EditorBlueprintResources/StandardMacros.DoOnce` false
    (:`Completed`
      (`/Game/Chapters/NEW_C2/BP/BP_TestBoots_Anim.Teleport To Ladder` (`self.BP_TestBootsAnim`)))))

(event `Sub 2-3-1`
  ;[1 1 1] SUB 2
  (`/Game/Chapters/NEW_C2/BP/BP_TestLeftHook.Disable Grab Attach` (`self.BP_TestLeftHook`))
  (`/Game/Chapters/NEW_C2/BP/BP_TestGrabPole.Enable Latch Pole1` (`self.BP_TestGrabPole`)))

(event `Sub 2-3-2`
  ;[1 1 1] SUB 2
)

(event `Sub 2-3-3`
  ;[1 1 1] SUB 2
  (`/Game/Chapters/NEW_C2/BP/BP_TestRightHook.Disable Grab Attach` (`self.BP_TestRightHook`))
  (`/Game/Chapters/NEW_C2/BP/BP_TestGrabPole2.Enable Latch Pole2` (`self.BP_TestGrabPole2`)))

(event `Sub 2-3-4`
  ;[1 1 1] SUB 2
  (`/Game/Chapters/NEW_C2/BP/BP_TestGrabPole.Disable Latch Pole1` (`self.BP_TestGrabPole`)))

(event `Sub 2-3-5`
  ;[1 1 1] SUB 2
  (`/Game/Chapters/NEW_C2/BP/BP_TestLeftHook.Disable Grab Attach` (`self.BP_TestLeftHook`))
  (`/Game/Chapters/NEW_C2/BP/BP_TestGrabPole3.Enable Latch Pole3` (`self.BP_TestGrabPole3`)))

(event `Sub 2-3-6`
  ;[1 1 1] SUB 2
  (`/Game/Chapters/NEW_C2/BP/BP_TestBoots_Anim.Pause Right 1 Up` (`self.BP_TestBootsAnim`))
  (`/Game/Chapters/NEW_C2/BP/BP_TestGrabPole2.Disable Latch Pole2` (`self.BP_TestGrabPole2`)))

(event `Reset Everything`
  ;[1 1 1] SUB 2
  (`/Game/Chapters/NEW_C2/BP/BP_TestGrabPole.Reset Pole 1` (`self.BP_TestGrabPole`))
  (`/Game/Chapters/NEW_C2/BP/BP_TestGrabPole2.Reset Pole 2` (`self.BP_TestGrabPole2`))
  (`/Game/Chapters/NEW_C2/BP/BP_TestGrabPole2.Disable Latch Pole2` (`self.BP_TestGrabPole2`))
  (`/Game/Chapters/NEW_C2/BP/BP_TestBoots_Anim.Reset Anim L` (`self.BP_TestBootsAnim`))
  (`/Game/Chapters/NEW_C2/BP/BP_TestBoots_Anim.Reset Anim R` (`self.BP_TestBootsAnim`))
  (`/Game/Chapters/NEW_C2/BP/BP_TestGrabPole3.Disable Latch Pole3` (`self.BP_TestGrabPole3`))
  (`/Game/Chapters/NEW_C2/BP/BP_TestLeftHook.Reset LeftHook` (`self.BP_TestLeftHook`))
  (`/Game/Chapters/NEW_C2/BP/BP_TestRightHook.Reset RightHook` (`self.BP_TestRightHook`)))

(event `Sub 3-1-1`
  ;[1 1 1] SUB 3
  (`/Game/Chapters/NEW_C2/BP/BP_TestRTGCrane.Set 3-1-1 Explain Hidden` (`self.BP_TestRTGCrane`))
  (`KismetSystemLibrary.Delay` 0.5)
  (`/Game/Chapters/NEW_C2/BP/BP_TestRTGCrane.Set 3-2-1 Explain Visible` (`self.BP_TestRTGCrane`))
  ;[1 0.04231 0] Instructions
  (`TrainingStepPage.AdvanceProgress` (`self.WBP_Step_Page`)))

(event `Step 3`
  ;[1 1 1] STEP 3
  (`/Game/Chapters/NEW_C2/BP/BP_TestRTGCrane.Set 3-1-1 Explain Visible` (`self.BP_TestRTGCrane`)))

(event `Sub 3-2-1-1`
  ;[1 1 1] SUB 3
  (`/Game/Chapters/NEW_C2/BP/BP_TestRTGCrane.Set 3-2-1 Explain Hidden` (`self.BP_TestRTGCrane`))
  (`/Game/Chapters/NEW_C2/BP/BP_Test_CubeWalkway.Enable Gaze` (`self.BP_Test_CubeWalkway`)))

(event `Sub 3-2-1-2`
  ;[1 1 1] SUB 3
  (`/Game/Chapters/NEW_C2/BP/BP_Test_CubeWalkway.Disable Gaze` (`self.BP_Test_CubeWalkway`))
  (`/Game/Chapters/NEW_C2/BP/BP_Test_CubeWalkway.Set 3-2-2 Explain Visible` (`self.BP_Test_CubeWalkway`)))

(event `Sub 3-2-2-1`
  ;[1 1 1] SUB 3
  (`/Game/Chapters/NEW_C2/BP/BP_Test_CubeWalkway.Set 3-2-2 Explain Hidden` (`self.BP_Test_CubeWalkway`))
  (`/Game/Chapters/NEW_C2/BP/BP_TestToeBoard.Enable Gaze` (`self.BP_TestToeBoard`)))

(event `Sub 3-2-2-2`
  ;[1 1 1] SUB 3
  (`/Game/Chapters/NEW_C2/BP/BP_TestToeBoard.Disable Gaze` (`self.BP_TestToeBoard`))
  (`/Game/Chapters/NEW_C2/BP/BP_TestToeBoard.Set 3-2-3 Explain Visible` (`self.BP_TestToeBoard`)))

(event `Sub 3-2-3`
  ;[1 1 1] SUB 3
  (`/Game/Chapters/NEW_C2/BP/BP_TestToeBoard.Set 3-2-3 Explain Hidden` (`self.BP_TestToeBoard`))
  (`KismetSystemLibrary.Delay` 0.5)
  (`/Game/Chapters/NEW_C2/BP/BP_TestRTGCrane.Set 3-3-1 Explain Visible` (`self.BP_TestRTGCrane`))
  ;[1 0.04231 0] Instructions
  (`TrainingStepPage.AdvanceProgress` (`self.WBP_Step_Page`)))

(event `Sub 3-3-1`
  ;[1 1 1] SUB 3
  (`/Game/Chapters/NEW_C2/BP/BP_TestRTGCrane.Set 3-3-1 Explain Hidden` (`self.BP_TestRTGCrane`))
  (`KismetSystemLibrary.Delay` 0.5)
  (`/Game/Chapters/NEW_C2/BP/BP_Test_Scattered_Tools.Enable Gaze` (`self.BP_TestScatteredTools`)))

(event `Sub 3-3-2-1`
  ;[1 1 1] SUB 3
  (`/Game/Chapters/NEW_C2/BP/BP_Test_Scattered_Tools.Disable Gaze` (`self.BP_TestScatteredTools`))
  (`/Game/Chapters/NEW_C2/BP/BP_Test_Scattered_Tools.Set 3-3-2 Explain Visible` (`self.BP_TestScatteredTools`)))

(event `Sub 3-3-2-2`
  ;[1 1 1] SUB 3
  (`/Game/Chapters/NEW_C2/BP/BP_Test_Scattered_Tools.Set 3-3-2 Explain Hidden` (`self.BP_TestScatteredTools`))
  (`/Game/Chapters/NEW_C2/BP/BP_Test_Scattered_Tools.Hide Tools` (`self.BP_TestScatteredTools`))
  (`/Game/Chapters/NEW_C2/BP/BP_TestMud.Enable Gaze` (`self.BP_TestMud`)))

(event `Sub 3-3-3-1`
  ;[1 1 1] SUB 3
  (`/Game/Chapters/NEW_C2/BP/BP_TestMud.Disable Gaze` (`self.BP_TestMud`))
  (`/Game/Chapters/NEW_C2/BP/BP_TestMud.Set 3-3-2 Explain Visible` (`self.BP_TestMud`)))

(event `Sub 3-3-3-2`
  ;[1 1 1] SUB 3
  (`/Game/Chapters/NEW_C2/BP/BP_TestMud.Set 3-3-2 Explain Hidden` (`self.BP_TestMud`))
  (`/Game/Chapters/NEW_C2/BP/BP_TestMud.Hide Mud` (`self.BP_TestMud`))
  (`/Game/Chapters/NEW_C2/BP/BP_TestHole.Enable Gaze` (`self.BP_TestHole`))
  (`/Game/Chapters/NEW_C2/BP/BP_TestRTGCrane.Show Crane Hole` (`self.BP_TestRTGCrane`)))

(event `Sub 3-3-4-1`
  ;[1 1 1] SUB 3
  (`/Game/Chapters/NEW_C2/BP/BP_TestHole.Disable Gaze` (`self.BP_TestHole`))
  (`/Game/Chapters/NEW_C2/BP/BP_TestHole.Set 3-3-4 Explain Visible` (`self.BP_TestHole`)))

(event `Sub 3-3-4-2`
  ;[1 1 1] SUB 3
  (`/Game/Chapters/NEW_C2/BP/BP_TestHole.Set 3-3-4 Explain Hidden` (`self.BP_TestHole`))
  (`/Game/Chapters/NEW_C2/BP/BP_TestHole.Hide Hole` (`self.BP_TestHole`))
  (`/Game/Chapters/NEW_C2/BP/BP_TestRTGCrane.Hide Crane Hole` (`self.BP_TestRTGCrane`))
  (`KismetSystemLibrary.Delay` 0.5)
  (`/Game/Chapters/NEW_C2/BP/BP_TestRTGCrane.Set 3-3-5 Explain Visible` (`self.BP_TestRTGCrane`)))

(event `Sub 3-3-5`
  ;[1 1 1] SUB 3
  (`/Game/Chapters/NEW_C2/BP/BP_TestRTGCrane.Set 3-3-5 Explain Hidden` (`self.BP_TestRTGCrane`))
  ;[1 0.04231 0] Instructions
  (`TrainingStepPage.AdvanceProgress` (`self.WBP_Step_Page`)))

(event `Step 4`
  ;[1 1 1] STEP 4
)

(fn `UserConstructionScript`)
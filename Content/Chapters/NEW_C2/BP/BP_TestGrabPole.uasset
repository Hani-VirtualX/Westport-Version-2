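; BP_TestGrabPole is a test grab pole for Chapter 2, apparently part of a climbing sequence with left and right hooks.
; It caches the game mode, pawn, second pole and hooks, exposes latch enable/disable, and toggles a hand mesh, hidden at start.
; The first latch notifies GM_TestC2 through a resettable DoOnce.
; Release only logs and checks the second pole; the fall-and-reset chain is disconnected.
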(event `self.ReceiveBeginPlay`
  (`KismetSystemLibrary.Delay` 0.2)
  (bind _returnvalue (`GameplayStatics.GetActorOfClass` "/Game/Chapters/NEW_C2/BP/GM_TestC2.GM_TestC2_C"))
  (set `self.GM_TestC2` _returnvalue)
  (bind _returnvalue_2 (`GameplayStatics.GetActorOfClass` "/AzurealXR/Core/BP_Azr_Pawn.BP_Azr_Pawn_C"))
  (set `self.BP_AZR_Pawn` _returnvalue_2)
  (bind _returnvalue_3 (`GameplayStatics.GetActorOfClass` "/Game/Chapters/NEW_C2/BP/BP_TestGrabPole2.BP_TestGrabPole2_C"))
  (set `self.BP_TestGrabPole2` _returnvalue_3)
  (bind _returnvalue_4 (`GameplayStatics.GetActorOfClass` "/Game/Chapters/NEW_C2/BP/BP_TestLeftHook.BP_TestLeftHook_C"))
  (set `self.BP_TestLeftHook` _returnvalue_4)
  (bind _returnvalue_5 (`GameplayStatics.GetActorOfClass` "/Game/Chapters/NEW_C2/BP/BP_TestRightHook.BP_TestRightHook_C"))
  (set `self.BP_TestRightHook` _returnvalue_5)
  (`self.Set Hidden Hand`))

(event `Enable Latch Pole1`
  (`Azr_Latch.EnableLatch` (`self.Azr_Latch`)))

(event `Disable Latch Pole1`
  (`Azr_Latch.DisableLatch` (`self.Azr_Latch`)))

(event `self.Azr_Latch.OnLatched`
  (`/Engine/EditorBlueprintResources/StandardMacros.DoOnce` false :!label _label
    (:`Completed`
      (`/Game/Chapters/NEW_C2/BP/GM_TestC2.Sub 2-3-2` (`self.GM_TestC2`))
      (`KismetSystemLibrary.PrintString` "LATCHED"))))

(event `Reset Pole 1`
  (goto _label :!via `Reset`))

(event `Set Hidden Hand`
  (`SceneComponent.SetHiddenInGame` (`self.LeftHand`) true false))

(event `Set Visible Hand`
  (`SceneComponent.SetHiddenInGame` (`self.LeftHand`) false false))

(event `self.Azr_Latch.OnLatchReleased`
  (`KismetSystemLibrary.PrintString` "RELEASE")
  (if (`/Game/Chapters/NEW_C2/BP/BP_TestGrabPole2.IsGrabbing` (`self.BP_TestGrabPole2`))
    _))

(fn `UserConstructionScript`)
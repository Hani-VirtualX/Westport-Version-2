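; Test cube walkway actor for Chapter 2 that links gaze and explanation interactions to the chapter's step sequence.
; It caches a GM_TestC2 reference shortly after BeginPlay and exposes events to toggle its AzrGaze and AzrExplain components.
; Gaze trigger and explanation completion each fire once, calling Sub3212 and Sub3221 respectively on GM_TestC2.
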(event `self.ReceiveBeginPlay`
  (`KismetSystemLibrary.Delay` 0.2)
  (bind _returnvalue (`GameplayStatics.GetActorOfClass` "/Game/Chapters/NEW_C2/BP/GM_TestC2.GM_TestC2_C"))
  (set `self.GM_TestC2` _returnvalue))

(event `Enable Gaze`
  (`Azr_Gaze.EnableGaze` (`self.Azr_Gaze`)))

(event `Disable Gaze`
  (`Azr_Gaze.DisableGaze` (`self.Azr_Gaze`)))

(event `Set 3-2-2 Explain Visible`
  (`Azr_Explain.EnableExplain` (`self.Azr_Explain`)))

(event `Set 3-2-2 Explain Hidden`
  (`Azr_Explain.DisableExplain` (`self.Azr_Explain`)))

(event `self.Azr_Gaze.OnGazeTriggered`
  (`/Engine/EditorBlueprintResources/StandardMacros.DoOnce` false
    (:`Completed`
      (`/Game/Chapters/NEW_C2/BP/GM_TestC2.Sub 3-2-1-2` (`self.GM_TestC2`)))))

(event `self.Azr_Explain.OnExplainCompleted`
  (`/Engine/EditorBlueprintResources/StandardMacros.DoOnce` false
    (:`Completed`
      (`/Game/Chapters/NEW_C2/BP/GM_TestC2.Sub 3-2-2-1` (`self.GM_TestC2`)))))

(fn `UserConstructionScript`)
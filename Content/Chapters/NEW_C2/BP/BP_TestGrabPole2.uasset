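; BP_TestGrabPole2 is a latchable grab pole in a Chapter 2 test sequence that reports being grabbed to GM_TestC2.
; On BeginPlay it caches the game mode, pawn, next pole and hook actors, then hides its guide right hand.
; The first latch sets IsGrabbing and calls Sub234 through a resettable DoOnce.
; External events toggle the latch and hand visibility; release only prints debug text, leaving the climb-reset logic disconnected.
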(event `self.ReceiveBeginPlay`
  (`KismetSystemLibrary.Delay` 0.2)
  (bind _returnvalue (`GameplayStatics.GetActorOfClass` "/Game/Chapters/NEW_C2/BP/GM_TestC2.GM_TestC2_C"))
  (set `self.GM_TestC2` _returnvalue)
  (bind _returnvalue_2 (`GameplayStatics.GetActorOfClass` "/AzurealXR/Core/BP_Azr_Pawn.BP_Azr_Pawn_C"))
  (set `self.BP_AZR_Pawn` _returnvalue_2)
  (bind _returnvalue_3 (`GameplayStatics.GetActorOfClass` "/Game/Chapters/NEW_C2/BP/BP_TestGrabPole3.BP_TestGrabPole3_C"))
  (set `self.BP_TestGrabPole3` _returnvalue_3)
  (bind _returnvalue_4 (`GameplayStatics.GetActorOfClass` "/Game/Chapters/NEW_C2/BP/BP_TestRightHook.BP_TestRightHook_C"))
  (set `self.BP_TestRightHook` _returnvalue_4)
  (bind _returnvalue_5 (`GameplayStatics.GetActorOfClass` "/Game/Chapters/NEW_C2/BP/BP_TestLeftHook.BP_TestLeftHook_C"))
  (set `self.BP_TestLeftHook` _returnvalue_5)
  (`self.Set Hidden Hand`))

(event `Set Hidden Hand`
  (`SceneComponent.SetHiddenInGame` (`self.RightHand`) true false))

(event `Set Visible Hand`
  (`SceneComponent.SetHiddenInGame` (`self.RightHand`) false false))

(event `Enable Latch Pole2`
  (`Azr_Latch.EnableLatch` (`self.Azr_Latch`)))

(event `Disable Latch Pole2`
  (`Azr_Latch.DisableLatch` (`self.Azr_Latch`)))

(event `self.Azr_Latch.OnLatched`
  (`/Engine/EditorBlueprintResources/StandardMacros.DoOnce` false :!label _label
    (:`Completed`
      (set `self.IsGrabbing` true)
      (`/Game/Chapters/NEW_C2/BP/GM_TestC2.Sub 2-3-4` (`self.GM_TestC2`)))))

(event `Reset Pole 2`
  (goto _label :!via `Reset`))

(event `self.Azr_Latch.OnLatchReleased`
  (`KismetSystemLibrary.PrintString` "FFFFFFFFFFFFFFFFFFFFFFF"))

(fn `UserConstructionScript`)
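; BP_C4_RTG_Crane is the Chapter 4 RTG crane actor, exposing scripted events for its gaze and explanation interactions and its hole, toe board and guard rail states.
; Events toggle the Azr explain and gaze components, swap the crane's bottom material, show or hide the hole, and permanently destroy the toe board or rail.
; BeginPlay hides the hole and caches GM_C4, whose numbered Sub steps are called when gaze triggers or explanations complete.
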(event `self.ReceiveBeginPlay`
  (`KismetSystemLibrary.Delay` 0.2)
  (`PrimitiveComponent.SetCollisionEnabled` (`self.WP_RTGCrane_Joined`) "QueryAndPhysics")
  (bind _returnvalue (`GameplayStatics.GetActorOfClass` "/Game/Chapters/Chapter_4/Blueprints_C4/GM_C4.GM_C4_C"))
  (set `self.GM C4` _returnvalue)
  (`self.Set Hidden Hole`))

(event `Enable Explain Plus`
  (`Azr_Explain.EnableExplainPlus` (`self.Azr_Explain`)))

(event `Enable Explain Hole`
  (`Azr_Explain.EnableExplain` (`self.Azr_Explain1`)))

(event `Enable Gaze`
  (`Azr_Gaze.EnableGaze` (`self.Azr_Gaze`)))

(event `Set Hole Fix Material`
  (`PrimitiveComponent.SetMaterial` (`self.WP_RTGCrane_Joined`) 0 "/Game/wesport_Stuff/Assets/RTGCrane/Materials/RTG_Bottom_Inst.RTG_Bottom_Inst"))

(event `Enable Explain Walkway`
  (`Azr_Explain.EnableExplain` (`self.Azr_Explain2`)))

(event `Enable Explain Walkway 2`
  (`Azr_Explain.EnableExplain` (`self.Azr_Explain3`)))

(event `Set Hidden ToeBoard`
  (`ActorComponent.K2_DestroyComponent` (`self.ToeBoard`)))

(event `Set Hole Material`
  (`PrimitiveComponent.SetMaterial` (`self.WP_RTGCrane_Joined`) 0 "/Game/wesport_Stuff/Assets/RTGCrane/Materials/RTG_Bottom_Inst_Hole.RTG_Bottom_Inst_Hole"))

(event `Disable Explain Plus`
  (`Azr_Explain.DisableExplain` (`self.Azr_Explain`)))

(event `Disable Explain Hole`
  (`Azr_Explain.DisableExplain` (`self.Azr_Explain1`)))

(event `Disable Explain Walkway`
  (`Azr_Explain.DisableExplain` (`self.Azr_Explain2`)))

(event `Disable Walkway Explain 2`
  (`Azr_Explain.DisableExplain` (`self.Azr_Explain3`)))

(event `Set Hidden GuardRail`
  (`ActorComponent.K2_DestroyComponent` (`self.Rail`)))

(event `Disable Gaze`
  (`Azr_Gaze.DisableGaze` (`self.Azr_Gaze`)))

(event `Set Visible Hole`
  (`SceneComponent.SetHiddenInGame` (`self.Hole`) false false))

(event `Set Hidden Hole`
  (`SceneComponent.SetHiddenInGame` (`self.Hole`) true false))

(event `self.Azr_Explain.OnExplainPlusCompleted`
  (params (StepIndex :type Integer))
  (switch `int` StepIndex
    (:`3`
      (`/Game/Chapters/Chapter_4/Blueprints_C4/GM_C4.Sub 1-1-3` (`self.GM C4`)))))

(event `self.Azr_Explain1.OnExplainCompleted`
  (`/Game/Chapters/Chapter_4/Blueprints_C4/GM_C4.Sub 3-1-6` (`self.GM C4`)))

(event `self.Azr_Gaze.OnGazeTriggered`
  (params (TriggeredZone :type "Azr_Gaze Object Reference"))
  (`/Game/Chapters/Chapter_4/Blueprints_C4/GM_C4.Sub 3-1-5` (`self.GM C4`)))

(event `self.Azr_Explain2.OnExplainCompleted`
  (`/Game/Chapters/Chapter_4/Blueprints_C4/GM_C4.Sub 3-1-7` (`self.GM C4`)))

(event `self.Azr_Explain3.OnExplainCompleted`
  (`/Game/Chapters/Chapter_4/Blueprints_C4/GM_C4.Sub3-1-8` (`self.GM C4`)))

(fn `UserConstructionScript`)
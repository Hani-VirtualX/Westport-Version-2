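; BP_C4_Scattered_Tools is the Chapter 4 scattered tools actor, a target for gaze and explain interactions in the chapter's sequence.
; It exposes events to enable or disable its AzrGaze and AzrExplain components.
; After a short delay on BeginPlay it caches GM_C4, then calls Sub311 on it when gaze triggers and Sub312 when the explanation completes.
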(event `self.ReceiveBeginPlay`
  (`KismetSystemLibrary.Delay` 0.2)
  (bind _returnvalue (`GameplayStatics.GetActorOfClass` "/Game/Chapters/Chapter_4/Blueprints_C4/GM_C4.GM_C4_C"))
  (set `self.GM C4` _returnvalue))

(event `Enable Gaze`
  (`Azr_Gaze.EnableGaze` (`self.Azr_Gaze`)))

(event `Disable Gaze`
  (`Azr_Gaze.DisableGaze` (`self.Azr_Gaze`)))

(event `self.Azr_Gaze.OnGazeTriggered`
  (params (TriggeredZone :type "Azr_Gaze Object Reference"))
  (`/Game/Chapters/Chapter_4/Blueprints_C4/GM_C4.Sub 3-1-1` (`self.GM C4`)))

(event `Enable Explain`
  (`Azr_Explain.EnableExplain` (`self.Azr_Explain`)))

(event `Disable Explain`
  (`Azr_Explain.DisableExplain` (`self.Azr_Explain`)))

(event `self.Azr_Explain.OnExplainCompleted`
  (`/Game/Chapters/Chapter_4/Blueprints_C4/GM_C4.Sub 3-1-2` (`self.GM C4`)))

(fn `UserConstructionScript`)
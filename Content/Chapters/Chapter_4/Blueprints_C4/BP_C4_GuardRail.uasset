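; BP_C4_GuardRail is the Chapter 4 guard rail and toe board actor for gaze-triggered explanation steps.
; Events called on it enable the gaze manager, unhide rail and toe board meshes, toggle each part's explain component and set final materials.
; Gaze and explain-completed callbacks advance matching Sub211 and Sub212 steps on GM_C4, cached after a short BeginPlay delay.
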(event `self.ReceiveBeginPlay`
  (`KismetSystemLibrary.Delay` 0.2)
  (bind _returnvalue (`GameplayStatics.GetActorOfClass` "/Game/Chapters/Chapter_4/Blueprints_C4/GM_C4.GM_C4_C"))
  (set `self.GM C4` _returnvalue))

(event `Enable Gaze - Sequential`
  (`Azr_GazeManager.EnableManager` (`self.Azr_GazeManager`))
  (`SceneComponent.SetHiddenInGame` (`self.Rail`) false true))

(event `Enable Explain GuardRail`
  (`Azr_Explain.EnableExplain` (`self.Azr_Explain1`)))

(event `Enable Explain ToeBoard`
  (`Azr_Explain.EnableExplain` (`self.Azr_Explain2`)))

(event `Set Visible ToeBoard Ghost`
  (`SceneComponent.SetHiddenInGame` (`self.ToeBoard`) false true))

(event `Disable Explain GuardRail`
  (`Azr_Explain.DisableExplain` (`self.Azr_Explain1`)))

(event `Disable Explain ToeBoard`
  (`Azr_Explain.DisableExplain` (`self.Azr_Explain2`)))

(event `Set Guard Rail Ori Material`
  (`PrimitiveComponent.SetMaterial` (`self.Rail`) 0 "/Game/wesport_Stuff/Assets/RTGCrane/Materials/RTG_Bottom_Inst.RTG_Bottom_Inst"))

(event `self.Azr_Gaze1.OnGazeTriggered`
  (params (TriggeredZone :type "Azr_Gaze Object Reference"))
  (`/Game/Chapters/Chapter_4/Blueprints_C4/GM_C4.Sub 2-1-1` (`self.GM C4`)))

(event `self.Azr_Explain1.OnExplainCompleted`
  (`/Game/Chapters/Chapter_4/Blueprints_C4/GM_C4.Sub 2-1-1-P2` (`self.GM C4`)))

(event `Set ToeBoard Ori Material`
  (`PrimitiveComponent.SetMaterial` (`self.ToeBoard`) 0 "/Game/Props/WhiteGrey.WhiteGrey"))

(event `self.Azr_Gaze2.OnGazeTriggered`
  (params (TriggeredZone :type "Azr_Gaze Object Reference"))
  (`/Game/Chapters/Chapter_4/Blueprints_C4/GM_C4.Sub 2-1-2` (`self.GM C4`)))

(event `self.Azr_Explain2.OnExplainCompleted`
  (`/Game/Chapters/Chapter_4/Blueprints_C4/GM_C4.Sub 2-1-2-P2` (`self.GM C4`)))

(fn `UserConstructionScript`)
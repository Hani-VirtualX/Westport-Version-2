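; Chapter 4 game mode that directs a three-step VR safety walkthrough on an RTG crane.
; BeginPlay sets the chapter number, caches scene actors and the step widget, and disables teleport.
; RunStepsOrder plays each step's audio before starting it.
; Externally called sub-step events chain gaze and explanation stages across guard rail, toe board, tools, puddle, hole and walkway, then advance progress, record completion and enable the CSM pointer.
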(event `self.ReceiveBeginPlay`
  (`KismetSystemLibrary.Delay` 0.2)
  (`|ExecutionSequence`
    (:`then_0`
      (bind _asazr_game_instance (cast `/AzurealXR/Core/Azr_GameInstance` (`GameplayStatics.GetGameInstance`)))
      (set `/AzurealXR/Core/Azr_GameInstance.Chapter Number` 4 _asazr_game_instance)
      (bind _returnvalue (`GameplayStatics.GetActorOfClass` "/Game/Chapters/Chapter_4/Blueprints_C4/BP_C4_GuardRail.BP_C4_GuardRail_C"))
      (set `self.BP C4 GuardRail` _returnvalue)
      (bind _returnvalue_2 (`GameplayStatics.GetActorOfClass` "/Game/Chapters/Chapter_4/Blueprints_C4/BP_C4_RTG_Crane.BP_C4_RTG_Crane_C"))
      (set `self.BP C4 RTG Crane` _returnvalue_2)
      (bind _returnvalue_3 (`GameplayStatics.GetActorOfClass` "/Game/Chapters/Chapter_4/Blueprints_C4/BP_C4_Scattered_Tools.BP_C4_Scattered_Tools_C"))
      (set `self.BP C4 Scattered Tools` _returnvalue_3)
      (bind _returnvalue_4 (`GameplayStatics.GetActorOfClass` "/Game/Chapters/Chapter_4/Blueprints_C4/BP_C4_Puddle.BP_C4_Puddle_C"))
      (set `self.BP C4 Puddle` _returnvalue_4)
      (bind _foundwidgets (`WidgetBlueprintLibrary.GetAllWidgetsOfClass` "/Azureal_CSM/WBP_StepPage.WBP_StepPage_C" false))
      (set `self.WBP Step Page` (`|GetArrayItem` _foundwidgets))
      (bind _returnvalue_5 (`GameplayStatics.GetActorOfClass` "/Game/Chapters/Chapter_4/CSM_C4/BP_C4_CSM.BP_C4_CSM_C"))
      (set `self.BP_C4_CSM` _returnvalue_5)
      (bind _returnvalue_6 (`GameplayStatics.GetActorOfClass` "/AzurealXR/Core/BP_Azr_Pawn.BP_Azr_Pawn_C"))
      (set `self.BP_Azr_Pawn` _returnvalue_6))
    (:`then_1`
      (`KismetSystemLibrary.Delay` 0.2)
      (`/AzurealXR/Core/BP_Azr_Pawn.Disable Teleport` (`self.BP_Azr_Pawn`)))))

(event `Step 1`
  ;[1 1 1] STEP 1
  (`/Game/Chapters/Chapter_4/Blueprints_C4/BP_C4_RTG_Crane.Enable Explain Plus` (`self.BP C4 RTG Crane`))
  (`ManualVRPluginBPLibrary.Start`))

(event `Sub 1-1-1`
  ;[1 1 1] SUB 1
)

(event `Sub 1-1-2`
  ;[1 1 1] SUB 1
)

(event `StepSequencerInterface.RunStepsOrder`
  (bind _result (`/Engine/EditorBlueprintResources/StandardMacros.IncrementInt` (`self.Steps Interger`))
    (:`  `
      (switch `int` _result
        (:`1`
          (bind _returnvalue (`GameplayStatics.SpawnSound2D` "/Game/Chapters/Steps_Num/1.1" 1.0 1.0 0.0 null))
          (`KismetSystemLibrary.Delay` (`SoundBase.Duration` (`AudioComponent.Sound` _returnvalue)))
          (bind _returnvalue_2 (`GameplayStatics.SpawnSound2D` "/Game/Chapters/Chapter1/Audio/Wes_C1/Step_Intro/C1_Step1.C1_Step1" 1.0 1.0 0.0 null))
          (`KismetSystemLibrary.Delay` (`SoundBase.Duration` (`AudioComponent.Sound` _returnvalue_2)))
          (`self.Step 1`))
        (:`2`
          (bind _returnvalue_3 (`GameplayStatics.SpawnSound2D` "/Game/Chapters/Steps_Num/2.2" 1.0 1.0 0.0 null))
          (`KismetSystemLibrary.Delay` (`SoundBase.Duration` (`AudioComponent.Sound` _returnvalue_3)))
          (bind _returnvalue_4 (`GameplayStatics.SpawnSound2D` "/Game/Chapters/Chapter_4/C4-Step2.C4-Step2" 1.0 1.0 0.0 null))
          (`KismetSystemLibrary.Delay` (`SoundBase.Duration` (`AudioComponent.Sound` _returnvalue_4)))
          (`self.Step 2`))
        (:`3`
          (bind _returnvalue_5 (`GameplayStatics.SpawnSound2D` "/Game/Chapters/Steps_Num/3.3" 1.0 1.0 0.0 null))
          (`KismetSystemLibrary.Delay` (`SoundBase.Duration` (`AudioComponent.Sound` _returnvalue_5)))
          (bind _returnvalue_6 (`GameplayStatics.SpawnSound2D` "/Game/Chapters/Chapter_4/C4-Step3.C4-Step3" 1.0 1.0 0.0 null))
          (`KismetSystemLibrary.Delay` (`SoundBase.Duration` (`AudioComponent.Sound` _returnvalue_6)))
          (`self.Step 3`))))))

(event `Sub 1-1-3`
  ;[1 1 1] SUB 1
  (`/Game/Chapters/Chapter_4/Blueprints_C4/BP_C4_RTG_Crane.Disable Explain Plus` (`self.BP C4 RTG Crane`))
  ;[1 0.04231 0] Instructions
  (`TrainingStepPage.AdvanceProgress` (`self.WBP Step Page`))
  ;[0.01405 0 1] ManualVR
  (`ManualVRPluginBPLibrary.Update` "4" "1" "1" 1)
  ;[1 1 1] Pointers
  (`/Game/Chapters/Chapter_4/CSM_C4/BP_C4_CSM.Enable Pointer` (`self.BP_C4_CSM`))
  (`GameplayStatics.SpawnSound2D` "/Game/Chapters/Steps_Completed/1Comp.1Comp" 1.0 1.0 0.0 null))

(event `Step 2`
  (bind _bp_c4_rtg_crane (`self.BP C4 RTG Crane`))
  ;[1 1 1] STEP 2
  (`/Game/Chapters/Chapter_4/Blueprints_C4/BP_C4_GuardRail.Enable Gaze - Sequential` (`self.BP C4 GuardRail`))
  (`/Game/Chapters/Chapter_4/Blueprints_C4/BP_C4_RTG_Crane.Set Hidden GuardRail` _bp_c4_rtg_crane)
  (`/Game/Chapters/Chapter_4/Blueprints_C4/BP_C4_RTG_Crane.Set Hole Material` _bp_c4_rtg_crane)
  (`SceneComponent.SetHiddenInGame` (`/Game/Chapters/Chapter_4/Blueprints_C4/BP_C4_Puddle.Puddle` (`self.BP C4 Puddle`)) false false)
  (`/Game/Chapters/Chapter_4/Blueprints_C4/BP_C4_Scattered_Tools.Set Visible Tools` (`self.BP C4 Scattered Tools`)))

(event `Sub 2-1-1`
  ;[1 1 1] SUB 2
  (`KismetSystemLibrary.Delay` 0.2)
  (`/Game/Chapters/Chapter_4/Blueprints_C4/BP_C4_GuardRail.Enable Explain GuardRail` (`self.BP C4 GuardRail`)))

(event `Sub 2-1-1-P2`
  (bind _bp_c4_guardrail (`self.BP C4 GuardRail`))
  ;[1 1 1] SUB 2
  (`/Game/Chapters/Chapter_4/Blueprints_C4/BP_C4_GuardRail.Disable Explain GuardRail` _bp_c4_guardrail)
  (`Azr_GazeManager.TriggerNextGaze` (`/Game/Chapters/Chapter_4/Blueprints_C4/BP_C4_GuardRail.Azr_GazeManager` _bp_c4_guardrail))
  (`/Game/Chapters/Chapter_4/Blueprints_C4/BP_C4_RTG_Crane.Set Hidden ToeBoard` (`self.BP C4 RTG Crane`))
  (`/Game/Chapters/Chapter_4/Blueprints_C4/BP_C4_GuardRail.Set Visible ToeBoard Ghost` _bp_c4_guardrail)
  (`/Game/Chapters/Chapter_4/Blueprints_C4/BP_C4_GuardRail.Set Guard Rail Ori Material` _bp_c4_guardrail))

(event `Sub 2-1-2`
  (bind _bp_c4_guardrail (`self.BP C4 GuardRail`))
  ;[1 1 1] SUB 2
  (`Azr_GazeManager.DisableManager` (`/Game/Chapters/Chapter_4/Blueprints_C4/BP_C4_GuardRail.Azr_GazeManager` _bp_c4_guardrail))
  (`/Game/Chapters/Chapter_4/Blueprints_C4/BP_C4_GuardRail.Enable Explain ToeBoard` _bp_c4_guardrail))

(event `Sub 2-1-2-P2`
  (bind _bp_c4_guardrail (`self.BP C4 GuardRail`))
  ;[1 1 1] SUB 2
  (`/Game/Chapters/Chapter_4/Blueprints_C4/BP_C4_GuardRail.Disable Explain ToeBoard` _bp_c4_guardrail)
  (`/Game/Chapters/Chapter_4/Blueprints_C4/BP_C4_GuardRail.Set ToeBoard Ori Material` _bp_c4_guardrail)
  ;[1 0.04231 0] Instructions
  (`TrainingStepPage.AdvanceProgress` (`self.WBP Step Page`))
  ;[0.01405 0 1] ManualVR
  (`ManualVRPluginBPLibrary.Update` "4" "2" "1" 1)
  ;[1 1 1] Pointers
  (`/Game/Chapters/Chapter_4/CSM_C4/BP_C4_CSM.Enable Pointer` (`self.BP_C4_CSM`))
  (`GameplayStatics.SpawnSound2D` "/Game/Chapters/Steps_Completed/2Comp.2Comp" 1.0 1.0 0.0 null))

(event `Step 3`
  ;[1 1 1] STEP 3
  (`/Game/Chapters/Chapter_4/Blueprints_C4/BP_C4_Scattered_Tools.Enable Gaze` (`self.BP C4 Scattered Tools`)))

(event `Sub 3-1-1`
  ;[1 1 1] SUB 3
  (`/Game/Chapters/Chapter_4/Blueprints_C4/BP_C4_Scattered_Tools.Disable Gaze` (`self.BP C4 Scattered Tools`))
  (`/Game/Chapters/Chapter_4/Blueprints_C4/BP_C4_Scattered_Tools.Enable Explain` (`self.BP C4 Scattered Tools`)))

(event `Sub 3-1-2`
  (bind _bp_c4_scattered_tools (`self.BP C4 Scattered Tools`))
  ;[1 1 1] SUB 3
  (`/Game/Chapters/Chapter_4/Blueprints_C4/BP_C4_Scattered_Tools.Disable Explain` _bp_c4_scattered_tools)
  (`self.K2_DestroyActor` _bp_c4_scattered_tools)
  (`/Game/Chapters/Chapter_4/Blueprints_C4/BP_C4_Puddle.Enable Gaze` (`self.BP C4 Puddle`)))

(event `Sub 3-1-3`
  (bind _bp_c4_puddle (`self.BP C4 Puddle`))
  ;[1 1 1] SUB 3
  (`/Game/Chapters/Chapter_4/Blueprints_C4/BP_C4_Puddle.Disable Gaze` _bp_c4_puddle)
  (`/Game/Chapters/Chapter_4/Blueprints_C4/BP_C4_Puddle.Enable Explain` _bp_c4_puddle))

(event `Sub 3-1-4`
  (bind _bp_c4_puddle (`self.BP C4 Puddle`))
  ;[1 1 1] SUB 3
  (`/Game/Chapters/Chapter_4/Blueprints_C4/BP_C4_Puddle.Disable Explain` _bp_c4_puddle)
  (`self.K2_DestroyActor` _bp_c4_puddle)
  (`/Game/Chapters/Chapter_4/Blueprints_C4/BP_C4_RTG_Crane.Set Visible Hole` (`self.BP C4 RTG Crane`))
  (`/Game/Chapters/Chapter_4/Blueprints_C4/BP_C4_RTG_Crane.Enable Gaze` (`self.BP C4 RTG Crane`)))

(event `Sub 3-1-5`
  (bind _bp_c4_rtg_crane (`self.BP C4 RTG Crane`))
  ;[1 1 1] SUB 3
  (`/Game/Chapters/Chapter_4/Blueprints_C4/BP_C4_RTG_Crane.Disable Gaze` _bp_c4_rtg_crane)
  (`/Game/Chapters/Chapter_4/Blueprints_C4/BP_C4_RTG_Crane.Set Hidden Hole` (`self.BP C4 RTG Crane`))
  (`/Game/Chapters/Chapter_4/Blueprints_C4/BP_C4_RTG_Crane.Enable Explain Hole` _bp_c4_rtg_crane))

(event `Sub 3-1-6`
  (bind _bp_c4_rtg_crane (`self.BP C4 RTG Crane`))
  ;[1 1 1] SUB 3
  (`/Game/Chapters/Chapter_4/Blueprints_C4/BP_C4_RTG_Crane.Disable Explain Hole` _bp_c4_rtg_crane)
  (`/Game/Chapters/Chapter_4/Blueprints_C4/BP_C4_RTG_Crane.Set Hole Fix Material` _bp_c4_rtg_crane)
  (`/Game/Chapters/Chapter_4/Blueprints_C4/BP_C4_RTG_Crane.Enable Explain Walkway` _bp_c4_rtg_crane))

(event `Sub 3-1-7`
  (bind _bp_c4_rtg_crane (`self.BP C4 RTG Crane`))
  ;[1 1 1] SUB 3
  (`/Game/Chapters/Chapter_4/Blueprints_C4/BP_C4_RTG_Crane.Disable Explain Walkway` _bp_c4_rtg_crane)
  (`/Game/Chapters/Chapter_4/Blueprints_C4/BP_C4_RTG_Crane.Enable Explain Walkway 2` _bp_c4_rtg_crane))

(event `Sub3-1-8`
  ;[1 1 1] SUB 3
  (`/Game/Chapters/Chapter_4/Blueprints_C4/BP_C4_RTG_Crane.Disable Walkway Explain 2` (`self.BP C4 RTG Crane`))
  ;[1 0.04231 0] Instructions
  (`TrainingStepPage.AdvanceProgress` (`self.WBP Step Page`))
  ;[0.01405 0 1] ManualVR
  (`ManualVRPluginBPLibrary.Update` "4" "3" "1" 1)
  ;[1 1 1] Pointers
  (`/Game/Chapters/Chapter_4/CSM_C4/BP_C4_CSM.Enable Pointer` (`self.BP_C4_CSM`))
  (`GameplayStatics.SpawnSound2D` "/Game/Chapters/Steps_Completed/3Comp.3Comp" 1.0 1.0 0.0 null)
  (`ManualVRPluginBPLibrary.End`))

(fn `UserConstructionScript`)
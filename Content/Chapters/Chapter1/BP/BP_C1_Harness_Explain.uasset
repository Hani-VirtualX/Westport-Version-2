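; Chapter 1 harness explainer actor that presents the parts of a harness: straps, buckles, stitches and backplate.
; It caches GM_C1 and hides the harness shortly after BeginPlay.
; Callable events toggle an Azr explain component per step (3-1-1 to 3-5-1), toggle part highlights and flip the harness front or back.
; Explain completion callbacks clear the related highlight and call the matching GM_C1 Sub function once to report the step.
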(event `self.ReceiveBeginPlay`
  (`KismetSystemLibrary.Delay` 0.2)
  (bind _returnvalue (`GameplayStatics.GetActorOfClass` "/Game/Chapters/Chapter1/GM_C1.GM_C1_C"))
  (set `self.GM_C1` _returnvalue)
  (`self.Set Hidden Harness`))

(event `Set 3-1-1 Explain Visible`
  ;[1 1 1] Explains
  ;;[0.15 0 0 0.5] 3-1-1
  (`Azr_Explain.EnableExplainPlus` (`self.Azr_Explain_3-1-1`)))

(event `Set 3-1-1 Explain Hidden`
  ;[1 1 1] Explains
  ;;[0.15 0 0 0.5] 3-1-1
  (`Azr_Explain.DisableExplain` (`self.Azr_Explain_3-1-1`)))

(event `Set Visible Harness`)

(event `self.Azr_Explain_3-1-1.OnExplainPlusCompleted`
  (params (StepIndex :type Integer))
  ;[1 1 1] Explains
  ;;[0.15 0 0 0.5] 3-1-1
  (switch `int` StepIndex
    (:`2`
      (`/Engine/EditorBlueprintResources/StandardMacros.DoOnce` false
        (:`Completed`
          (`/Game/Chapters/Chapter1/GM_C1.Sub 3-1-1` (`self.GM_C1`)))))))

(event `Set Hidden Harness`
  (`SceneComponent.SetHiddenInGame` (`self.Harness`) true true))

(event `Set 3-2-1 Explain Visible`
  ;[1 1 1] Explains
  ;;[0.15 0 0 0.5] 3-2-1
  (`Azr_Explain.EnableExplainPlus` (`self.Azr_Explain_3-2-1`)))

(event `Enable Highlight Harness Straps`
  ;[1 1 1] Explains
  ;;[0.15 0 0 0.5] 3-2-1
  (`|ExecutionSequence`
    (:`then_0`
      (`Azr_Highlight.EnableHighlight` (`self.Azr_Highlight_ChestHarness`)))
    (:`then_1`
      (`Azr_Highlight.EnableHighlight` (`self.Azr_Highlight_ShoulderHarness`)))
    (:`then_2`
      (`Azr_Highlight.EnableHighlight` (`self.Azr_Highlight_LegHarness`)))))

(event `Disable Highlight Harness Straps`
  ;[1 1 1] Explains
  ;;[0.15 0 0 0.5] 3-2-1
  (`|ExecutionSequence`
    (:`then_0`
      (`Azr_Highlight.DisableHighlight` (`self.Azr_Highlight_ChestHarness`)))
    (:`then_1`
      (`Azr_Highlight.DisableHighlight` (`self.Azr_Highlight_ShoulderHarness`)))
    (:`then_2`
      (`Azr_Highlight.DisableHighlight` (`self.Azr_Highlight_LegHarness`)))))

(event `Set 3-2-1 Explain Hidden`
  ;[1 1 1] Explains
  ;;[0.15 0 0 0.5] 3-2-1
  (`Azr_Explain.DisableExplain` (`self.Azr_Explain_3-2-1`)))

(event `Rotate Harness Back`
  (`SceneComponent.K2_SetRelativeRotation` (`self.Harness`) (struct :`Yaw` 180.0) false false))

(event `self.Azr_Explain_3-2-1.OnExplainPlusStarted`
  (params (StepIndex :type Integer))
  ;[1 1 1] Explains
  ;;[0.15 0 0 0.5] 3-2-1
)

(event `self.Azr_Explain_3-2-1.OnExplainPlusCompleted`
  (params (StepIndex :type Integer))
  ;[1 1 1] Explains
  ;;[0.15 0 0 0.5] 3-2-1
  (switch `int` StepIndex
    (:`2`
      (`self.Disable Highlight Harness Straps`)
      (`/Engine/EditorBlueprintResources/StandardMacros.DoOnce` false
        (:`Completed`
          (`/Game/Chapters/Chapter1/GM_C1.Sub 3-2-1` (`self.GM_C1`)))))))

(event `Rotate Harness Front`
  (`SceneComponent.K2_SetRelativeRotation` :`self` (`self.Harness`)))

(event `Enable Highlight Buckles`
  ;[1 1 1] Explains
  ;;[0.15 0 0 0.5] 3-3-1
  (`|ExecutionSequence`
    (:`then_0`
      (`Azr_Highlight.EnableHighlight` (`self.Azr_Highlight_LegBuckles`)))
    (:`then_1`
      (`Azr_Highlight.EnableHighlight` (`self.Azr_Highlight_ChestBuckles`)))))

(event `Disable Highlight Buckles`
  ;[1 1 1] Explains
  ;;[0.15 0 0 0.5] 3-3-1
  (`|ExecutionSequence`
    (:`then_0`
      (`Azr_Highlight.DisableHighlight` (`self.Azr_Highlight_LegBuckles`)))
    (:`then_1`
      (`Azr_Highlight.DisableHighlight` (`self.Azr_Highlight_ChestBuckles`)))))

(event `Set 3-3-1 Explain Visible`
  ;[1 1 1] Explains
  ;;[0.15 0 0 0.5] 3-3-1
  (`Azr_Explain.EnableExplain` (`self.Azr_Explain_3-3-1`)))

(event `Set 3-3-1 Explain Hidden`
  ;[1 1 1] Explains
  ;;[0.15 0 0 0.5] 3-3-1
  (`Azr_Explain.DisableExplain` (`self.Azr_Explain_3-3-1`)))

(event `self.Azr_Explain_3-3-1.OnExplainStarted`
  ;[1 1 1] Explains
  ;;[0.15 0 0 0.5] 3-3-1
)

(event `self.Azr_Explain_3-3-1.OnExplainCompleted`
  ;[1 1 1] Explains
  ;;[0.15 0 0 0.5] 3-3-1
  (`self.Disable Highlight Buckles`)
  (`/Engine/EditorBlueprintResources/StandardMacros.DoOnce` false
    (:`Completed`
      (`/Game/Chapters/Chapter1/GM_C1.Sub 3-3-1` (`self.GM_C1`)))))

(event `Set 3-4-1 Explain Visible`
  ;[1 1 1] Explains
  ;;[0.15 0 0 0.5] 3-4-1
  (`Azr_Explain.EnableExplainPlus` (`self.Azr_Explain_3-4-1`)))

(event `Set 3-4-1 Explain Hidden`
  ;[1 1 1] Explains
  ;;[0.15 0 0 0.5] 3-4-1
  (`Azr_Explain.DisableExplain` (`self.Azr_Explain_3-4-1`)))

(event `Enable Highlight Stitches`
  ;[1 1 1] Explains
  ;;[0.15 0 0 0.5] 3-4-1
  (`|ExecutionSequence`
    (:`then_0`
      (`Azr_Highlight.EnableHighlight` (`self.Azr_Highlight_LegStitches`)))
    (:`then_1`
      (`Azr_Highlight.EnableHighlight` (`self.Azr_Highlight_ShoulderStitches`)))
    (:`then_2`
      (`Azr_Highlight.EnableHighlight` (`self.Azr_Highlight_ChestStitches`)))))

(event `Disable Highlight Stitches`
  ;[1 1 1] Explains
  ;;[0.15 0 0 0.5] 3-4-1
  (`|ExecutionSequence`
    (:`then_0`
      (`Azr_Highlight.DisableHighlight` (`self.Azr_Highlight_LegStitches`)))
    (:`then_1`
      (`Azr_Highlight.DisableHighlight` (`self.Azr_Highlight_ShoulderStitches`)))
    (:`then_2`
      (`Azr_Highlight.DisableHighlight` (`self.Azr_Highlight_ChestStitches`)))))

(event `self.Azr_Explain_3-4-1.OnExplainPlusStarted`
  (params (StepIndex :type Integer))
  ;[1 1 1] Explains
  ;;[0.15 0 0 0.5] 3-4-1
)

(event `self.Azr_Explain_3-4-1.OnExplainPlusCompleted`
  (params (StepIndex :type Integer))
  ;[1 1 1] Explains
  ;;[0.15 0 0 0.5] 3-4-1
  (switch `int` StepIndex
    (:`2`
      (`self.Disable Highlight Stitches`)
      (`/Engine/EditorBlueprintResources/StandardMacros.DoOnce` false
        (:`Completed`
          (`/Game/Chapters/Chapter1/GM_C1.Sub 3-4-1` (`self.GM_C1`)))))))

(event `Set 3-5-1 Explain Visible`
  ;[1 1 1] Explains
  (`Azr_Explain.EnableExplainPlus` (`self.Azr_Explain_3-5-1`)))

(event `Set 3-5-1 Explain Hidden`
  ;[1 1 1] Explains
  (`Azr_Explain.DisableExplain` (`self.Azr_Explain_3-5-1`)))

(event `Disable Highlight Backplate`
  ;[1 1 1] Explains
  (`Azr_Highlight.DisableHighlight` (`self.Azr_Highlight_Backplate`)))

(event `Enable Highlight Backplate`
  ;[1 1 1] Explains
  (`Azr_Highlight.EnableHighlight` (`self.Azr_Highlight_Backplate`)))

(event `self.Azr_Explain_3-5-1.OnExplainPlusStarted`
  (params (StepIndex :type Integer))
  ;[1 1 1] Explains
)

(event `self.Azr_Explain_3-5-1.OnExplainPlusCompleted`
  (params (StepIndex :type Integer))
  ;[1 1 1] Explains
  (switch `int` StepIndex
    (:`2`
      (`self.Disable Highlight Backplate`)
      (`/Engine/EditorBlueprintResources/StandardMacros.DoOnce` false
        (:`Completed`
          (`/Game/Chapters/Chapter1/GM_C1.Sub 3-5-1` (`self.GM_C1`)))))))

(fn `UserConstructionScript`)
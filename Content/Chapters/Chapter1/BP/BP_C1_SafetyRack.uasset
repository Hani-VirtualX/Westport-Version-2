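; BP_C1_SafetyRack is a Chapter 1 safety rack with two swinging doors, each opened by its own timeline-driven yaw rotation.
; After a short delay on BeginPlay it caches the GM_C1 actor and calls Step2a on it when the left door finishes opening.
; The right door has no completion callback, and HideRack hides both doors and the main rack in game.
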(event `self.ReceiveBeginPlay`
  (`KismetSystemLibrary.Delay` 0.2)
  (bind _returnvalue (`GameplayStatics.GetActorOfClass` "/Game/Chapters/Chapter1/GM_C1.GM_C1_C"))
  (set `self.GM_C1` _returnvalue))

(event `Open Left Door`
  (bind (_direction _newtrack_0) (`Timeline|OpenLeftDoor` :!via `PlayFromStart`)
    (:`Update`
      (`SceneComponent.K2_SetRelativeRotation` (`self.Left_Door`) (`KismetMathLibrary.MakeRotator` 0.0 0.0 _newtrack_0) false false))
    (:`Finished`
      (`/Game/Chapters/Chapter1/GM_C1.Step 2a` (`self.GM_C1`)))))

(event `Open Right Door`
  (bind (_direction _newtrack_0) (`Timeline|OpenRightDoor` :!via `PlayFromStart`)
    (:`Update`
      (`SceneComponent.K2_SetRelativeRotation` (`self.Right_Door`) (`KismetMathLibrary.MakeRotator` 0.0 0.0 _newtrack_0) false false))))

(event `Hide Rack`
  (`SceneComponent.SetHiddenInGame` (`self.Right_Door`) true false)
  (`SceneComponent.SetHiddenInGame` (`self.Main_Rack`) true false)
  (`SceneComponent.SetHiddenInGame` (`self.Left_Door`) true false))

(fn `UserConstructionScript`)
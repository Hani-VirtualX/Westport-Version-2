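; Chapter 1 safety lanyard actor that serves as an explain-and-grab prop for steps 4-1-1, 4-1-2 and 4-2-1.
; It caches GM_C1 and hides its lanyard, connectors and hooks shortly after BeginPlay, exposing events to toggle visibility, part highlights, explanations and grab attach.
; Completing each explanation or attaching the grab calls the matching GM_C1 sub-step through a DoOnce, and the second explanation also clears the highlights.
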(event `self.ReceiveBeginPlay`
  (`KismetSystemLibrary.Delay` 0.2)
  (bind _returnvalue (`GameplayStatics.GetActorOfClass` "/Game/Chapters/Chapter1/GM_C1.GM_C1_C"))
  (set `self.GM_C1` _returnvalue)
  (`self.Set Hidden Lanyard`))

(event `Set Hidden Lanyard`
  (`SceneComponent.SetHiddenInGame` (`self.WP_SafetyLanyard`) true false)
  (`SceneComponent.SetHiddenInGame` (`self.Connector_R`) true false)
  (`SceneComponent.SetHiddenInGame` (`self.Connector_L`) true false)
  (`SceneComponent.SetHiddenInGame` (`self.SM_Metal_Hook_L`) true true)
  (`SceneComponent.SetHiddenInGame` (`self.SM_Metal_Hook_R`) true true))

(event `Set Visible Lanyard`
  (`SceneComponent.SetHiddenInGame` (`self.WP_SafetyLanyard`) false false)
  (`SceneComponent.SetHiddenInGame` (`self.Connector_R`) false false)
  (`SceneComponent.SetHiddenInGame` (`self.Connector_L`) false false)
  (`SceneComponent.SetHiddenInGame` (`self.SM_Metal_Hook_L`) false true)
  (`SceneComponent.SetHiddenInGame` (`self.SM_Metal_Hook_R`) false true))

(event `Set 4-1-1 Explain Visible`
  (`Azr_Explain.EnableExplain` (`self.Azr_Explain_4-1-1`)))

(event `Set 4-1-1 Explain Hidden`
  (`Azr_Explain.DisableExplain` (`self.Azr_Explain_4-1-1`)))

(event `self.Azr_Explain_4-1-1.OnExplainCompleted`
  (`/Engine/EditorBlueprintResources/StandardMacros.DoOnce` false
    (:`Completed`
      (`/Game/Chapters/Chapter1/GM_C1.Sub 4-1-1` (`self.GM_C1`)))))

(event `Enable Highlight`
  (`|ExecutionSequence`
    (:`then_0`
      (`Azr_Highlight.EnableHighlight` (`self.Azr_Highlight_Shock`)))
    (:`then_1`
      (`Azr_Highlight.EnableHighlight` (`self.Azr_Highlight_Connector_R`)))
    (:`then_2`
      (`Azr_Highlight.EnableHighlight` (`self.Azr_Highlight_Hooks_L`)))
    (:`then_3`
      (`Azr_Highlight.EnableHighlight` (`self.Azr_Highlight_Hooks_R`)))
    (:`then_4`
      (`Azr_Highlight.EnableHighlight` (`self.Azr_Highlight_Connector_L`)))))

(event `Disable Highlight`
  (`|ExecutionSequence`
    (:`then_0`
      (`Azr_Highlight.DisableHighlight` (`self.Azr_Highlight_Shock`)))
    (:`then_1`
      (`Azr_Highlight.DisableHighlight` (`self.Azr_Highlight_Connector_R`)))
    (:`then_2`
      (`Azr_Highlight.DisableHighlight` (`self.Azr_Highlight_Hooks_L`)))
    (:`then_3`
      (`Azr_Highlight.DisableHighlight` (`self.Azr_Highlight_Hooks_R`)))
    (:`then_4`
      (`Azr_Highlight.DisableHighlight` (`self.Azr_Highlight_Connector_L`)))))

(event `Set 4-1-2 Explain Visible`
  (`Azr_Explain.EnableExplain` (`self.Azr_Explain_4-1-2`)))

(event `Set 4-1-2 Explain Hidden`
  (`Azr_Explain.DisableExplain` (`self.Azr_Explain_4-1-2`)))

(event `self.Azr_Explain_4-1-2.OnExplainStarted`)

(event `self.Azr_Explain_4-1-2.OnExplainCompleted`
  (`self.Disable Highlight`)
  (`/Engine/EditorBlueprintResources/StandardMacros.DoOnce` false
    (:`Completed`
      (`/Game/Chapters/Chapter1/GM_C1.Sub 4-1-2` (`self.GM_C1`)))))

(event `self.Azr_Grab.OnGrabAttached`
  (params (SequenceID :type Integer) (Target :type "Azr_AttachTarget Object Reference"))
  (`/Engine/EditorBlueprintResources/StandardMacros.DoOnce` false
    (:`Completed`
      (`/Game/Chapters/Chapter1/GM_C1.Sub 4-2-1` (`self.GM_C1`)))))

(event `Disable Grab Attach`
  (`Azr_Grab.DisableGrabAttach` (`self.Azr_Grab`)))

(event `Enable Grab Attach`
  (`Azr_Grab.EnableGrabAttach` (`self.Azr_Grab`) 1))

(fn `UserConstructionScript`)
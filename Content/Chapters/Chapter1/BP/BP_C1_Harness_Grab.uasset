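; Chapter 1 VR-style grabbable harness actor that triggers a Chapter 1 step when the player first grabs it.
; It caches the Chapter 1 game mode shortly after BeginPlay and starts with the harness mesh and D-ring hidden.
; Exposed events show or hide it, flip it to face behind, and toggle grab attachment on its AzrGrab component.
; The first grab attach calls Sub431 on the game mode, guarded by DoOnce.
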(event `self.ReceiveBeginPlay`
  (`KismetSystemLibrary.Delay` 0.2)
  (bind _returnvalue (`GameplayStatics.GetActorOfClass` "/Game/Chapters/Chapter1/GM_C1.GM_C1_C"))
  (set `self.GM_C1` _returnvalue)
  (`self.Set Hidden Harness`))

(event `Enable Grab Attach`
  (`Azr_Grab.EnableGrabAttach` (`self.Azr_Grab`) 1))

(event `Disable Grab Attach`
  (`Azr_Grab.DisableGrabAttach` (`self.Azr_Grab`)))

(event `self.Azr_Grab.OnGrabAttached`
  (params (SequenceID :type Integer) (Target :type "Azr_AttachTarget Object Reference"))
  (`/Engine/EditorBlueprintResources/StandardMacros.DoOnce` false
    (:`Completed`
      (`/Game/Chapters/Chapter1/GM_C1.Sub 4-3-1` (`self.GM_C1`)))))

(event `Set Hidden Harness`
  (`SceneComponent.SetHiddenInGame` (`self.SM_Harness`) true false)
  (`SceneComponent.SetHiddenInGame` (`self.D-Ring`) true false))

(event `Set Visible Harness`
  (`SceneComponent.SetHiddenInGame` (`self.SM_Harness`) false false)
  (`SceneComponent.SetHiddenInGame` (`self.D-Ring`) false false))

(event `Rotate Harness Behind`
  (`SceneComponent.K2_SetRelativeRotation` (`self.SM_Harness`) (struct :`Yaw` 180.0) false false))

(fn `UserConstructionScript`)
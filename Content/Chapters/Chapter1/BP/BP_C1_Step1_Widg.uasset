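; Chapter 1 Step 1 widget actor that shows and hides the explanation widgets for sub-steps 1-1-1 through 1-1-4.
; Each sub-step has paired Visible and Hidden events that call SetExplain on VXExplain with preset widget settings, arrow, highlight type and cable positions.
; BeginPlay waits briefly, then caches the GM_C1 actor, though these events never use it.
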(event `self.ReceiveBeginPlay`
  (`KismetSystemLibrary.Delay` 0.2)
  (bind _returnvalue (`GameplayStatics.GetActorOfClass` "/Game/Chapters/Chapter1/GM_C1.GM_C1_C"))
  (set `self.GM_C1` _returnvalue))

(event `Set 1-1-1 Explain Visible`
  (`/Game/Azureal_Template/VX_Explain/VX_Explain.Set [ Explain + ]` (`self.VX_Explain`) null (`self.1-1-1_Explain`) true "NewEnumerator8" "NewEnumerator8" "NewEnumerator1" "NewEnumerator4" "NewEnumerator4"))

(event `Set 1-1-1 Explain Hidden`
  (`/Game/Azureal_Template/VX_Explain/VX_Explain.Set [ Explain + ]` (`self.VX_Explain`) null (`self.1-1-1_Explain`) false "NewEnumerator8" "NewEnumerator6" "NewEnumerator4" "NewEnumerator4" "NewEnumerator4"))

(event `Set 1-1-2 Explain Visible`
  (`/Game/Azureal_Template/VX_Explain/VX_Explain.Set [ Explain + ]` (`self.VX_Explain`) null (`self.1-1-2_Explain`) true "NewEnumerator6" "NewEnumerator8" "NewEnumerator1" "NewEnumerator4" "NewEnumerator4"))

(event `Set 1-1-2 Explain Hidden`
  (`/Game/Azureal_Template/VX_Explain/VX_Explain.Set [ Explain + ]` (`self.VX_Explain`) null (`self.1-1-2_Explain`) false "NewEnumerator6" "NewEnumerator6" "NewEnumerator4" "NewEnumerator4" "NewEnumerator4"))

(event `Set 1-1-3 Explain Visible`
  (`/Game/Azureal_Template/VX_Explain/VX_Explain.Set [ Explain + ]` (`self.VX_Explain`) null (`self.1-1-3_Explain`) true "NewEnumerator6" "NewEnumerator8" "NewEnumerator1" "NewEnumerator4" "NewEnumerator4"))

(event `Set 1-1-3 Explain Hidden`
  (`/Game/Azureal_Template/VX_Explain/VX_Explain.Set [ Explain + ]` (`self.VX_Explain`) null (`self.1-1-3_Explain`) false "NewEnumerator6" "NewEnumerator6" "NewEnumerator4" "NewEnumerator4" "NewEnumerator4"))

(event `Set 1-1-4 Explain Visible`
  (`/Game/Azureal_Template/VX_Explain/VX_Explain.Set [ Explain + ]` (`self.VX_Explain`) null (`self.1-1-4_Explain`) true "NewEnumerator9" "NewEnumerator8" "NewEnumerator1" "NewEnumerator4" "NewEnumerator4"))

(event `Set 1-1-4 Explain Hidden`
  (`/Game/Azureal_Template/VX_Explain/VX_Explain.Set [ Explain + ]` (`self.VX_Explain`) null (`self.1-1-4_Explain`) false "NewEnumerator9" "NewEnumerator6" "NewEnumerator4" "NewEnumerator4" "NewEnumerator4"))

(fn `UserConstructionScript`)
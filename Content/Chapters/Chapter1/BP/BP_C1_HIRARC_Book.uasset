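; Chapter 1 HIRARC book actor that hides or shows a book and toggles an explanation component for step 7-2-1.
; On BeginPlay it waits briefly, caches the GM_C1 actor and hides the book.
; Events expose book visibility and enabling or disabling of the Azr explain component.
; When the explanation completes, a DoOnce calls Sub721 on GM_C1 a single time.
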(event `self.ReceiveBeginPlay`
  (`KismetSystemLibrary.Delay` 0.2)
  (bind _returnvalue (`GameplayStatics.GetActorOfClass` "/Game/Chapters/Chapter1/GM_C1.GM_C1_C"))
  (set `self.GM_C1` _returnvalue)
  (`self.Set Book Hidden`))

(event `Set Book Visible`
  (`SceneComponent.SetHiddenInGame` (`self.Book`) false false))

(event `Set 7-2-1 Explain Visible`
  (`Azr_Explain.EnableExplain` (`self.Azr_Explain`)))

(event `Set 7-2-1 Explain Hidden`
  (`Azr_Explain.DisableExplain` (`self.Azr_Explain`)))

(event `Set Book Hidden`
  (`SceneComponent.SetHiddenInGame` (`self.Book`) true false))

(event `self.Azr_Explain.OnExplainCompleted`
  (`/Engine/EditorBlueprintResources/StandardMacros.DoOnce` false
    (:`Completed`
      (`/Game/Chapters/Chapter1/GM_C1.Sub 7-2-1` (`self.GM_C1`)))))

(fn `UserConstructionScript`)
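; Chapter 1 safety boots prop that the player grabs and attaches to a matching ghost placement.
; BeginPlay waits briefly, then caches GM_C1 and the BP_C1_SafetyBoots_Ghost actor.
; Custom events switch the VX_Grab setup on or off with mesh, indicator, UI tag and ghost, or hide the boot mesh.
; The first GrabObjectAttached event calls Sub231 on GM_C1, guarded by a DoOnce.
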(event `self.ReceiveBeginPlay`
  (`KismetSystemLibrary.Delay` 0.2)
  (bind _returnvalue (`GameplayStatics.GetActorOfClass` "/Game/Chapters/Chapter1/GM_C1.GM_C1_C"))
  (set `self.GM_C1` _returnvalue)
  (bind _returnvalue_2 (`GameplayStatics.GetActorOfClass` "/Game/Chapters/Chapter1/BP/BP_C1_SafetyBoots_Ghost.BP_C1_SafetyBoots_Ghost_C"))
  (set `self.BP_C1_SafetyBoots_Ghost` _returnvalue_2))

(event `Set Grab Attach Enable`
  (`/Game/Azureal_Template/VX_Grab/VX_Grab.Set Grab Attach` (`self.VX_Grab`) (`self.Boots_Single`) (`self.BP_GrabIndicator`) (`self.2-3-1_Tag`) (`/Game/Chapters/Chapter1/BP/BP_C1_SafetyBoots_Ghost.Boots_Single` (`self.BP_C1_SafetyBoots_Ghost`)) "GhostUI" true "NewEnumerator0" "NewEnumerator7" "NewEnumerator1" "NewEnumerator0"))

(event `Set Grab Attach Disable`
  (`/Game/Azureal_Template/VX_Grab/VX_Grab.Set Grab Attach` (`self.VX_Grab`) (`self.Boots_Single`) (`self.BP_GrabIndicator`) (`self.2-3-1_Tag`) (`/Game/Chapters/Chapter1/BP/BP_C1_SafetyBoots_Ghost.Boots_Single` (`self.BP_C1_SafetyBoots_Ghost`)) "GhostUI" false "NewEnumerator4" "NewEnumerator6" "NewEnumerator4" "NewEnumerator4"))

(event `Set Hidden Boot`
  (`SceneComponent.SetHiddenInGame` (`self.Boots_Single`) true false))

(event `self.VX_Grab.Grab Object - Attached`
  (params (`Comp Connector Achor` :type "/Game/AFCore/Blueprints/Components/Snapping/Comp_Connector_Anchor Object Reference"))
  (`/Engine/EditorBlueprintResources/StandardMacros.DoOnce` false
    (:`Completed`
      (`/Game/Chapters/Chapter1/GM_C1.Sub 2-3-1` (`self.GM_C1`)))))

(fn `UserConstructionScript`)
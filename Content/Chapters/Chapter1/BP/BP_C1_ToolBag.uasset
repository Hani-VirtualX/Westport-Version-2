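; Chapter 1 tool bag actor that can be shown, explained and grabbed as tutorial steps.
; On BeginPlay it waits briefly, caches the GM_C1 actor and hides the bag mesh.
; Events toggle mesh visibility, the AzrExplain component and AzrGrab attachment.
; The first explain completion calls GMC1.Sub611 and the first grab attach calls Sub621, each guarded by DoOnce.
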(event `self.ReceiveBeginPlay`
  (`KismetSystemLibrary.Delay` 0.2)
  (bind _returnvalue (`GameplayStatics.GetActorOfClass` "/Game/Chapters/Chapter1/GM_C1.GM_C1_C"))
  (set `self.GM_C1` _returnvalue)
  (`self.Set Hidden ToolBag`))

(event `Set Hidden ToolBag`
  (`SceneComponent.SetHiddenInGame` (`self.SM_ToolBag`) true false))

(event `Set Visible ToolBag`
  (`SceneComponent.SetHiddenInGame` (`self.SM_ToolBag`) false false))

(event `Set 6-1-1 Explain Visible`
  (`Azr_Explain.EnableExplain` (`self.Azr_Explain`)))

(event `Set 6-1-1 Explain Hidden`
  (`Azr_Explain.DisableExplain` (`self.Azr_Explain`)))

(event `self.Azr_Explain.OnExplainCompleted`
  (`/Engine/EditorBlueprintResources/StandardMacros.DoOnce` false
    (:`Completed`
      (`/Game/Chapters/Chapter1/GM_C1.Sub 6-1-1` (`self.GM_C1`)))))

(event `Enable Grab Attach`
  (`Azr_Grab.EnableGrabAttach` (`self.Azr_Grab`) 1))

(event `Disable Grab Attach`
  (`Azr_Grab.DisableGrabAttach` (`self.Azr_Grab`)))

(event `self.Azr_Grab.OnGrabAttached`
  (params (SequenceID :type Integer) (Target :type "Azr_AttachTarget Object Reference"))
  (`/Engine/EditorBlueprintResources/StandardMacros.DoOnce` false
    (:`Completed`
      (`/Game/Chapters/Chapter1/GM_C1.Sub 6-2-1` (`self.GM_C1`)))))

(fn `UserConstructionScript`)
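; Chapter 1 game mode for a safety training lesson, apparently VR, covering PPE, harness and lanyard, tool bag and procedure books in seven steps.
; BeginPlay caches the step widget and scene actors; RunStepsOrder increments a counter and plays two voice clips before each step.
; Sub-step events toggle explanations, highlights, grabs and avatar gear, advance the progress page and report completion via Update.
; Each finished step re-enables the pointer and plays a completion sound.
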(event `self.ReceiveBeginPlay`
  (`KismetSystemLibrary.Delay` 0.2)
  (`|ExecutionSequence`
    (:`then_0`
      (bind _asazr_game_instance (cast `/AzurealXR/Core/Azr_GameInstance` (`GameplayStatics.GetGameInstance`)))
      (set `/AzurealXR/Core/Azr_GameInstance.Chapter Number` 1 _asazr_game_instance))
    (:`then_1`
      (bind _returnvalue (`GameplayStatics.GetActorOfClass` "/Game/Chapters/Chapter1/BP/BP_C1_CSM.BP_C1_CSM_C"))
      (set `self.BP_C1_CSM` _returnvalue)
      (`/Game/Chapters/Chapter1/BP/BP_C1_CSM.Enable Pointer` (`self.BP_C1_CSM`)))
    (:`then_2`
      (bind _foundwidgets (`WidgetBlueprintLibrary.GetAllWidgetsOfClass` "/Azureal_CSM/WBP_StepPage.WBP_StepPage_C" false))
      (set `self.WBP_Step_Page` (`|GetArrayItem` _foundwidgets)))
    (:`then_3`
      (bind _returnvalue_2 (`GameplayStatics.GetActorOfClass` "/Game/Chapters/Chapter1/BP/BP_C1_Step1_Widg.BP_C1_Step1_Widg_C"))
      (set `self.BP_C1_Step1_Widg` _returnvalue_2)
      (bind _returnvalue_3 (`GameplayStatics.GetActorOfClass` "/Game/Chapters/Chapter1/BP/BP_C1_SafetyHelmet.BP_C1_SafetyHelmet_C"))
      (set `self.BP_C1_SafetyHelmet` _returnvalue_3)
      (bind _returnvalue_4 (`GameplayStatics.GetActorOfClass` "/Game/Chapters/Chapter1/BP/BP_C1_SafetyRack.BP_C1_SafetyRack_C"))
      (set `self.BP_C1_SafetyRack` _returnvalue_4)
      (bind _returnvalue_5 (`GameplayStatics.GetActorOfClass` "/Game/Chapters/Chapter1/BP/BP_C1_Avatar.BP_C1_Avatar_C"))
      (set `self.BP_C1_Avatar` _returnvalue_5)
      (bind _returnvalue_6 (`GameplayStatics.GetActorOfClass` "/Game/Chapters/Chapter1/BP/BP_C1_HighViz.BP_C1_HighViz_C"))
      (set `self.BP_C1_HighVIZ` _returnvalue_6)
      (bind _returnvalue_7 (`GameplayStatics.GetActorOfClass` "/Game/Chapters/Chapter1/BP/BP_C1_SafetyBoots.BP_C1_SafetyBoots_C"))
      (set `self.BP_C1_SafetyBoots` _returnvalue_7)
      (bind _returnvalue_8 (`GameplayStatics.GetActorOfClass` "/Game/Chapters/Chapter1/BP/BP_C1_SafetyGlove.BP_C1_SafetyGlove_C"))
      (set `self.BP_C1_SafetyGlove` _returnvalue_8)
      (bind _returnvalue_9 (`GameplayStatics.GetActorOfClass` "/Game/Chapters/Chapter1/BP/BP_C1_Harness_Explain.BP_C1_Harness_Explain_C"))
      (set `self.BP_C1_Harness_Explain` _returnvalue_9)
      (bind _returnvalue_10 (`GameplayStatics.GetActorOfClass` "/Game/Chapters/Chapter1/BP/BP_C1_Lanyard.BP_C1_Lanyard_C"))
      (set `self.BP_C1_Lanyard` _returnvalue_10)
      (bind _returnvalue_11 (`GameplayStatics.GetActorOfClass` "/Game/Chapters/Chapter1/BP/BP_C1_Harness_Grab.BP_C1_Harness_Grab_C"))
      (set `self.BP_C1_Harness_Grab` _returnvalue_11)
      (bind _returnvalue_12 (`GameplayStatics.GetActorOfClass` "/Game/Chapters/Chapter1/BP/BP_C1_ToolBag.BP_C1_ToolBag_C"))
      (set `self.BP_C1_ToolBag` _returnvalue_12)
      (bind _returnvalue_13 (`GameplayStatics.GetActorOfClass` "/Game/Chapters/Chapter1/BP/BP_C1_HIRARC_Book.BP_C1_HIRARC_Book_C"))
      (set `self.BP_C1_HIRARC_Book` _returnvalue_13)
      (bind _returnvalue_14 (`GameplayStatics.GetActorOfClass` "/Game/Chapters/Chapter1/BP/BP_C1_SOP_Book.BP_C1_SOP_Book_C"))
      (set `self.BP_C1_SOP_Book` _returnvalue_14)
      (bind _returnvalue_15 (`GameplayStatics.GetActorOfClass` "/Game/Chapters/Chapter1/BP/BP_C1_SafetyTable.BP_C1_SafetyTable_C"))
      (set `self.BP_C1_SafetyTable` _returnvalue_15))))

(event `StepSequencerInterface.RunStepsOrder`
  (bind _result (`/Engine/EditorBlueprintResources/StandardMacros.IncrementInt` (`self.Steps Interger`))
    (:`  `
      (switch `int` _result
        (:`1`
          (bind _returnvalue (`GameplayStatics.SpawnSound2D` "/Game/Chapters/Steps_Num/1.1" 1.0 1.0 0.0 null))
          (`KismetSystemLibrary.Delay` (`SoundBase.Duration` (`AudioComponent.Sound` _returnvalue)))
          (bind _returnvalue_2 (`GameplayStatics.SpawnSound2D` "/Game/Chapters/Chapter1/Audio/Wes_C1/Step_Intro/C1_Step1.C1_Step1" 1.0 1.0 0.0 null))
          (`KismetSystemLibrary.Delay` (`SoundBase.Duration` (`AudioComponent.Sound` _returnvalue_2)))
          (`self.Step 1`))
        (:`2`
          (bind _returnvalue_3 (`GameplayStatics.SpawnSound2D` "/Game/Chapters/Steps_Num/2.2" 1.0 1.0 0.0 null))
          (`KismetSystemLibrary.Delay` (`SoundBase.Duration` (`AudioComponent.Sound` _returnvalue_3)))
          (bind _returnvalue_4 (`GameplayStatics.SpawnSound2D` "/Game/Chapters/Chapter1/Audio/Wes_C1/Step_Intro/C1_Step2.C1_Step2" 1.0 1.0 0.0 null))
          (`KismetSystemLibrary.Delay` (`SoundBase.Duration` (`AudioComponent.Sound` _returnvalue_4)))
          (`self.Step 2`))
        (:`3`
          (bind _returnvalue_5 (`GameplayStatics.SpawnSound2D` "/Game/Chapters/Steps_Num/3.3" 1.0 1.0 0.0 null))
          (`KismetSystemLibrary.Delay` (`SoundBase.Duration` (`AudioComponent.Sound` _returnvalue_5)))
          (bind _returnvalue_6 (`GameplayStatics.SpawnSound2D` "/Game/Chapters/Chapter1/Audio/Wes_C1/Step_Intro/C1_Step3.C1_Step3" 1.0 1.0 0.0 null))
          (`KismetSystemLibrary.Delay` (`SoundBase.Duration` (`AudioComponent.Sound` _returnvalue_6)))
          (`self.Step 3`))
        (:`4`
          (bind _returnvalue_7 (`GameplayStatics.SpawnSound2D` "/Game/Chapters/Steps_Num/4.4" 1.0 1.0 0.0 null))
          (`KismetSystemLibrary.Delay` (`SoundBase.Duration` (`AudioComponent.Sound` _returnvalue_7)))
          (bind _returnvalue_8 (`GameplayStatics.SpawnSound2D` "/Game/Chapters/Chapter1/Audio/Wes_C1/Step_Intro/C1_Step4.C1_Step4" 1.0 1.0 0.0 null))
          (`KismetSystemLibrary.Delay` (`SoundBase.Duration` (`AudioComponent.Sound` _returnvalue_8)))
          (`self.Step 4`))
        (:`5`
          (bind _returnvalue_9 (`GameplayStatics.SpawnSound2D` "/Game/Chapters/Steps_Num/5.5" 1.0 1.0 0.0 null))
          (`KismetSystemLibrary.Delay` (`SoundBase.Duration` (`AudioComponent.Sound` _returnvalue_9)))
          (bind _returnvalue_10 (`GameplayStatics.SpawnSound2D` "/Game/Chapters/Chapter1/Audio/Wes_C1/Step_Intro/C1_Step5.C1_Step5" 1.0 1.0 0.0 null))
          (`KismetSystemLibrary.Delay` (`SoundBase.Duration` (`AudioComponent.Sound` _returnvalue_10)))
          (`self.Step 5`))
        (:`6`
          (bind _returnvalue_11 (`GameplayStatics.SpawnSound2D` "/Game/Chapters/Steps_Num/6.6" 1.0 1.0 0.0 null))
          (`KismetSystemLibrary.Delay` (`SoundBase.Duration` (`AudioComponent.Sound` _returnvalue_11)))
          (bind _returnvalue_12 (`GameplayStatics.SpawnSound2D` "/Game/Chapters/Chapter1/Audio/Wes_C1/Step_Intro/C1_Step6.C1_Step6" 1.0 1.0 0.0 null))
          (`KismetSystemLibrary.Delay` (`SoundBase.Duration` (`AudioComponent.Sound` _returnvalue_12)))
          (`self.Step 6`))
        (:`7`
          (bind _returnvalue_13 (`GameplayStatics.SpawnSound2D` "/Game/Chapters/Steps_Num/7.7" 1.0 1.0 0.0 null))
          (`KismetSystemLibrary.Delay` (`SoundBase.Duration` (`AudioComponent.Sound` _returnvalue_13)))
          (bind _returnvalue_14 (`GameplayStatics.SpawnSound2D` "/Game/Chapters/Chapter1/Audio/Wes_C1/Step_Intro/C1_Step7.C1_Step7" 1.0 1.0 0.0 null))
          (`KismetSystemLibrary.Delay` (`SoundBase.Duration` (`AudioComponent.Sound` _returnvalue_14)))
          (`self.Step 7`))))))

(event `Step 1`
  ;[1 1 1] STEP 1
  (`/Game/Chapters/Chapter1/BP/BP_C1_Step1_Widg.Set 1-1-1 Explain Visible` (`self.BP_C1_Step1_Widg`))
  (`ManualVRPluginBPLibrary.Start`))

(event `Sub 1-1-1`
  ;[1 1 1] SUB 1
  (`/Game/Chapters/Chapter1/BP/BP_C1_Step1_Widg.Set 1-1-1 Explain Hidden` (`self.BP_C1_Step1_Widg`))
  ;[1 0.04231 0] Instructions
  (`TrainingStepPage.AdvanceProgress` (`self.WBP_Step_Page`))
  ;[0.01405 0 1] ManualVR
  (`ManualVRPluginBPLibrary.Update` "1" "1" "1" 1)
  ;[1 1 1] Pointers
  (`/Game/Chapters/Chapter1/BP/BP_C1_CSM.Enable Pointer` (`self.BP_C1_CSM`))
  (`GameplayStatics.SpawnSound2D` "/Game/Chapters/Steps_Completed/1Comp.1Comp" 1.0 1.0 0.0 null))

(event `Step 2`
  ;[1 1 1] STEP 2
  (`/Game/Chapters/Chapter1/BP/BP_C1_SafetyRack.Open Left Door` (`self.BP_C1_SafetyRack`))
  (`/Game/Chapters/Chapter1/BP/BP_C1_SafetyRack.Open Right Door` (`self.BP_C1_SafetyRack`)))

(event `Sub 2-1-1`
  ;[1 1 1] SUB 2
  (`/Game/Chapters/Chapter1/BP/BP_C1_SafetyHelmet.Disable Grab Attach` (`self.BP_C1_SafetyHelmet`))
  (`/Game/Chapters/Chapter1/BP/BP_C1_Avatar.Set Visible Face` (`self.BP_C1_Avatar`))
  (`KismetSystemLibrary.Delay` 0.2)
  (`/Game/Chapters/Chapter1/BP/BP_C1_HighViz.Enable Grab Attach` (`self.BP_C1_HighVIZ`))
  ;[1 0.04231 0] Instructions
  (`TrainingStepPage.AdvanceProgress` (`self.WBP_Step_Page`))
  ;[0.01405 0 1] ManualVR
  (`ManualVRPluginBPLibrary.Update` "1" "2" "1" 1))

(event `Step 2a`
  ;[1 1 1] STEP 2
  (`/Game/Chapters/Chapter1/BP/BP_C1_SafetyHelmet.Enable Grab Attach` (`self.BP_C1_SafetyHelmet`))
  (`/Game/Chapters/Chapter1/BP/BP_C1_Avatar.Set Ghost Torso` (`self.BP_C1_Avatar`))
  (`/Game/Chapters/Chapter1/BP/BP_C1_Avatar.Set Visible Face Ghost` (`self.BP_C1_Avatar`))
  (`/Game/Chapters/Chapter1/BP/BP_C1_Avatar.Set Visible Pants Ghost` (`self.BP_C1_Avatar`)))

(event `Sub 2-2-1`
  ;[1 1 1] SUB 2
  (`/Game/Chapters/Chapter1/BP/BP_C1_HighViz.Disable Grab Attach` (`self.BP_C1_HighVIZ`))
  (`/Game/Chapters/Chapter1/BP/BP_C1_HighViz.Set Hidden HighViz` (`self.BP_C1_HighVIZ`))
  (`/Game/Chapters/Chapter1/BP/BP_C1_Avatar.Set Visible HighViz` (`self.BP_C1_Avatar`))
  (`/Game/Chapters/Chapter1/BP/BP_C1_Avatar.Set Visible Torso` (`self.BP_C1_Avatar`))
  (`KismetSystemLibrary.Delay` 0.2)
  (`/Game/Chapters/Chapter1/BP/BP_C1_SafetyBoots.Enable Grab Attach` (`self.BP_C1_SafetyBoots`))
  ;[1 0.04231 0] Instructions
  (`TrainingStepPage.AdvanceProgress` (`self.WBP_Step_Page`))
  ;[0.01405 0 1] ManualVR
  (`ManualVRPluginBPLibrary.Update` "1" "2" "2" 1))

(event `Sub 2-3-1`
  ;[1 1 1] SUB 2
  (`/Game/Chapters/Chapter1/BP/BP_C1_SafetyBoots.Disable Grab Attach` (`self.BP_C1_SafetyBoots`))
  (`/Game/Chapters/Chapter1/BP/BP_C1_SafetyBoots.Set Hidden Boot` (`self.BP_C1_SafetyBoots`))
  (`/Game/Chapters/Chapter1/BP/BP_C1_Avatar.Set Visible Real Boots` (`self.BP_C1_Avatar`))
  (`/Game/Chapters/Chapter1/BP/BP_C1_Avatar.Set Visible Pants` (`self.BP_C1_Avatar`))
  (`KismetSystemLibrary.Delay` 0.2)
  (`/Game/Chapters/Chapter1/BP/BP_C1_SafetyGlove.Enable Grab Attach` (`self.BP_C1_SafetyGlove`))
  ;[1 0.04231 0] Instructions
  (`TrainingStepPage.AdvanceProgress` (`self.WBP_Step_Page`))
  ;[0.01405 0 1] ManualVR
  (`ManualVRPluginBPLibrary.Update` "1" "2" "3" 1))

(event `Sub 2-4-1`
  ;[1 1 1] SUB 2
  (`/Game/Chapters/Chapter1/BP/BP_C1_SafetyGlove.Disable Grab Attach` (`self.BP_C1_SafetyGlove`))
  (`/Game/Chapters/Chapter1/BP/BP_C1_SafetyGlove.Set Hidden Glove` (`self.BP_C1_SafetyGlove`))
  (`/Game/Chapters/Chapter1/BP/BP_C1_Avatar.Set Visible Real Glove` (`self.BP_C1_Avatar`))
  (`/Game/Chapters/Chapter1/BP/BP_C1_SafetyRack.Close Right Door` (`self.BP_C1_SafetyRack`))
  (`/Game/Chapters/Chapter1/BP/BP_C1_SafetyRack.Close Left Door` (`self.BP_C1_SafetyRack`))
  (`KismetSystemLibrary.Delay` 2.5)
  (`/Game/Chapters/Chapter1/BP/BP_C1_SafetyRack.Hide Rack` (`self.BP_C1_SafetyRack`))
  ;[1 0.04231 0] Instructions
  (`TrainingStepPage.AdvanceProgress` (`self.WBP_Step_Page`))
  ;[0.01405 0 1] ManualVR
  (`ManualVRPluginBPLibrary.Update` "1" "2" "4" 1)
  ;[1 1 1] Pointers
  (`/Game/Chapters/Chapter1/BP/BP_C1_CSM.Enable Pointer` (`self.BP_C1_CSM`))
  (`GameplayStatics.SpawnSound2D` "/Game/Chapters/Steps_Completed/2Comp.2Comp" 1.0 1.0 0.0 null))

(event `Sub 2-4-1a`
  ;[1 1 1] SUB 2
)

(event `Step 3`
  ;[1 1 1] STEP 3
  (`/Game/Chapters/Chapter1/BP/BP_C1_SafetyTable.Set Visible Table` (`self.BP_C1_SafetyTable`))
  (`/Game/Chapters/Chapter1/BP/BP_C1_Harness_Explain.Set Visible Harness` (`self.BP_C1_Harness_Explain`))
  (`/Game/Chapters/Chapter1/BP/BP_C1_Lanyard.Set Visible Lanyard` (`self.BP_C1_Lanyard`))
  (`KismetSystemLibrary.Delay` 0.2)
  (`/Game/Chapters/Chapter1/BP/BP_C1_Harness_Explain.Set 3-1-1 Explain Visible` (`self.BP_C1_Harness_Explain`)))

(event `Sub 3-1-1`
  ;[1 1 1] SUB 3
  (`/Game/Chapters/Chapter1/BP/BP_C1_Harness_Explain.Set 3-1-1 Explain Hidden` (`self.BP_C1_Harness_Explain`))
  (`/Game/Chapters/Chapter1/BP/BP_C1_Harness_Explain.Set 3-2-1 Explain Visible` (`self.BP_C1_Harness_Explain`))
  (`/Game/Chapters/Chapter1/BP/BP_C1_Harness_Explain.Enable Highlight Harness Straps` (`self.BP_C1_Harness_Explain`))
  ;[1 0.04231 0] Instructions
  (`TrainingStepPage.AdvanceProgress` (`self.WBP_Step_Page`))
  ;[0.01405 0 1] ManualVR
  (`ManualVRPluginBPLibrary.Update` "1" "3" "1" 1))

(event `Sub 3-2-1`
  ;[1 1 1] SUB 3
  (`/Game/Chapters/Chapter1/BP/BP_C1_Harness_Explain.Set 3-2-1 Explain Hidden` (`self.BP_C1_Harness_Explain`))
  (`/Game/Chapters/Chapter1/BP/BP_C1_Harness_Explain.Set 3-3-1 Explain Visible` (`self.BP_C1_Harness_Explain`))
  (`/Game/Chapters/Chapter1/BP/BP_C1_Harness_Explain.Enable Highlight Buckles` (`self.BP_C1_Harness_Explain`))
  ;[1 0.04231 0] Instructions
  (`TrainingStepPage.AdvanceProgress` (`self.WBP_Step_Page`))
  ;[0.01405 0 1] ManualVR
  (`ManualVRPluginBPLibrary.Update` "1" "3" "2" 1))

(event `Sub 3-3-1`
  ;[1 1 1] SUB 3
  (`/Game/Chapters/Chapter1/BP/BP_C1_Harness_Explain.Set 3-3-1 Explain Hidden` (`self.BP_C1_Harness_Explain`))
  (`/Game/Chapters/Chapter1/BP/BP_C1_Harness_Explain.Set 3-4-1 Explain Visible` (`self.BP_C1_Harness_Explain`))
  (`/Game/Chapters/Chapter1/BP/BP_C1_Harness_Explain.Enable Highlight Stitches` (`self.BP_C1_Harness_Explain`))
  ;[1 0.04231 0] Instructions
  (`TrainingStepPage.AdvanceProgress` (`self.WBP_Step_Page`))
  ;[0.01405 0 1] ManualVR
  (`ManualVRPluginBPLibrary.Update` "1" "3" "3" 1))

(event `Sub 3-4-1`
  ;[1 1 1] SUB 3
  (`/Game/Chapters/Chapter1/BP/BP_C1_Harness_Explain.Set 3-4-1 Explain Hidden` (`self.BP_C1_Harness_Explain`))
  (`/Game/Chapters/Chapter1/BP/BP_C1_Harness_Explain.Rotate Harness Back` (`self.BP_C1_Harness_Explain`))
  (`/Game/Chapters/Chapter1/BP/BP_C1_Harness_Explain.Set 3-5-1 Explain Visible` (`self.BP_C1_Harness_Explain`))
  (`/Game/Chapters/Chapter1/BP/BP_C1_Harness_Explain.Enable Highlight Backplate` (`self.BP_C1_Harness_Explain`))
  ;[1 0.04231 0] Instructions
  (`TrainingStepPage.AdvanceProgress` (`self.WBP_Step_Page`))
  ;[0.01405 0 1] ManualVR
  (`ManualVRPluginBPLibrary.Update` "1" "3" "4" 1))

(event `Sub 3-5-1`
  ;[1 1 1] SUB 3
  (`/Game/Chapters/Chapter1/BP/BP_C1_Harness_Explain.Set 3-5-1 Explain Hidden` (`self.BP_C1_Harness_Explain`))
  (`/Game/Chapters/Chapter1/BP/BP_C1_Harness_Explain.Rotate Harness Front` (`self.BP_C1_Harness_Explain`))
  (`/Game/Chapters/Chapter1/BP/BP_C1_Harness_Explain.Set Hidden Harness` (`self.BP_C1_Harness_Explain`))
  (`/Game/Chapters/Chapter1/BP/BP_C1_Harness_Grab.Set Visible Harness` (`self.BP_C1_Harness_Grab`))
  ;[1 0.04231 0] Instructions
  (`TrainingStepPage.AdvanceProgress` (`self.WBP_Step_Page`))
  ;[0.01405 0 1] ManualVR
  (`ManualVRPluginBPLibrary.Update` "1" "3" "5" 1)
  ;[1 1 1] Pointers
  (`/Game/Chapters/Chapter1/BP/BP_C1_CSM.Enable Pointer` (`self.BP_C1_CSM`))
  (`GameplayStatics.SpawnSound2D` "/Game/Chapters/Steps_Completed/3Comp.3Comp" 1.0 1.0 0.0 null))

(event `Sub 4-1-1`
  ;[1 1 1] Sub 4
  (`/Game/Chapters/Chapter1/BP/BP_C1_Lanyard.Set 4-1-1 Explain Hidden` (`self.BP_C1_Lanyard`))
  (`KismetSystemLibrary.Delay` 0.2)
  (`/Game/Chapters/Chapter1/BP/BP_C1_Lanyard.Set 4-1-2 Explain Visible` (`self.BP_C1_Lanyard`))
  (`/Game/Chapters/Chapter1/BP/BP_C1_Lanyard.Enable Highlight` (`self.BP_C1_Lanyard`)))

(event `Step 4`
  ;[1 1 1] STEP 4
  (`/Game/Chapters/Chapter1/BP/BP_C1_Lanyard.Set 4-1-1 Explain Visible` (`self.BP_C1_Lanyard`)))

(event `Sub 4-1-2`
  ;[1 1 1] Sub 4
  (`/Game/Chapters/Chapter1/BP/BP_C1_Lanyard.Set 4-1-2 Explain Hidden` (`self.BP_C1_Lanyard`))
  (`KismetSystemLibrary.Delay` 0.2)
  (`/Game/Chapters/Chapter1/BP/BP_C1_Harness_Grab.Rotate Harness Behind` (`self.BP_C1_Harness_Grab`))
  (`/Game/Chapters/Chapter1/BP/BP_C1_Lanyard.Enable Grab Attach` (`self.BP_C1_Lanyard`))
  ;[1 0.04231 0] Instructions
  (`TrainingStepPage.AdvanceProgress` (`self.WBP_Step_Page`))
  ;[0.01405 0 1] ManualVR
  (`ManualVRPluginBPLibrary.Update` "1" "4" "1" 1))

(event `Sub 4-2-1`
  ;[1 1 1] Sub 4
  (`/Game/Chapters/Chapter1/BP/BP_C1_Lanyard.Disable Grab Attach` (`self.BP_C1_Lanyard`))
  (`KismetSystemLibrary.Delay` 0.2)
  (`/Game/Chapters/Chapter1/BP/BP_C1_Harness_Grab.Enable Grab Attach` (`self.BP_C1_Harness_Grab`))
  ;[1 0.04231 0] Instructions
  (`TrainingStepPage.AdvanceProgress` (`self.WBP_Step_Page`))
  ;[0.01405 0 1] ManualVR
  (`ManualVRPluginBPLibrary.Update` "1" "4" "2" 1))

(event `Sub 4-3-1`
  ;[1 1 1] Sub 4
  (`/Game/Chapters/Chapter1/BP/BP_C1_Harness_Grab.Disable Grab Attach` (`self.BP_C1_Harness_Grab`))
  (`/Game/Chapters/Chapter1/BP/BP_C1_Harness_Grab.Set Hidden Harness` (`self.BP_C1_Harness_Grab`))
  (`/Game/Chapters/Chapter1/BP/BP_C1_Lanyard.Set Hidden Lanyard` (`self.BP_C1_Lanyard`))
  (`/Game/Chapters/Chapter1/BP/BP_C1_Avatar.Set Visible Real Harness` (`self.BP_C1_Avatar`))
  ;[1 0.04231 0] Instructions
  (`TrainingStepPage.AdvanceProgress` (`self.WBP_Step_Page`))
  ;[0.01405 0 1] ManualVR
  (`ManualVRPluginBPLibrary.Update` "1" "4" "3" 1)
  ;[1 1 1] Pointers
  (`/Game/Chapters/Chapter1/BP/BP_C1_CSM.Enable Pointer` (`self.BP_C1_CSM`))
  (`GameplayStatics.SpawnSound2D` "/Game/Chapters/Steps_Completed/4Comp.4Comp" 1.0 1.0 0.0 null))

(event `Step 5`
  ;[1 1 1] STEP 5
  (`/Game/Chapters/Chapter1/BP/BP_C1_Avatar.Set 5-1-1 Explain Visible` (`self.BP_C1_Avatar`))
  (`/Game/Chapters/Chapter1/BP/BP_C1_Avatar.Enable Highlight Harness` (`self.BP_C1_Avatar`)))

(event `Sub 5-1-1`
  ;[1 1 1] Sub 5
  (`/Game/Chapters/Chapter1/BP/BP_C1_Avatar.Set 5-1-1 Explain Hidden` (`self.BP_C1_Avatar`))
  (`/Game/Chapters/Chapter1/BP/BP_C1_Avatar.Set 5-1-2 Explain Visible` (`self.BP_C1_Avatar`))
  (`/Game/Chapters/Chapter1/BP/BP_C1_Avatar.Enable Highlight Buckle` (`self.BP_C1_Avatar`)))

(event `Sub 5-1-2`
  ;[1 1 1] Sub 5
  (`/Game/Chapters/Chapter1/BP/BP_C1_Avatar.Set 5-1-2 Explain Hidden` (`self.BP_C1_Avatar`))
  (`/Game/Chapters/Chapter1/BP/BP_C1_Avatar.Rotate Behind` (`self.BP_C1_Avatar`))
  (`/Game/Chapters/Chapter1/BP/BP_C1_Avatar.Set 5-2-1 Explain Visible` (`self.BP_C1_Avatar`))
  ;[1 0.04231 0] Instructions
  (`TrainingStepPage.AdvanceProgress` (`self.WBP_Step_Page`))
  ;[0.01405 0 1] ManualVR
  (`ManualVRPluginBPLibrary.Update` "1" "5" "1" 1))

(event `Sub 5-2-1`
  ;[1 1 1] Sub 5
  (`/Game/Chapters/Chapter1/BP/BP_C1_Avatar.Set 5-2-1 Explain Hidden` (`self.BP_C1_Avatar`))
  (`/Game/Chapters/Chapter1/BP/BP_C1_Avatar.Rotate Forward` (`self.BP_C1_Avatar`))
  (`/Game/Chapters/Chapter1/BP/BP_C1_Avatar.Set 5-2-2 Explain Visible` (`self.BP_C1_Avatar`)))

(event `Sub 5-2-2`
  ;[1 1 1] Sub 5
  (`/Game/Chapters/Chapter1/BP/BP_C1_Avatar.Set 5-2-2 Explain Hidden` (`self.BP_C1_Avatar`))
  ;[1 0.04231 0] Instructions
  (`TrainingStepPage.AdvanceProgress` (`self.WBP_Step_Page`))
  ;[0.01405 0 1] ManualVR
  (`ManualVRPluginBPLibrary.Update` "1" "5" "2" 1)
  ;[1 1 1] Pointers
  (`/Game/Chapters/Chapter1/BP/BP_C1_CSM.Enable Pointer` (`self.BP_C1_CSM`))
  (`GameplayStatics.SpawnSound2D` "/Game/Chapters/Steps_Completed/5Comp.5Comp" 1.0 1.0 0.0 null))

(event `Step 6`
  ;[1 1 1] STEP 6
  (`/Game/Chapters/Chapter1/BP/BP_C1_ToolBag.Set Visible ToolBag` (`self.BP_C1_ToolBag`))
  (`/Game/Chapters/Chapter1/BP/BP_C1_ToolBag.Set 6-1-1 Explain Visible` (`self.BP_C1_ToolBag`)))

(event `Sub 6-1-1`
  ;[1 1 1] Sub 6
  (`/Game/Chapters/Chapter1/BP/BP_C1_ToolBag.Set 6-1-1 Explain Hidden` (`self.BP_C1_ToolBag`))
  (`/Game/Chapters/Chapter1/BP/BP_C1_ToolBag.Enable Grab Attach` (`self.BP_C1_ToolBag`))
  ;[1 0.04231 0] Instructions
  (`TrainingStepPage.AdvanceProgress` (`self.WBP_Step_Page`))
  ;[0.01405 0 1] ManualVR
  (`ManualVRPluginBPLibrary.Update` "1" "6" "1" 1))

(event `Sub 6-2-1`
  ;[1 1 1] Sub 6
  (`/Game/Chapters/Chapter1/BP/BP_C1_ToolBag.Disable Grab Attach` (`self.BP_C1_ToolBag`))
  ;[1 0.04231 0] Instructions
  (`TrainingStepPage.AdvanceProgress` (`self.WBP_Step_Page`))
  ;[0.01405 0 1] ManualVR
  (`ManualVRPluginBPLibrary.Update` "1" "6" "2" 1)
  ;[1 1 1] Pointers
  (`/Game/Chapters/Chapter1/BP/BP_C1_CSM.Enable Pointer` (`self.BP_C1_CSM`))
  (`GameplayStatics.SpawnSound2D` "/Game/Chapters/Steps_Completed/6Comp.6Comp" 1.0 1.0 0.0 null))

(event `Step 7`
  ;[1 1 1] STEP 7
  (`/Game/Chapters/Chapter1/BP/BP_C1_Avatar.Set 7-1-1 Explain Visible` (`self.BP_C1_Avatar`))
  (`/Game/Chapters/Chapter1/BP/BP_C1_SOP_Book.Set Book Visible` (`self.BP_C1_SOP_Book`))
  (`/Game/Chapters/Chapter1/BP/BP_C1_HIRARC_Book.Set Book Visible` (`self.BP_C1_HIRARC_Book`)))

(event `Sub 7-1-1`
  ;[1 1 1] Sub 7
  (`/Game/Chapters/Chapter1/BP/BP_C1_Avatar.Set 7-1-1 Explain Hidden` (`self.BP_C1_Avatar`))
  (`/Game/Chapters/Chapter1/BP/BP_C1_HIRARC_Book.Set 7-2-1 Explain Visible` (`self.BP_C1_HIRARC_Book`))
  ;[1 0.04231 0] Instructions
  (`TrainingStepPage.AdvanceProgress` (`self.WBP_Step_Page`))
  ;[0.01405 0 1] ManualVR
  (`ManualVRPluginBPLibrary.Update` "1" "7" "1" 1))

(event `Sub 7-2-1`
  ;[1 1 1] Sub 7
  (`/Game/Chapters/Chapter1/BP/BP_C1_HIRARC_Book.Set 7-2-1 Explain Hidden` (`self.BP_C1_HIRARC_Book`))
  (`/Game/Chapters/Chapter1/BP/BP_C1_SOP_Book.Set 7-3-1 Explain Visible` (`self.BP_C1_SOP_Book`))
  ;[1 0.04231 0] Instructions
  (`TrainingStepPage.AdvanceProgress` (`self.WBP_Step_Page`))
  ;[0.01405 0 1] ManualVR
  (`ManualVRPluginBPLibrary.Update` "1" "7" "2" 1))

(event `Sub 7-3-1`
  ;[1 1 1] Sub 7
  (`/Game/Chapters/Chapter1/BP/BP_C1_SOP_Book.Set 7-3-1 Explain Hidden` (`self.BP_C1_SOP_Book`))
  ;[1 0.04231 0] Instructions
  (`TrainingStepPage.AdvanceProgress` (`self.WBP_Step_Page`))
  ;[0.01405 0 1] ManualVR
  (`ManualVRPluginBPLibrary.Update` "1" "7" "3" 1)
  ;[1 1 1] Pointers
  (`/Game/Chapters/Chapter1/BP/BP_C1_CSM.Enable Pointer` (`self.BP_C1_CSM`))
  (`GameplayStatics.SpawnSound2D` "/Game/Chapters/Steps_Completed/7Comp.7Comp" 1.0 1.0 0.0 null)
  (`ManualVRPluginBPLibrary.End`))

(fn `UserConstructionScript`)
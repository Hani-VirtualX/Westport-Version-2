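; BP_C5_RTGCrane is the Chapter 5 RTG crane actor, hosting scripted VR steps staged on and around the crane.
; Exposed events show or hide explain and action components per step, whose start or completion callbacks fire once into GM_C5 to advance the chapter.
; Other events teleport the pawn to stair and ladder points, toggle teleporting, play a fall via scripted move, and swap the crane material to show a hole.
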(event `self.ReceiveBeginPlay`
  (`KismetSystemLibrary.Delay` 0.2)
  (bind _returnvalue (`GameplayStatics.GetActorOfClass` "/Game/Chapters/Chapter5/GM_C5.GM_C5_C"))
  (set `self.GM_C5` _returnvalue)
  (bind _returnvalue_2 (`GameplayStatics.GetActorOfClass` "/AzurealXR/Core/BP_Azr_Pawn.BP_Azr_Pawn_C"))
  (set `self.BP_Azr_Pawn` _returnvalue_2))

(event `Teleport To Stair`
  (`Azr_Pawn.TeleportPlayer` (`self.BP_Azr_Pawn`) (`self.Impact Location`) (`self.Input Rotation_0`)))

(event `Set 1-1-1 Explain Visible`
  ; 1-1-1 Explain
  (`Azr_Explain.EnableExplain` (`self.Step1_Explain`)))

(event `Set 1-1-1 Explain Hidden`
  ; 1-1-1 Explain
  (`Azr_Explain.DisableExplain` (`self.Step1_Explain`)))

(event `Teleport To Ladder`
  (`Azr_Pawn.TeleportPlayer` (`self.BP_Azr_Pawn`) (`self.Impact Location_0`) (`self.Input Rotation`)))

(event `self.Step1_Explain.OnExplainCompleted`
  ; 1-1-1 Explain
  (`/Engine/EditorBlueprintResources/StandardMacros.DoOnce` false
    (:`Completed`
      (`/Game/Chapters/Chapter5/GM_C5.Sub 1-1-1` (`self.GM_C5`)))))

(event `Disable Teleport`
  (`/AzurealXR/Core/BP_Azr_Pawn.Disable Teleport` (`self.BP_Azr_Pawn`)))

(event `Teleport Beside Ladder`
  (bind (_impact_location_1_x _impact_location_1_y) (`KismetMathLibrary.BreakVector` (`self.Impact Location_1`)))
  (bind _bp_azr_pawn (`self.BP_Azr_Pawn`))
  (bind (_returnvalue_x _returnvalue_y _returnvalue_z) (`KismetMathLibrary.BreakVector` (`SceneComponent.K2_GetComponentLocation` (`Azr_Pawn.VROrigin` _bp_azr_pawn))))
  (`Azr_Pawn.TeleportPlayer` _bp_azr_pawn (`KismetMathLibrary.MakeVector` _impact_location_1_x _impact_location_1_y _returnvalue_z) (`self.Input Rotation_1`)))

(event `Set 2-1-1 Action Visible`
  ; 2-1-1 Action
  (`Azr_Action.EnableAction` (`self.Azr_Action_2-1-1`)))

(event `Set 2-1-1 Action Hidden`
  ; 2-1-1 Action
  (`Azr_Action.DisableAction` (`self.Azr_Action_2-1-1`)))

(event `Enable Teleport`
  (`/AzurealXR/Core/BP_Azr_Pawn.Enable Teleport` (`self.BP_Azr_Pawn`)))

(event `self.Azr_Action_2-1-1.OnStartButtonPressed`
  ; 2-1-1 Action
  (`/Engine/EditorBlueprintResources/StandardMacros.DoOnce` false
    (:`Completed`
      (`/Game/Chapters/Chapter5/GM_C5.Sub 2-1-a` (`self.GM_C5`)))))

(event `self.Azr_Action_2-1-1.OnCompletedButtonPressed`
  ; 2-1-1 Action
  (`/Engine/EditorBlueprintResources/StandardMacros.DoOnce` false
    (:`Completed`
      (`/Game/Chapters/Chapter5/GM_C5.Sub 2-1-1` (`self.GM_C5`)))))

(event `Show Crane Hole`
  (`PrimitiveComponent.SetMaterial` (`self.WP_RTGCrane_Joined`) 0 "/Game/wesport_Stuff/Assets/RTGCrane/Materials/RTG_Bottom_Inst_Hole.RTG_Bottom_Inst_Hole"))

(event `Hide Crane Hole`
  (`PrimitiveComponent.SetMaterial` (`self.WP_RTGCrane_Joined`) 0 "/Game/wesport_Stuff/Assets/RTGCrane/Materials/RTG_Bottom_Inst.RTG_Bottom_Inst"))

(event `Set 3-1-1 Action Hidden`
  ; 3-1-1 Action
  (`Azr_Action.DisableAction` (`self.Azr_Action_3-1-1`)))

(event `Set 3-1-1 Action Visible`
  ; 3-1-1 Action
  (`Azr_Action.EnableAction` (`self.Azr_Action_3-1-1`)))

(event `self.Azr_Action_3-1-1.OnStartButtonPressed`
  ; 3-1-1 Action
  (`/Engine/EditorBlueprintResources/StandardMacros.DoOnce` false
    (:`Completed`
      (`/Game/Chapters/Chapter5/GM_C5.Sub 3-1-1` (`self.GM_C5`)))))

(event `BP Pawn Fall`
  (`Azr_Pawn.ScriptedMoveTo` (`self.BP_Azr_Pawn`) (-2720.0 4088.0 100.0) (struct :`Yaw` -90.0) 900.0))

(event `Set 3-2-1 Action Visible`
  ; 3-2-1 Action
  (`Azr_Action.EnableAction` (`self.Azr_Action_3-2-1`)))

(event `Set 3-2-1 Action Hidden`
  ; 3-2-1 Action
  (`Azr_Action.DisableAction` (`self.Azr_Action_3-2-1`)))

(event `self.Azr_Action_3-2-1.OnStartButtonPressed`
  ; 3-2-1 Action
  (`/Engine/EditorBlueprintResources/StandardMacros.DoOnce` false
    (:`Completed`
      (`/Game/Chapters/Chapter5/GM_C5.Sub 3-2-1` (`self.GM_C5`)))))

(event `Set 3-3-1 Action Hidden`
  ; 3-3-1 Action
  (`Azr_Action.DisableAction` (`self.Azr_Action_3-3-1`)))

(event `Set 3-3-1 Action Visible`
  ; 3-3-1 Action
  (`Azr_Action.EnableAction` (`self.Azr_Action_3-3-1`))
  (`self.EnablePointer` (`self.Action_Widget3`)))

(event `self.Azr_Action_3-3-1.OnStartButtonPressed`
  ; 3-3-1 Action
  (`/Engine/EditorBlueprintResources/StandardMacros.DoOnce` false
    (:`Completed`
      (`/Game/Chapters/Chapter5/GM_C5.Sub 3-3-1` (`self.GM_C5`)))))

(fn `UserConstructionScript`)
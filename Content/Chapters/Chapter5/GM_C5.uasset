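; Game mode for Chapter 5, a VR training chapter on harness use and fall scenarios at an RTG crane.
; On BeginPlay it sets the chapter number, caches level actors and the step-page widget, and disables teleport until the final sub-step.
; RunStepsOrder advances three steps, each after sequential voice-overs timed by sound duration.
; Sub-step events toggle prompts, drive fall sequences and hooks, advance the widget and record completion through Update.
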(event `self.ReceiveBeginPlay`
  (`KismetSystemLibrary.Delay` 0.2)
  (`|ExecutionSequence`
    (:`then_0`
      (bind _asazr_game_instance (cast `/AzurealXR/Core/Azr_GameInstance` (`GameplayStatics.GetGameInstance`)))
      (set `/AzurealXR/Core/Azr_GameInstance.Chapter Number` 5 _asazr_game_instance))
    (:`then_1`
      (bind _returnvalue (`GameplayStatics.GetActorOfClass` "/Game/Chapters/Chapter5/BP_C5_CSM.BP_C5_CSM_C"))
      (set `self.BP_C5_CSM` _returnvalue))
    (:`then_2`
      (bind _foundwidgets (`WidgetBlueprintLibrary.GetAllWidgetsOfClass` "/Azureal_CSM/WBP_StepPage.WBP_StepPage_C" false))
      (set `self.WBP_Step_Page` (`|GetArrayItem` _foundwidgets)))
    (:`then_3`
      (bind _returnvalue_2 (`GameplayStatics.GetActorOfClass` "/Game/Chapters/Chapter5/BP/BP_C5_RTGCrane.BP_C5_RTGCrane_C"))
      (set `self.BP_C5_RTG_Crane` _returnvalue_2)
      (bind _returnvalue_3 (`GameplayStatics.GetActorOfClass` "/Game/Chapters/Chapter5/BP/BP_C5_LiftSupervisorFall.BP_C5_LiftSupervisorFall_C"))
      (set `self.BP_C5_LiftSupervisorFall` _returnvalue_3)
      (bind _returnvalue_4 (`GameplayStatics.GetActorOfClass` "/Game/Chapters/Chapter5/BP/BP_C5_PlayClimbAnim.BP_C5_PlayClimbAnim_C"))
      (set `self.BP_C5_PlayClimbAnimation` _returnvalue_4)
      (bind _returnvalue_5 (`GameplayStatics.GetActorOfClass` "/AzurealXR/Core/BP_Azr_Pawn.BP_Azr_Pawn_C"))
      (set `self.BP_AZR_Pawn` _returnvalue_5)
      (bind _returnvalue_6 (`GameplayStatics.GetActorOfClass` "/Game/Chapters/Chapter5/BP/BP_C5_LeftHook.BP_C5_LeftHook_C"))
      (set `self.BP_C5_LeftHook` _returnvalue_6)
      (bind _returnvalue_7 (`GameplayStatics.GetActorOfClass` "/Game/Chapters/Chapter5/BP/BP_C5_RightHook.BP_C5_RightHook_C"))
      (set `self.BP_C5_RightHook` _returnvalue_7))
    (:`then_4`
      (`/AzurealXR/Core/BP_Azr_Pawn.Disable Teleport` (`self.BP_AZR_Pawn`)))))

(event `self.RunStepsOrder`
  (bind _result (`/Engine/EditorBlueprintResources/StandardMacros.IncrementInt` (`self.Steps Interger`))
    (:`  `
      (switch `int` _result
        (:`1`
          (bind _returnvalue (`GameplayStatics.SpawnSound2D` "/Game/Chapters/Steps_Num/1.1" 1.0 1.0 0.0 null))
          (`KismetSystemLibrary.Delay` (`SoundBase.Duration` (`AudioComponent.Sound` _returnvalue)))
          (bind _returnvalue_2 (`GameplayStatics.SpawnSound2D` "/Game/Chapters/Chapter5/Audio/Step_Intro/C5-Step1.C5-Step1" 1.0 1.0 0.0 null))
          (`KismetSystemLibrary.Delay` (`SoundBase.Duration` (`AudioComponent.Sound` _returnvalue_2)))
          (`self.Step 1`))
        (:`2`
          (bind _returnvalue_3 (`GameplayStatics.SpawnSound2D` "/Game/Chapters/Steps_Num/2.2" 1.0 1.0 0.0 null))
          (`KismetSystemLibrary.Delay` (`SoundBase.Duration` (`AudioComponent.Sound` _returnvalue_3)))
          (bind _returnvalue_4 (`GameplayStatics.SpawnSound2D` "/Game/Chapters/Chapter5/Audio/Step_Intro/C5-Step2.C5-Step2" 1.0 1.0 0.0 null))
          (`KismetSystemLibrary.Delay` (`SoundBase.Duration` (`AudioComponent.Sound` _returnvalue_4)))
          (`self.Step 2`))
        (:`3`
          (bind _returnvalue_5 (`GameplayStatics.SpawnSound2D` "/Game/Chapters/Steps_Num/3.3" 1.0 1.0 0.0 null))
          (`KismetSystemLibrary.Delay` (`SoundBase.Duration` (`AudioComponent.Sound` _returnvalue_5)))
          (bind _returnvalue_6 (`GameplayStatics.SpawnSound2D` "/Game/Chapters/Chapter5/Audio/Step_Intro/C5-Step3.C5-Step3" 1.0 1.0 0.0 null))
          (`KismetSystemLibrary.Delay` (`SoundBase.Duration` (`AudioComponent.Sound` _returnvalue_6)))
          (`self.Step 3`))))))

(event `Sub 1-1-1`
  ;[1 1 1] SUB 1
  (`/Game/Chapters/Chapter5/BP/BP_C5_RTGCrane.Set 1-1-1 Explain Hidden` (`self.BP_C5_RTG_Crane`))
  ;[1 0.04231 0] Instructions
  (`TrainingStepPage.AdvanceProgress` (`self.WBP_Step_Page`))
  ;[0.01405 0 1] ManualVR
  (`ManualVRPluginBPLibrary.Update` "5" "1" "1" 1)
  ;[1 1 1] Pointers
  (`/Game/Chapters/Chapter5/BP_C5_CSM.Enable Pointer` (`self.BP_C5_CSM`))
  (`GameplayStatics.SpawnSound2D` "/Game/Chapters/Steps_Completed/1Comp.1Comp" 1.0 1.0 0.0 null))

(event `Step 1`
  ;[1 1 1] STEP 1
  (`/AzurealXR/Core/BP_Azr_Pawn.Turn On Harness` (`self.BP_AZR_Pawn`))
  (`/Game/Chapters/Chapter5/BP/BP_C5_RTGCrane.Set 1-1-1 Explain Visible` (`self.BP_C5_RTG_Crane`))
  (`ManualVRPluginBPLibrary.Start`))

(event `Sub 2-1-a`
  ;[1 1 1] SUB 2
  (`/Game/Chapters/Chapter5/BP/BP_C5_LiftSupervisorFall.Spawn Operator` (`self.BP_C5_LiftSupervisorFall`))
  (`/Game/Chapters/Chapter5/BP/BP_C5_LiftSupervisorFall.Enabel Highlight npc` (`self.BP_C5_LiftSupervisorFall`))
  (`/Game/Chapters/Chapter5/BP/BP_C5_PlayClimbAnim.Play Animation Climb` (`self.BP_C5_PlayClimbAnimation`))
  (`/Game/Chapters/Chapter5/BP/BP_C5_LiftSupervisorFall.Play Fall Sound` (`self.BP_C5_LiftSupervisorFall`))
  (`KismetSystemLibrary.Delay` 4.0)
  (`/Game/Chapters/Chapter5/BP/BP_C5_PlayClimbAnim.Pause Animation Climb` (`self.BP_C5_PlayClimbAnimation`)))

(event `Step 2`
  ;[1 1 1] STEP 2
  (`/Game/Chapters/Chapter5/BP/BP_C5_RTGCrane.Set 2-1-1 Action Visible` (`self.BP_C5_RTG_Crane`)))

(event `Sub 2-1-1`
  ;[1 1 1] SUB 2
  (`/Game/Chapters/Chapter5/BP/BP_C5_RTGCrane.Set 2-1-1 Action Hidden` (`self.BP_C5_RTG_Crane`))
  (`/Game/Chapters/Chapter5/BP/BP_C5_LiftSupervisorFall.Set 2-2-1 Explain Visible` (`self.BP_C5_LiftSupervisorFall`))
  ;[1 0.04231 0] Instructions
  (`TrainingStepPage.AdvanceProgress` (`self.WBP_Step_Page`))
  ;[0.01405 0 1] ManualVR
  (`ManualVRPluginBPLibrary.Update` "5" "2" "1" 1))

(event `Sub 2-2-1`
  ;[1 1 1] SUB 2
  (`/Game/Chapters/Chapter5/BP/BP_C5_LiftSupervisorFall.Set 2-2-1 Explain Hidden` (`self.BP_C5_LiftSupervisorFall`))
  (`/Game/Chapters/Chapter5/BP/BP_C5_LiftSupervisorFall.Hide Operator` (`self.BP_C5_LiftSupervisorFall`))
  ;[1 0.04231 0] Instructions
  (`TrainingStepPage.AdvanceProgress` (`self.WBP_Step_Page`))
  ;[0.01405 0 1] ManualVR
  (`ManualVRPluginBPLibrary.Update` "5" "2" "2" 1)
  ;[1 1 1] Pointers
  (`/Game/Chapters/Chapter5/BP_C5_CSM.Enable Pointer` (`self.BP_C5_CSM`))
  (`GameplayStatics.SpawnSound2D` "/Game/Chapters/Steps_Completed/2Comp.2Comp" 1.0 1.0 0.0 null))

(event `Step 3`
  ;[1 1 1] STEP 3
  (`/Game/Chapters/Chapter5/BP/BP_C5_RTGCrane.Set 3-1-1 Action Visible` (`self.BP_C5_RTG_Crane`)))

(event `Sub 3-1-1`
  ;[1 1 1] SUB 3
  (`/Game/Chapters/Chapter5/BP/BP_C5_RTGCrane.Set 3-1-1 Action Hidden` (`self.BP_C5_RTG_Crane`))
  (`/Game/Chapters/Chapter5/BP/BP_C5_LeftHook.Spawn LeftHook` (`self.BP_C5_LeftHook`))
  (`/Game/Chapters/Chapter5/BP/BP_C5_RightHook.Spawn RightHook` (`self.BP_C5_RightHook`))
  (`/Game/Chapters/Chapter5/BP/BP_C5_RTGCrane.Set 3-2-1 Action Visible` (`self.BP_C5_RTG_Crane`))
  ;[1 0.04231 0] Instructions
  (`TrainingStepPage.AdvanceProgress` (`self.WBP_Step_Page`))
  ;[0.01405 0 1] ManualVR
  (`ManualVRPluginBPLibrary.Update` "5" "3" "1" 1))

(event `Sub 3-2-1`
  ;[1 1 1] SUB 3
  (`/Game/Chapters/Chapter5/BP/BP_C5_RTGCrane.BP Pawn Fall` (`self.BP_C5_RTG_Crane`))
  (`/Game/Chapters/Chapter5/BP/BP_C5_RTGCrane.Set 3-2-1 Action Hidden` (`self.BP_C5_RTG_Crane`))
  (`KismetSystemLibrary.Delay` 3.0)
  (`/Game/Chapters/Chapter5/BP/BP_C5_RTGCrane.Set 3-3-1 Action Visible` (`self.BP_C5_RTG_Crane`))
  ;[1 0.04231 0] Instructions
  (`TrainingStepPage.AdvanceProgress` (`self.WBP_Step_Page`))
  ;[0.01405 0 1] ManualVR
  (`ManualVRPluginBPLibrary.Update` "5" "3" "2" 1))

(event `Sub 3-3-1`
  ;[1 1 1] SUB 3
  (`/Game/Chapters/Chapter5/BP/BP_C5_LeftHook.Hide LeftHook` (`self.BP_C5_LeftHook`))
  (`/Game/Chapters/Chapter5/BP/BP_C5_RightHook.Hide RightHook` (`self.BP_C5_RightHook`))
  (`/Game/Chapters/Chapter5/BP/BP_C5_RTGCrane.Set 3-3-1 Action Hidden` (`self.BP_C5_RTG_Crane`))
  (`/AzurealXR/Core/BP_Azr_Pawn.Enable Teleport` (`self.BP_AZR_Pawn`))
  ;[1 0.04231 0] Instructions
  (`TrainingStepPage.AdvanceProgress` (`self.WBP_Step_Page`))
  ;[0.01405 0 1] ManualVR
  (`ManualVRPluginBPLibrary.Update` "5" "3" "3" 1)
  ;[1 1 1] Pointers
  (`/Game/Chapters/Chapter5/BP_C5_CSM.Enable Pointer` (`self.BP_C5_CSM`))
  (`GameplayStatics.SpawnSound2D` "/Game/Chapters/Steps_Completed/3Comp.3Comp" 1.0 1.0 0.0 null)
  (`ManualVRPluginBPLibrary.End`))

(fn `UserConstructionScript`)
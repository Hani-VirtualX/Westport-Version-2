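; BP_C5_CSM is a Chapter 5 Blueprint that handles main menu display, pointer toggling and a teleport to the top of a crane.
; BeginPlay makes the MainMenu component visible without propagating to its children.
; EnablePointer and DisablePointer events forward to same-named functions not defined in this file.
; TeleportToTopCrane moves SceneRoot to a world location with a fixed rotation.
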(event `self.ReceiveBeginPlay`
  (`SceneComponent.SetVisibility` (`self.MainMenu`) true false))

(event `Enable Pointer`
  (`self.EnablePointer` null))

(event `Disable Pointer`
  (`self.DisablePointer`))

(event `Teleport To Top Crane`
  (`SceneComponent.K2_SetWorldLocationAndRotation` (`self.SceneRoot`) (`self.New Location`) (struct :`Yaw` -89.999999) false false))

(fn `UserConstructionScript`)
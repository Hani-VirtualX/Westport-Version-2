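; BP_C2_RTGCrane is the Chapter 2 RTG crane actor, providing explanation steps and player teleport points around its stair and ladder.
; It caches GM_C2 and BP_Azr_Pawn shortly after BeginPlay, then exposes events to toggle two explains, teleport the pawn and enable or disable teleporting.
; Each explain's completion advances the game mode once, through Sub111 or Sub211.
; A material swap on the crane mesh shows or hides a hole.
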(event `self.ReceiveBeginPlay`
  (`KismetSystemLibrary.Delay` 0.2)
  (bind _returnvalue (`GameplayStatics.GetActorOfClass` "/Game/Chapters/Chapter2/Blueprint/GM_C2.GM_C2_C"))
  (set `self.GM_C2` _returnvalue)
  (bind _returnvalue_2 (`GameplayStatics.GetActorOfClass` "/AzurealXR/Core/BP_Azr_Pawn.BP_Azr_Pawn_C"))
  (set `self.BP_Azr_Pawn` _returnvalue_2))

(event `Teleport To Stair`
  (`Azr_Pawn.TeleportPlayer` (`self.BP_Azr_Pawn`) (`self.Impact Location`) (`self.Input Rotation_0`)))

(event `Set 1-1-1 Explain Visible`
  (`Azr_Explain.EnableExplain` (`self.Step1_Explain`)))

(event `Set 1-1-1 Explain Hidden`
  (`Azr_Explain.DisableExplain` (`self.Step1_Explain`)))

(event `Teleport To Ladder`
  (`Azr_Pawn.TeleportPlayer` (`self.BP_Azr_Pawn`) (`self.Impact Location_0`) (`self.Input Rotation`)))

(event `self.Step1_Explain.OnExplainCompleted`
  (`/Engine/EditorBlueprintResources/StandardMacros.DoOnce` false
    (:`Completed`
      (`/Game/Chapters/Chapter2/Blueprint/GM_C2.Sub 1-1-1` (`self.GM_C2`)))))

(event `Set 2-1-1 Explain Visible`
  (`Azr_Explain.EnableExplain` (`self.Step2-1-1_Explain`)))

(event `Set 2-1-1 Explain Hidden`
  (`Azr_Explain.DisableExplain` (`self.Step2-1-1_Explain`)))

(event `Disable Teleport`
  (`/AzurealXR/Core/BP_Azr_Pawn.Disable Teleport` (`self.BP_Azr_Pawn`)))

(event `Teleport Beside Ladder`
  (`Azr_Pawn.TeleportPlayer` (`self.BP_Azr_Pawn`) (`self.Impact Location_1`) (`self.Input Rotation_1`)))

(event `self.Step2-1-1_Explain.OnExplainCompleted`
  (`/Engine/EditorBlueprintResources/StandardMacros.DoOnce` false
    (:`Completed`
      (`/Game/Chapters/Chapter2/Blueprint/GM_C2.Sub 2-1-1` (`self.GM_C2`)))))

(event `Enable Teleport`
  (`/AzurealXR/Core/BP_Azr_Pawn.Enable Teleport` (`self.BP_Azr_Pawn`)))

(event `Show Crane Hole`
  (`PrimitiveComponent.SetMaterial` (`self.WP_RTGCrane_Joined`) 0 "/Game/wesport_Stuff/Assets/RTGCrane/Materials/RTG_Bottom_Inst_Hole.RTG_Bottom_Inst_Hole"))

(event `Hide Crane Hole`
  (`PrimitiveComponent.SetMaterial` (`self.WP_RTGCrane_Joined`) 0 "/Game/wesport_Stuff/Assets/RTGCrane/Materials/RTG_Bottom_Inst.RTG_Bottom_Inst"))

(fn `UserConstructionScript`)
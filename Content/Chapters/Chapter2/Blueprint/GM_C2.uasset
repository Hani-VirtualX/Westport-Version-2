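; Game mode for Chapter 2 of a VR RTG crane training, sequencing narrated procedure steps.
; BeginPlay sets the chapter number and caches the crane, operator, climb-animation, CSM and step-page references.
; RunStepsOrder increments a step counter and plays voice-overs before each step; step 3 is only stubbed.
; Sub-step events swap explanation panels, advance a ladder-climb animation using timed play/pause, and record completion, re-enabling the CSM pointer when steps finish.
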(event `self.ReceiveBeginPlay`
  (`KismetSystemLibrary.Delay` 0.2)
  (`|ExecutionSequence`
    (:`then_0`
      (bind _asazr_game_instance (cast `/AzurealXR/Core/Azr_GameInstance` (`GameplayStatics.GetGameInstance`)))
      (set `/AzurealXR/Core/Azr_GameInstance.Chapter Number` 2 _asazr_game_instance))
    (:`then_1`
      (bind _returnvalue (`GameplayStatics.GetActorOfClass` "/Game/Chapters/Chapter2/Blueprint/BP_C2_CSM.BP_C2_CSM_C"))
      (set `self.BP_C2_CSM` _returnvalue))
    (:`then_2`
      (bind _foundwidgets (`WidgetBlueprintLibrary.GetAllWidgetsOfClass` "/Azureal_CSM/WBP_StepPage.WBP_StepPage_C" false))
      (set `self.WBP_Step_Page` (`|GetArrayItem` _foundwidgets)))
    (:`then_3`
      (bind _returnvalue_2 (`GameplayStatics.GetActorOfClass` "/Game/Chapters/Chapter2/Blueprint/BP_C2_RTGCrane.BP_C2_RTGCrane_C"))
      (set `self.BP_C2_RTGCrane` _returnvalue_2)
      (bind _returnvalue_3 (`GameplayStatics.GetActorOfClass` "/Game/Chapters/Chapter2/Blueprint/BP_TestCraneOperator.BP_TestCraneOperator_C"))
      (set `self.BP_TestCraneOperator` _returnvalue_3)
      (bind _returnvalue_4 (`GameplayStatics.GetActorOfClass` "/Game/Chapters/Chapter2/Blueprint/BP_PlayClimbAnimation.BP_PlayClimbAnimation_C"))
      (set `self.BP_PlayClimbAnimation` _returnvalue_4))
    (:`then_4`
      ;[1 1 1] STEP 2
      (`KismetSystemLibrary.Delay` 3.0))))

(event `StepSequencerInterface.RunStepsOrder`
  (bind _result (`/Engine/EditorBlueprintResources/StandardMacros.IncrementInt` (`self.Steps Interger`))
    (:`  `
      (switch `int` _result
        (:`1`
          (bind _returnvalue (`GameplayStatics.SpawnSound2D` "/Game/Chapters/Steps_Num/1.1" 1.0 1.0 0.0 null))
          (`KismetSystemLibrary.Delay` (`SoundBase.Duration` (`AudioComponent.Sound` _returnvalue)))
          (bind _returnvalue_2 (`GameplayStatics.SpawnSound2D` "/Game/Chapters/Chapter2/Audio/Wes_C2/Step_Intro/C2_Step1.C2_Step1" 1.0 1.0 0.0 null))
          (`KismetSystemLibrary.Delay` (`SoundBase.Duration` (`AudioComponent.Sound` _returnvalue_2)))
          (`self.Step 1`))
        (:`2`
          (bind _returnvalue_3 (`GameplayStatics.SpawnSound2D` "/Game/Chapters/Steps_Num/2.2" 1.0 1.0 0.0 null))
          (`KismetSystemLibrary.Delay` (`SoundBase.Duration` (`AudioComponent.Sound` _returnvalue_3)))
          (bind _returnvalue_4 (`GameplayStatics.SpawnSound2D` "/Game/Chapters/Chapter2/Audio/Wes_C2/Step_Intro/C2-Step2.C2-Step2" 1.0 1.0 0.0 null))
          (`KismetSystemLibrary.Delay` (`SoundBase.Duration` (`AudioComponent.Sound` _returnvalue_4)))
          (`self.Step 2`))
        (:`3`
          (bind _returnvalue_5 (`GameplayStatics.SpawnSound2D` "/Game/Chapters/Steps_Num/3.3" 1.0 1.0 0.0 null))
          (`KismetSystemLibrary.Delay` (`SoundBase.Duration` (`AudioComponent.Sound` _returnvalue_5)))
          (bind _returnvalue_6 (`GameplayStatics.SpawnSound2D` null 1.0 1.0 0.0 null))
          (`KismetSystemLibrary.Delay` (`SoundBase.Duration` (`AudioComponent.Sound` _returnvalue_6))))))))

(event `Sub 1-1-1`
  ;[1 1 1] SUB 1
  (`/Game/Chapters/Chapter2/Blueprint/BP_C2_RTGCrane.Set 1-1-1 Explain Hidden` (`self.BP_C2_RTGCrane`))
  ;[1 0.04231 0] Instructions
  (`TrainingStepPage.AdvanceProgress` (`self.WBP_Step_Page`))
  ;[0.01405 0 1] ManualVR
  (`ManualVRPluginBPLibrary.Update` "2" "1" "1" 1)
  ;[1 1 1] Pointers
  (`/Game/Chapters/Chapter2/Blueprint/BP_C2_CSM.Enable Pointer` (`self.BP_C2_CSM`))
  (`GameplayStatics.SpawnSound2D` "/Game/Chapters/Steps_Completed/1Comp.1Comp" 1.0 1.0 0.0 null))

(event `Step 1`
  ;[1 1 1] STEP 1
  (`/Game/Chapters/Chapter2/Blueprint/BP_C2_RTGCrane.Set 1-1-1 Explain Visible` (`self.BP_C2_RTGCrane`)))

(event `Step 2`
  ;[1 1 1] STEP 2
  (`/Game/Chapters/Chapter2/Blueprint/BP_C2_RTGCrane.Set 2-1-1 Explain Visible` (`self.BP_C2_RTGCrane`)))

(event `Sub 2-1-1`
  ;[1 1 1] SUB 2
  (`/Game/Chapters/Chapter2/Blueprint/BP_C2_RTGCrane.Set 2-1-1 Explain Hidden` (`self.BP_C2_RTGCrane`))
  (`KismetSystemLibrary.Delay` 0.2)
  (`/Game/Chapters/Chapter2/Blueprint/BP_TestCraneOperator.Set 2-2-1 Explain Visible` (`self.BP_TestCraneOperator`))
  (`/Game/Chapters/Chapter2/Blueprint/BP_TestCraneOperator.Spawn Operator` (`self.BP_TestCraneOperator`))
  (`/Game/Chapters/Chapter2/Blueprint/BP_PlayClimbAnimation.Play Animation Climb` (`self.BP_PlayClimbAnimation`))
  (`KismetSystemLibrary.Delay` 0.1)
  (`/Game/Chapters/Chapter2/Blueprint/BP_PlayClimbAnimation.Pause Animation Climb` (`self.BP_PlayClimbAnimation`))
  (`/Game/Chapters/Chapter2/Blueprint/BP_C2_RTGCrane.Teleport Beside Ladder` (`self.BP_C2_RTGCrane`))
  (`/Game/Chapters/Chapter2/Blueprint/BP_C2_RTGCrane.Disable Teleport` (`self.BP_C2_RTGCrane`))
  ;[1 0.04231 0] Instructions
  (`TrainingStepPage.AdvanceProgress` (`self.WBP_Step_Page`))
  ;[0.01405 0 1] ManualVR
  (`ManualVRPluginBPLibrary.Update` "2" "2" "1" 1))

(event `Sub 2-2-1`
  ;[1 1 1] SUB 2
  (`/Game/Chapters/Chapter2/Blueprint/BP_TestCraneOperator.Set 2-2-1 Explain Hidden` (`self.BP_TestCraneOperator`))
  (`KismetSystemLibrary.Delay` 0.5)
  (`/Game/Chapters/Chapter2/Blueprint/BP_TestCraneOperator.Set 2-2-2 Explain Visible` (`self.BP_TestCraneOperator`)))

(event `Sub 2-2-2`
  ;[1 1 1] SUB 2
  (`/Game/Chapters/Chapter2/Blueprint/BP_TestCraneOperator.Set 2-2-2 Explain Hidden` (`self.BP_TestCraneOperator`))
  (`KismetSystemLibrary.Delay` 0.5)
  (`/Game/Chapters/Chapter2/Blueprint/BP_TestCraneOperator.Set 2-2-3 Explain Visible` (`self.BP_TestCraneOperator`))
  (`/Game/Chapters/Chapter2/Blueprint/BP_PlayClimbAnimation.Play Animation Climb` (`self.BP_PlayClimbAnimation`))
  (`KismetSystemLibrary.Delay` 3.0)
  (`/Game/Chapters/Chapter2/Blueprint/BP_PlayClimbAnimation.Pause Animation Climb` (`self.BP_PlayClimbAnimation`)))

(event `Sub 2-2-3`
  ;[1 1 1] SUB 2
  (`/Game/Chapters/Chapter2/Blueprint/BP_TestCraneOperator.Set 2-2-3 Explain Hidden` (`self.BP_TestCraneOperator`))
  (`KismetSystemLibrary.Delay` 0.5)
  (`/Game/Chapters/Chapter2/Blueprint/BP_TestCraneOperator.Set 2-2-4 Explain Visible` (`self.BP_TestCraneOperator`))
  (`/Game/Chapters/Chapter2/Blueprint/BP_PlayClimbAnimation.Play Animation Climb` (`self.BP_PlayClimbAnimation`))
  (`KismetSystemLibrary.Delay` 4.0)
  (`/Game/Chapters/Chapter2/Blueprint/BP_PlayClimbAnimation.Pause Animation Climb` (`self.BP_PlayClimbAnimation`)))

(event `Sub 2-2-4`
  ;[1 1 1] SUB 2
  (`/Game/Chapters/Chapter2/Blueprint/BP_TestCraneOperator.Set 2-2-4 Explain Hidden` (`self.BP_TestCraneOperator`))
  (`KismetSystemLibrary.Delay` 0.5)
  (`/Game/Chapters/Chapter2/Blueprint/BP_TestCraneOperator.Set 2-2-5 Explain Visible` (`self.BP_TestCraneOperator`))
  (`/Game/Chapters/Chapter2/Blueprint/BP_PlayClimbAnimation.Play Animation Climb` (`self.BP_PlayClimbAnimation`))
  (`KismetSystemLibrary.Delay` 2.0)
  (`/Game/Chapters/Chapter2/Blueprint/BP_PlayClimbAnimation.Pause Animation Climb` (`self.BP_PlayClimbAnimation`)))

(event `Sub 2-2-5`
  ;[1 1 1] SUB 2
  (`/Game/Chapters/Chapter2/Blueprint/BP_TestCraneOperator.Set 2-2-5 Explain Hidden` (`self.BP_TestCraneOperator`))
  (`KismetSystemLibrary.Delay` 0.5)
  (`/Game/Chapters/Chapter2/Blueprint/BP_TestCraneOperator.Set 2-2-6 Explain Visible` (`self.BP_TestCraneOperator`))
  (`/Game/Chapters/Chapter2/Blueprint/BP_PlayClimbAnimation.Play Animation Climb` (`self.BP_PlayClimbAnimation`))
  (`KismetSystemLibrary.Delay` 15.0)
  (`/Game/Chapters/Chapter2/Blueprint/BP_PlayClimbAnimation.Pause Animation Climb` (`self.BP_PlayClimbAnimation`)))

(event `Sub 2-2-6`
  ;[1 1 1] SUB 2
  (`/Game/Chapters/Chapter2/Blueprint/BP_TestCraneOperator.Set 2-2-6 Explain Hidden` (`self.BP_TestCraneOperator`))
  (`KismetSystemLibrary.Delay` 0.5)
  (`/Game/Chapters/Chapter2/Blueprint/BP_TestCraneOperator.Set 2-2-7 Explain Visible` (`self.BP_TestCraneOperator`)))

(event `Sub 2-2-7`
  ;[1 1 1] SUB 2
  (`/Game/Chapters/Chapter2/Blueprint/BP_TestCraneOperator.Set 2-2-7 Explain Hidden` (`self.BP_TestCraneOperator`))
  (`/Game/Chapters/Chapter2/Blueprint/BP_TestCraneOperator.Hide Operator` (`self.BP_TestCraneOperator`))
  ;[1 0.04231 0] Instructions
  (`TrainingStepPage.AdvanceProgress` (`self.WBP_Step_Page`))
  ;[0.01405 0 1] ManualVR
  (`ManualVRPluginBPLibrary.Update` "2" "2" "2" 1)
  ;[1 1 1] Pointers
  (`/Game/Chapters/Chapter2/Blueprint/BP_C2_CSM.Enable Pointer` (`self.BP_C2_CSM`))
  (`GameplayStatics.SpawnSound2D` "/Game/Chapters/Steps_Completed/2Comp.2Comp" 1.0 1.0 0.0 null))

(fn `UserConstructionScript`)
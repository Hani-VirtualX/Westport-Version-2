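; Left safety-lanyard hook for the Chapter 2 VR ladder climb, which the player grabs and attaches to hook points.
; On BeginPlay it caches level actors, hides itself and connects its cable to the pawn's lanyard.
; Events toggle VX_Grab attachment with ghost targets at attach point 1 or 3, and show, hide or reset the hook.
; On attach, flag-gated checks notify GM_C2 of substep 2-3-1 or 2-3-5.
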(event `self.ReceiveBeginPlay`
  (`KismetSystemLibrary.Delay` 0.2)
  (`|ExecutionSequence`
    (:`then_0`
      (bind _returnvalue (`GameplayStatics.GetActorOfClass` "/Game/Chapters/Chapter2/Blueprint/BP_ClimbLadder/BP_Hook_AttachPoint_1.BP_Hook_AttachPoint_1_C"))
      (set `self.BP Bar 1` _returnvalue)
      (bind _returnvalue_2 (`GameplayStatics.GetActorOfClass` "/Game/Chapters/Chapter2/Blueprint/BP_ClimbLadder/BP_Hook_AttachPoint_2.BP_Hook_AttachPoint_2_C"))
      (set `self.BP Bar 2` _returnvalue_2)
      (bind _returnvalue_3 (`GameplayStatics.GetActorOfClass` "/Game/Chapters/Chapter2/Blueprint/BP_ClimbLadder/BP_GrabPole.BP_GrabPole_C"))
      (set `self.BP Grab Pole` _returnvalue_3)
      (bind _returnvalue_4 (`GameplayStatics.GetActorOfClass` "/Game/Chapters/Chapter2/Blueprint/BP_ClimbLadder/BP_GrabPole3.BP_GrabPole3_C"))
      (set `self.BP Grab Pole 3` _returnvalue_4)
      (bind _returnvalue_5 (`GameplayStatics.GetActorOfClass` "/Game/Chapters/Chapter2/Blueprint/BP_ClimbLadder/BP_Hook_AttachPoint_3.BP_Hook_AttachPoint_3_C"))
      (set `self.BP Hook Attach Point 3` _returnvalue_5)
      (bind _returnvalue_6 (`GameplayStatics.GetActorOfClass` "/Game/Chapters/Chapter2/Blueprint/GM_C2.GM_C2_C"))
      (set `self.GM_C2` _returnvalue_6)
      (bind _returnvalue_7 (`GameplayStatics.GetActorOfClass` "/Game/AFCore/Blueprints/Pawn/VR/BP_Pawn_VR.BP_Pawn_VR_C"))
      (set `self.BP Pawn VR` _returnvalue_7)
      (`self.Hide Hook Left`))
    (:`then_1`
      (`CableComponent.SetAttachEndTo` (`self.Cable`) (`GameplayStatics.GetPlayerPawn` 0) "WP_SafetyLanyard" "None"))))

(event `Allow 2-3-1`
  (set `self.2-3-1` true))

(event `Enable Grab Attach`
  (`/Game/Azureal_Template/VX_Grab/VX_Grab.Set Grab Attach` (`self.VX_Grab`) (`self.Hook`) (`self.BP_Grab_Indicator`) (`self.Widget`) (`/Game/Chapters/Chapter2/Blueprint/BP_ClimbLadder/BP_Hook_AttachPoint_1.Hook` (`self.BP Bar 1`)) "AttachWidget" true "NewEnumerator0" "NewEnumerator7" "NewEnumerator1" "NewEnumerator0"))

(event `Disable Grab Attach`
  (`/Game/Azureal_Template/VX_Grab/VX_Grab.Set Grab Attach` (`self.VX_Grab`) (`self.Hook`) (`self.BP_Grab_Indicator`) (`self.Widget`) (`/Game/Chapters/Chapter2/Blueprint/BP_ClimbLadder/BP_Hook_AttachPoint_1.Hook` (`self.BP Bar 1`)) "AttachWidget" false "NewEnumerator4" "NewEnumerator6" "NewEnumerator4" "NewEnumerator4")
  (set `/Game/AFCore/Blueprints/Pawn/VR/BP_Pawn_VR.Force Release` false (`self.BP Pawn VR`)))

(event `Disable 2-3-1`
  (set `self.2-3-1` false))

(event `Allow 2-3-5`
  (set `self.2-3-5` true))

(event `self.VX_Grab.Grab Object - Attached`
  (params (`Comp Connector Achor` :type "/Game/AFCore/Blueprints/Components/Snapping/Comp_Connector_Anchor Object Reference"))
  (`|ExecutionSequence`
    (:`then_0`
      (if (`self.2-3-1`)
        (`/Game/Chapters/Chapter2/Blueprint/GM_C2.Sub 2-3-1` (`self.GM_C2`))))
    (:`then_1`
      (if (`self.2-3-5`)
        (`/Game/Chapters/Chapter2/Blueprint/GM_C2.Sub 2-3-5` (`self.GM_C2`))))))

(event `Disable 2-3-5`
  (set `self.2-3-5` false))

(event `Disable Grab Attach 2`
  (`/Game/Azureal_Template/VX_Grab/VX_Grab.Set Grab Attach` (`self.VX_Grab`) (`self.Hook`) (`self.BP_Grab_Indicator`) (`self.Widget`) (`/Game/Chapters/Chapter2/Blueprint/BP_ClimbLadder/BP_Hook_AttachPoint_3.Hook` (`self.BP Hook Attach Point 3`)) "AttachWidget" false "NewEnumerator4" "NewEnumerator6" "NewEnumerator4" "NewEnumerator4"))

(event `Enable Grab Attach 2`
  (set `self.2-3-5` true)
  (`/Game/Azureal_Template/VX_Grab/VX_Grab.Set Grab Attach` (`self.VX_Grab`) (`self.Hook`) (`self.BP_Grab_Indicator`) (`self.Widget`) (`/Game/Chapters/Chapter2/Blueprint/BP_ClimbLadder/BP_Hook_AttachPoint_3.Hook` (`self.BP Hook Attach Point 3`)) "AttachWidget" true "NewEnumerator0" "NewEnumerator7" "NewEnumerator1" "NewEnumerator0"))

(event `Hide Hook Left`
  (`SceneComponent.SetHiddenInGame` (`self.Hook`) true false)
  (`SceneComponent.SetHiddenInGame` (`self.Cable`) true false))

(event `Reset Hook Left`
  (`SceneComponent.K2_SetWorldLocationAndRotation` (`self.DefaultSceneRoot`) (`self.New Location`) (`self.New Rotation`) false false))

(event `Spawn Hook Left`
  (`SceneComponent.SetHiddenInGame` (`self.Hook`) false false)
  (`SceneComponent.SetHiddenInGame` (`self.Cable`) false false))

(fn `UserConstructionScript`)
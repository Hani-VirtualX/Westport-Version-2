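; BP_C2_CSM is a Chapter 2 actor that hosts the MainMenu component and can relocate it during play.
; On BeginPlay it shows MainMenu without propagating visibility to children and enables pointer interaction for it.
; The MoveMenuUpstairs event sets the root's world location and rotation, and a separate EnablePointer event re-applies pointer interaction on demand.
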(event `self.ReceiveBeginPlay`
  (`SceneComponent.SetVisibility` (`self.MainMenu`) true false)
  (`self.EnablePointer` (`self.MainMenu`)))

(event `Move Menu Upstairs`
  (`SceneComponent.K2_SetWorldLocationAndRotation` (`self.Root`) (`self.New Location`) (`self.New Rotation`) false false))

(event `Enable Pointer`
  (`self.EnablePointer` (`self.MainMenu`)))

(fn `UserConstructionScript`)
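; Chapter 1 game mode that sequences an eight-step interactive RMU switchgear procedure covering the circuit switch, caution signs and earth switch.
; After a short BeginPlay delay, it caches the step page widget and interactable actors.
; RunStepsOrder increments a counter to start each step.
; Sub-step events, with no callers here, switch off the finished interaction, enable the next interaction or explanation, and usually advance the step page's progress.
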(event `self.ReceiveBeginPlay`
  (`KismetSystemLibrary.Delay` 0.2)
  (`|ExecutionSequence`
    (:`then_2`
      (bind _foundwidgets (`WidgetBlueprintLibrary.GetAllWidgetsOfClass` "/Game/Test_Chapter/CSM/WBP_StepPage.WBP_StepPage_C" false))
      (set `self.WBP_Step_Page` (`|GetArrayItem` _foundwidgets)))
    (:`then_3`
      (bind _returnvalue (`GameplayStatics.GetActorOfClass` "/Game/Test_Chapter/BP/BP_C1_Step1_Widg.BP_C1_Step1_Widg_C"))
      (set `self.BP_C1_Step1_Widg` _returnvalue)
      (bind _returnvalue_2 (`GameplayStatics.GetActorOfClass` "/Game/Test_Chapter/BP/BP_C1_VCBRoom_Door.BP_C1_VCBRoom_Door_C"))
      (set `self.BP_C1_VCBRoom_Door` _returnvalue_2)
      (bind _returnvalue_3 (`GameplayStatics.GetActorOfClass` "/Game/Test_Chapter/BP/BP_C1_Step2_Widg.BP_C1_Step2_Widg_C"))
      (set `self.BP_C1_Step2_Widg` _returnvalue_3)
      (bind _returnvalue_4 (`GameplayStatics.GetActorOfClass` "/Game/Test_Chapter/BP/BP_C1_RMU_HVI.BP_C1_RMU_HVI_C"))
      (set `self.BP_C1_RMU_HVI` _returnvalue_4)
      (bind _returnvalue_5 (`GameplayStatics.GetActorOfClass` "/Game/Test_Chapter/BP/BP_C1_Circ_Switch_Knob.BP_C1_Circ_Switch_Knob_C"))
      (set `self.BP_C1_Circ_Switch_Knob` _returnvalue_5)
      (bind _returnvalue_6 (`GameplayStatics.GetActorOfClass` "/Game/Test_Chapter/BP/BP_C1_OperatingHandle.BP_C1_OperatingHandle_C"))
      (set `self.BP_C1_OperatingHandle` _returnvalue_6)
      (bind _returnvalue_7 (`GameplayStatics.GetActorOfClass` "/Game/Test_Chapter/BP/BP_C1_Caution_Circuit.BP_C1_Caution_Circuit_C"))
      (set `self.BP_C1_Caution_Circuit` _returnvalue_7)
      (bind _returnvalue_8 (`GameplayStatics.GetActorOfClass` "/Game/Test_Chapter/BP/BP_C1_Caution_Earthing.BP_C1_Caution_Earthing_C"))
      (set `self.BP_C1_Caution_Earthing` _returnvalue_8)
      (bind _returnvalue_9 (`GameplayStatics.GetActorOfClass` "/Game/Test_Chapter/BP/BP_C1_Earth_Switch_Knob.BP_C1_Earth_Switch_Knob_C"))
      (set `self.BP_C1_Earth_Switch_Knob` _returnvalue_9))
    (:`then_4`
      (`KismetSystemLibrary.Delay` 3.0))))

(event `StepSequencerInterface.RunStepsOrder`
  (bind _result (`/Engine/EditorBlueprintResources/StandardMacros.IncrementInt` (`self.Steps Interger`))
    (:`  `
      (switch `int` _result
        (:`1`
          (`self.Step 1`))
        (:`2`
          (`self.Step 2`))
        (:`3`
          (`self.Step 3`))
        (:`4`
          (`self.Step 4`))
        (:`5`
          (`self.Step 5`))
        (:`6`
          (`self.Step 6`))
        (:`7`
          (`self.Step 7`))
        (:`8`
          (`self.Step 8`))))))

(event `Step 1`
  ;[1 1 1] STEP 1
  (`/Game/Test_Chapter/BP/BP_C1_Step1_Widg.Set 1-1-1 Explain Enable` (`self.BP_C1_Step1_Widg`)))

(event `Sub 1-1-1`
  ;[1 1 1] SUB 1
  (`/Game/Test_Chapter/BP/BP_C1_Step1_Widg.Set 1-1-1 Explain Disable` (`self.BP_C1_Step1_Widg`))
  ;[1 0.04231 0] Instructions
  (`TrainingStepPage.AdvanceProgress` (`self.WBP_Step_Page`)))

(event `Sub 2-1-1`
  ;[1 1 1] SUB 2
  (`/Game/Test_Chapter/BP/BP_C1_VCBRoom_Door.Teleport To RMU` (`self.BP_C1_VCBRoom_Door`))
  (`/Game/Test_Chapter/BP/BP_C1_Step2_Widg.Set Explain Widget Enable` (`self.BP_C1_Step2_Widg`))
  ;[1 0.04231 0] Instructions
  (`TrainingStepPage.AdvanceProgress` (`self.WBP_Step_Page`)))

(event `Step 2`
  ;[1 1 1] STEP 1
  (`/Game/Test_Chapter/BP/BP_C1_VCBRoom_Door.Set 2-1 Action Visible` (`self.BP_C1_VCBRoom_Door`)))

(event `Sub 2-2-1`
  ;[1 1 1] SUB 2
  (`/Game/Test_Chapter/BP/BP_C1_Step2_Widg.Set Explain Widget Disable` (`self.BP_C1_Step2_Widg`))
  ;[1 0.04231 0] Instructions
  (`TrainingStepPage.AdvanceProgress` (`self.WBP_Step_Page`)))

(event `Sub 3-1-1`
  ;[1 1 1] SUB 3
  (`/Game/Test_Chapter/BP/BP_C1_RMU_HVI.Disable Select` (`self.BP_C1_RMU_HVI`))
  (`/Game/Test_Chapter/BP/BP_C1_RMU_HVI.Light Up` (`self.BP_C1_RMU_HVI`))
  (`/Game/Test_Chapter/BP/BP_C1_RMU_HVI.Set 3-1-2 Explain Visible` (`self.BP_C1_RMU_HVI`)))

(event `Step 3`
  ;[1 1 1] STEP 3
  (`/Game/Test_Chapter/BP/BP_C1_RMU_HVI.Enable Select` (`self.BP_C1_RMU_HVI`))
  (`/Game/Test_Chapter/BP/BP_C1_RMU_HVI.Enable 3-1-1` (`self.BP_C1_RMU_HVI`)))

(event `Sub 3-1-2`
  ;[1 1 1] SUB 3
  (`/Game/Test_Chapter/BP/BP_C1_RMU_HVI.Set 3-1-2 Explain Hidden` (`self.BP_C1_RMU_HVI`))
  ;[1 0.04231 0] Instructions
  (`TrainingStepPage.AdvanceProgress` (`self.WBP_Step_Page`)))

(event `Sub 4-1-1`
  ;[1 1 1] SUB 4
  (`/Game/Test_Chapter/BP/BP_C1_Circ_Switch_Knob.Disable Touch` (`self.BP_C1_Circ_Switch_Knob`))
  (`/Game/Test_Chapter/BP/BP_C1_Circ_Switch_Knob.OpenKnob` (`self.BP_C1_Circ_Switch_Knob`))
  (`/Game/Test_Chapter/BP/BP_C1_OperatingHandle.Set Grab Attach 4-2-1 Enable` (`self.BP_C1_OperatingHandle`))
  ;[1 0.04231 0] Instructions
  (`TrainingStepPage.AdvanceProgress` (`self.WBP_Step_Page`)))

(event `Step 4`
  ;[1 1 1] STEP 4
  (`/Game/Test_Chapter/BP/BP_C1_Circ_Switch_Knob.Enable Touch` (`self.BP_C1_Circ_Switch_Knob`)))

(event `Sub 4-2-1`
  ;[1 1 1] SUB 4
  (`/Game/Test_Chapter/BP/BP_C1_OperatingHandle.Set Grab Attach 4-2-1 Disable` (`self.BP_C1_OperatingHandle`))
  (`KismetSystemLibrary.Delay` 0.5)
  (`/Game/Test_Chapter/BP/BP_C1_OperatingHandle.Set Latch Enable` (`self.BP_C1_OperatingHandle`))
  (`/Game/Test_Chapter/BP/BP_C1_OperatingHandle.Enable 4-3-1` (`self.BP_C1_OperatingHandle`))
  ;[1 0.04231 0] Instructions
  (`TrainingStepPage.AdvanceProgress` (`self.WBP_Step_Page`)))

(event `Sub 4-3-1`
  ;[1 1 1] SUB 4
  (`/Game/Test_Chapter/BP/BP_C1_OperatingHandle.Disable 4-3-1` (`self.BP_C1_OperatingHandle`))
  (`/Game/Test_Chapter/BP/BP_C1_OperatingHandle.Set Latch Disable` (`self.BP_C1_OperatingHandle`))
  (`/Game/Test_Chapter/BP/BP_C1_OperatingHandle.Enable Grab Remove` (`self.BP_C1_OperatingHandle`))
  (`/Game/Test_Chapter/BP/BP_C1_OperatingHandle.Enable 4-4-1` (`self.BP_C1_OperatingHandle`))
  ;[1 0.04231 0] Instructions
  (`TrainingStepPage.AdvanceProgress` (`self.WBP_Step_Page`)))

(event `Sub 4-4-1`
  ;[1 1 1] SUB 4
  (`/Game/Test_Chapter/BP/BP_C1_OperatingHandle.Disable Grab Remove` (`self.BP_C1_OperatingHandle`))
  (`/Game/Test_Chapter/BP/BP_C1_OperatingHandle.Disable 4-4-1` (`self.BP_C1_OperatingHandle`))
  (`/Game/Test_Chapter/BP/BP_C1_RMU_HVI.Enable Select` (`self.BP_C1_RMU_HVI`))
  (`/Game/Test_Chapter/BP/BP_C1_RMU_HVI.Enable 4-5-1` (`self.BP_C1_RMU_HVI`))
  (`/Game/Test_Chapter/BP/BP_C1_Circ_Switch_Knob.CloseKnob` (`self.BP_C1_Circ_Switch_Knob`))
  ;[1 0.04231 0] Instructions
  (`TrainingStepPage.AdvanceProgress` (`self.WBP_Step_Page`)))

(event `Sub 4-5-1`
  ;[1 1 1] SUB 4
  (`/Game/Test_Chapter/BP/BP_C1_RMU_HVI.Disable 4-5-1` (`self.BP_C1_RMU_HVI`))
  (`/Game/Test_Chapter/BP/BP_C1_RMU_HVI.Disable Select` (`self.BP_C1_RMU_HVI`))
  (`/Game/Test_Chapter/BP/BP_C1_RMU_HVI.Set 4-5-2 Explain Visible` (`self.BP_C1_RMU_HVI`)))

(event `Sub 4-5-2`
  ;[1 1 1] SUB 4
  (`/Game/Test_Chapter/BP/BP_C1_RMU_HVI.Set 4-5-2 Explain Hidden` (`self.BP_C1_RMU_HVI`))
  ;[1 0.04231 0] Instructions
  (`TrainingStepPage.AdvanceProgress` (`self.WBP_Step_Page`)))

(event `Step 5`
  ;[1 1 1] STEP 5
  (`/Game/Test_Chapter/BP/BP_C1_Caution_Circuit.Set Grab Attach Enable` (`self.BP_C1_Caution_Circuit`)))

(event `Sub 5-1-1`
  ;[1 1 1] SUB 5
  (`/Game/Test_Chapter/BP/BP_C1_Caution_Circuit.Set Grab Attach Disable` (`self.BP_C1_Caution_Circuit`))
  (`/Game/Test_Chapter/BP/BP_C1_Caution_Earthing.Set Grab Attach 5-2-1 Enable` (`self.BP_C1_Caution_Earthing`))
  ;[1 0.04231 0] Instructions
  (`TrainingStepPage.AdvanceProgress` (`self.WBP_Step_Page`)))

(event `Sub 5-2-1`
  ;[1 1 1] SUB 5
  (`/Game/Test_Chapter/BP/BP_C1_Caution_Earthing.Set Grab Attach 5-2-1 Disable` (`self.BP_C1_Caution_Earthing`))
  ;[1 0.04231 0] Instructions
  (`TrainingStepPage.AdvanceProgress` (`self.WBP_Step_Page`)))

(event `Sub 6-1-1`
  ;[1 1 1] SUB 6
  (`/Game/Test_Chapter/BP/BP_C1_RMU_HVI.Disable 6-1-1` (`self.BP_C1_RMU_HVI`))
  (`/Game/Test_Chapter/BP/BP_C1_RMU_HVI.Disable Select` (`self.BP_C1_RMU_HVI`))
  (`/Game/Test_Chapter/BP/BP_C1_RMU_HVI.Set 6-1-2 Explain Visible` (`self.BP_C1_RMU_HVI`)))

(event `Step 6`
  ;[1 1 1] STEP 6
  (`/Game/Test_Chapter/BP/BP_C1_RMU_HVI.Enable Select` (`self.BP_C1_RMU_HVI`))
  (`/Game/Test_Chapter/BP/BP_C1_RMU_HVI.Enable 6-1-1` (`self.BP_C1_RMU_HVI`)))

(event `Sub 6-1-2`
  ;[1 1 1] SUB 6
  (`/Game/Test_Chapter/BP/BP_C1_RMU_HVI.Set 6-1-2 Explain Hidden` (`self.BP_C1_RMU_HVI`))
  ;[1 0.04231 0] Instructions
  (`TrainingStepPage.AdvanceProgress` (`self.WBP_Step_Page`)))

(event `Step 7`
  ;[1 1 1] STEP 7
  (`/Game/Test_Chapter/BP/BP_C1_Caution_Earthing.Enable Grab Remove` (`self.BP_C1_Caution_Earthing`)))

(event `Sub 7-1-1`
  ;[1 1 1] SUB 7
  (`/Game/Test_Chapter/BP/BP_C1_Caution_Earthing.Disable Grab Remove` (`self.BP_C1_Caution_Earthing`))
  (`KismetSystemLibrary.Delay` 0.5)
  (`/Game/Test_Chapter/BP/BP_C1_Earth_Switch_Knob.Enable Touch` (`self.BP_C1_Earth_Switch_Knob`))
  ;[1 0.04231 0] Instructions
  (`TrainingStepPage.AdvanceProgress` (`self.WBP_Step_Page`)))

(event `Sub 7-2-1`
  ;[1 1 1] SUB 7
  (`/Game/Test_Chapter/BP/BP_C1_Earth_Switch_Knob.Disable Touch` (`self.BP_C1_Earth_Switch_Knob`))
  (`/Game/Test_Chapter/BP/BP_C1_Earth_Switch_Knob.OpenKnob` (`self.BP_C1_Earth_Switch_Knob`))
  (`/Game/Test_Chapter/BP/BP_C1_OperatingHandle.Enable 7-3-1` (`self.BP_C1_OperatingHandle`))
  (`/Game/Test_Chapter/BP/BP_C1_OperatingHandle.Set Grab Attach 7-3-1 Enable` (`self.BP_C1_OperatingHandle`))
  ;[1 0.04231 0] Instructions
  (`TrainingStepPage.AdvanceProgress` (`self.WBP_Step_Page`)))

(event `Sub 7-3-1`
  ;[1 1 1] SUB 7
  (`/Game/Test_Chapter/BP/BP_C1_OperatingHandle.Set Grab Attach 7-3-1 Disable` (`self.BP_C1_OperatingHandle`))
  (`/Game/Test_Chapter/BP/BP_C1_OperatingHandle.Disable 7-3-1` (`self.BP_C1_OperatingHandle`))
  (`/Game/Test_Chapter/BP/BP_C1_OperatingHandle.Set Rotate Clock` (`self.BP_C1_OperatingHandle`))
  (`/Game/Test_Chapter/BP/BP_C1_OperatingHandle.Enable 7-4-1` (`self.BP_C1_OperatingHandle`))
  ;[1 0.04231 0] Instructions
  (`TrainingStepPage.AdvanceProgress` (`self.WBP_Step_Page`)))

(event `Sub 7-4-1`
  ;[1 1 1] SUB 7
  (`/Game/Test_Chapter/BP/BP_C1_OperatingHandle.Disable 7-4-1` (`self.BP_C1_OperatingHandle`))
  (`/Game/Test_Chapter/BP/BP_C1_OperatingHandle.Set Latch Disable` (`self.BP_C1_OperatingHandle`))
  (`/Game/Test_Chapter/BP/BP_C1_Earth_Switch_Knob.Set 7-4-2 Explain Visible` (`self.BP_C1_Earth_Switch_Knob`)))

(event `Sub 7-4-2`
  ;[1 1 1] SUB 7
  (`/Game/Test_Chapter/BP/BP_C1_Earth_Switch_Knob.Set 7-4-2 Explain Hidden` (`self.BP_C1_Earth_Switch_Knob`))
  (`/Game/Test_Chapter/BP/BP_C1_OperatingHandle.Enable Grab Remove` (`self.BP_C1_OperatingHandle`))
  (`/Game/Test_Chapter/BP/BP_C1_OperatingHandle.Enable 7-5-1` (`self.BP_C1_OperatingHandle`))
  ;[1 0.04231 0] Instructions
  (`TrainingStepPage.AdvanceProgress` (`self.WBP_Step_Page`)))

(event `Sub 7-5-1`
  ;[1 1 1] SUB 7
  (`/Game/Test_Chapter/BP/BP_C1_OperatingHandle.Disable Grab Remove` (`self.BP_C1_OperatingHandle`))
  (`/Game/Test_Chapter/BP/BP_C1_OperatingHandle.Disable 7-5-1` (`self.BP_C1_OperatingHandle`))
  (`/Game/Test_Chapter/BP/BP_C1_Earth_Switch_Knob.CloseKnob` (`self.BP_C1_Earth_Switch_Knob`))
  ;[1 0.04231 0] Instructions
  (`TrainingStepPage.AdvanceProgress` (`self.WBP_Step_Page`)))

(event `Step 8`
  ;[1 1 1] STEP 8
  (`/Game/Test_Chapter/BP/BP_C1_Caution_Earthing.Set Grab Attach 8-1-1 Enable` (`self.BP_C1_Caution_Earthing`)))

(event `Sub 8-1-1`
  ;[1 1 1] SUB 8
  (`/Game/Test_Chapter/BP/BP_C1_Caution_Earthing.Set Grab Attach 8-1-1 Disable` (`self.BP_C1_Caution_Earthing`))
  ;[1 0.04231 0] Instructions
  (`TrainingStepPage.AdvanceProgress` (`self.WBP_Step_Page`)))

(fn `UserConstructionScript`)
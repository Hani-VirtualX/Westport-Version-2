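; Chapter 1 ring main unit (RMU HVI) actor that serves as a touch and explanation target for steps 3, 4 and 6 of the chapter.
; External calls toggle touch, per-step flags and explain components, and can turn an LED panel material emissive blue.
; Touches on flagged steps and completed explanations each fire a one-shot substep call on the GM_C1 actor, cached shortly after BeginPlay.
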(event `self.ReceiveBeginPlay`
  (`KismetSystemLibrary.Delay` 0.2)
  (bind _returnvalue (`GameplayStatics.GetActorOfClass` "/Game/Test_Chapter/GM_C1.GM_C1_C"))
  (set `self.GM_C1` _returnvalue))

(event `Enable 3-1-1`
  (set `self.3-1-1` true))

(event `Disable 3-1-1`
  (set `self.3-1-1` false))

(event `Enable 4-5-1`
  (set `self.4-5-1` true))

(event `Disable 4-5-1`
  (set `self.4-5-1` false))

(event `Enable 6-1-1`
  (set `self.6-1-1` true))

(event `Disable 6-1-1`
  (set `self.6-1-1` false))

(event `Set 3-1-2 Explain Visible`
  (`Azr_Explain.EnableExplain` (`self.Azr_Explain_Step3`)))

(event `Set 3-1-2 Explain Hidden`
  (`Azr_Explain.DisableExplain` (`self.Azr_Explain_Step3`)))

(event `self.Azr_Explain_Step3.OnExplainCompleted`
  (`/Engine/EditorBlueprintResources/StandardMacros.DoOnce` false
    (:`Completed`
      (`/Game/Test_Chapter/GM_C1.Sub 3-1-2` (`self.GM_C1`)))))

(event `Light Up`
  (`PrimitiveComponent.SetMaterial` (`self.TNB_RingMainUnit_LEDPanel`) 2 "/Game/Props/RingMainUnit/Emissive_Blue.Emissive_Blue"))

(event `Set 4-5-2 Explain Visible`
  (`Azr_Explain.EnableExplain` (`self.Azr_Explain_Step4`)))

(event `Set 4-5-2 Explain Hidden`
  (`Azr_Explain.DisableExplain` (`self.Azr_Explain_Step4`)))

(event `self.Azr_Explain_Step4.OnExplainCompleted`
  (`/Engine/EditorBlueprintResources/StandardMacros.DoOnce` false
    (:`Completed`
      (`/Game/Test_Chapter/GM_C1.Sub 4-5-2` (`self.GM_C1`)))))

(event `Set 6-1-2 Explain Visible`
  (`Azr_Explain.EnableExplain` (`self.Azr_Explain_Step6`)))

(event `Set 6-1-2 Explain Hidden`
  (`Azr_Explain.DisableExplain` (`self.Azr_Explain_Step6`)))

(event `self.Azr_Explain_Step6.OnExplainCompleted`
  (`/Engine/EditorBlueprintResources/StandardMacros.DoOnce` false
    (:`Completed`
      (`/Game/Test_Chapter/GM_C1.Sub 6-1-2` (`self.GM_C1`)))))

(event `Enable Select`
  (`Azr_Touch.EnableTouch` (`self.Azr_Touch`)))

(event `Disable Select`
  (`Azr_Touch.DisableTouch` (`self.Azr_Touch`)))

(event `self.Azr_Touch.OnTouched`
  (`|ExecutionSequence`
    (:`then_0`
      (if (`self.3-1-1`)
        (`/Engine/EditorBlueprintResources/StandardMacros.DoOnce` false
          (:`Completed`
            (`/Game/Test_Chapter/GM_C1.Sub 3-1-1` (`self.GM_C1`))))))
    (:`then_1`
      (if (`self.4-5-1`)
        (`/Engine/EditorBlueprintResources/StandardMacros.DoOnce` false
          (:`Completed`
            (`/Game/Test_Chapter/GM_C1.Sub 4-5-1` (`self.GM_C1`))))))
    (:`then_2`
      (if (`self.6-1-1`)
        (`/Engine/EditorBlueprintResources/StandardMacros.DoOnce` false
          (:`Completed`
            (`/Game/Test_Chapter/GM_C1.Sub 6-1-1` (`self.GM_C1`))))))))

(fn `UserConstructionScript`)
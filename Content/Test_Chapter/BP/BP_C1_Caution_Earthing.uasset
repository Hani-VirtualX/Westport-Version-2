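; Chapter 1 "Caution Earthing" actor that uses an AzrGrab component to report grab attach and remove actions to the chapter's game mode.
; It caches GM_C1 shortly after BeginPlay and exposes events that toggle attaching for steps 5-2-1 and 8-1-1, plus removal.
; Attach callbacks branch on sequence ID to call Sub521 or Sub811, and removal calls Sub711, each guarded by a DoOnce.
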(event `self.ReceiveBeginPlay`
  (`KismetSystemLibrary.Delay` 0.2)
  (bind _returnvalue (`GameplayStatics.GetActorOfClass` "/Game/Test_Chapter/GM_C1.GM_C1_C"))
  (set `self.GM_C1` _returnvalue))

(event `Set Grab Attach 5-2-1 Enable`
  ; Grab Attach Enable/Disable
  (`Azr_Grab.EnableGrabAttach` (`self.Azr_Grab`) 1))

(event `Set Grab Attach 5-2-1 Disable`
  ; Grab Attach Enable/Disable
  (`Azr_Grab.DisableGrabAttach` (`self.Azr_Grab`)))

(event `Set Grab Attach 8-1-1 Disable`
  ; Grab Attach Enable/Disable
  (`Azr_Grab.DisableGrabAttach` (`self.Azr_Grab`)))

(event `Set Grab Attach 8-1-1 Enable`
  ; Grab Attach Enable/Disable
  (`Azr_Grab.EnableGrabAttach` (`self.Azr_Grab`) 2))

(event `Enable Grab Remove`
  (`Azr_Grab.EnableGrabRemove` (`self.Azr_Grab`)))

(event `Disable Grab Remove`
  (`Azr_Grab.DisableGrabRemove` (`self.Azr_Grab`) true))

(event `self.Azr_Grab.OnGrabAttached`
  (params (SequenceID :type Integer) (Target :type "Azr_AttachTarget Object Reference"))
  (switch `int` SequenceID
    (:`1`
      (`/Engine/EditorBlueprintResources/StandardMacros.DoOnce` false
        (:`Completed`
          (`/Game/Test_Chapter/GM_C1.Sub 5-2-1` (`self.GM_C1`)))))
    (:`2`
      (`/Engine/EditorBlueprintResources/StandardMacros.DoOnce` false
        (:`Completed`
          (`/Game/Test_Chapter/GM_C1.Sub 8-1-1` (`self.GM_C1`)))))))

(event `self.Azr_Grab.OnGrabRemoved`
  (`/Engine/EditorBlueprintResources/StandardMacros.DoOnce` false
    (:`Completed`
      (`/Game/Test_Chapter/GM_C1.Sub 7-1-1` (`self.GM_C1`)))))

(fn `UserConstructionScript`)
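; Sliding double door for the VCB room in Chapter 1, with an action component that the player triggers.
; Two timelines slide the leaves and play in reverse to close, with opposing door collision changes when they finish.
; The action's start press opens the door and its completed press calls Sub211 on GM_C1, each once.
; Other events toggle the action and teleport the player to a fixed RMU spot.
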(event `self.ReceiveBeginPlay`
  (`KismetSystemLibrary.Delay` 0.2)
  (bind _returnvalue (`GameplayStatics.GetActorOfClass` "/Game/Test_Chapter/GM_C1.GM_C1_C"))
  (set `self.GM_C1` _returnvalue))

(event `Door Open`
  (`|ExecutionSequence`
    (:`then_0`
      (bind (_direction _newtrack_0) (`Timeline|Timeline` :!label _label)
        (:`Update`
          (`SceneComponent.K2_SetRelativeLocation` (`self.RightDoor`) (`KismetMathLibrary.MakeVector` (.x _newtrack_0) 0.0 7.0) false false))
        (:`Finished`
          (`PrimitiveComponent.SetCollisionEnabled` (`self.LeftDoor`) "NoCollision")
          (`PrimitiveComponent.SetCollisionEnabled` (`self.RightDoor`) "NoCollision"))))
    (:`then_1`
      (bind (_direction_2 _newtrack_0_2) (`Timeline|Timeline_0` :!label _label_2)
        (:`Update`
          (`SceneComponent.K2_SetRelativeLocation` (`self.LeftDoor`) (`KismetMathLibrary.MakeVector` (.x _newtrack_0_2) 0.0 -1.0) false false))
        (:`Finished`
          (`PrimitiveComponent.SetCollisionEnabled` (`self.LeftDoor`) "QueryAndPhysics")
          (`PrimitiveComponent.SetCollisionEnabled` (`self.RightDoor`) "QueryAndPhysics"))))))

(event `Close Door`
  (`|ExecutionSequence`
    (:`then_0`
      (goto _label :!via `Reverse`))
    (:`then_1`
      (goto _label_2 :!via `Reverse`))))

(event `Teleport To RMU`
  (bind _returnvalue (`GameplayStatics.GetPlayerPawn` 0))
  (bind (_returnvalue_x _returnvalue_y _returnvalue_z) (`KismetMathLibrary.BreakVector` (`self.K2_GetActorLocation` _returnvalue)))
  (`self.K2_SetActorLocation` _returnvalue (`KismetMathLibrary.MakeVector` 370.0 -610.0 _returnvalue_z) false true))

(event `Set 2-1 Action Visible`
  (`Azr_Action.EnableAction` (`self.Azr_Action`)))

(event `Set 2-1 Action Hidden`
  (`Azr_Action.DisableAction` (`self.Azr_Action`)))

(event `self.Azr_Action.OnCompletedButtonPressed`
  (`/Engine/EditorBlueprintResources/StandardMacros.DoOnce` false
    (:`Completed`
      (`/Game/Test_Chapter/GM_C1.Sub 2-1-1` (`self.GM_C1`)))))

(event `self.Azr_Action.OnStartButtonPressed`
  (`/Engine/EditorBlueprintResources/StandardMacros.DoOnce` false
    (:`Completed`
      (`self.Door Open`))))

(fn `UserConstructionScript`)
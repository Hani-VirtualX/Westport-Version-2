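; Earth switch knob actor for Chapter 1 that can be touched, explained and animated open or closed.
; Open and Close timelines rotate the PlugHole's yaw, while other events toggle the AzrTouch and AzrExplain components.
; Touch and explanation completion each pass through a DoOnce to call Sub721 and Sub742 respectively on GM_C1, which is cached shortly after BeginPlay.
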(event `self.ReceiveBeginPlay`
  (`KismetSystemLibrary.Delay` 0.2)
  (bind _returnvalue (`GameplayStatics.GetActorOfClass` "/Game/Test_Chapter/GM_C1.GM_C1_C"))
  (set `self.GM_C1` _returnvalue))

(event `Enable Touch`
  (`Azr_Touch.EnableTouch` (`self.Azr_Touch`)))

(event `Disable Touch`
  (`Azr_Touch.DisableTouch` (`self.Azr_Touch`)))

(event `OpenKnob`
  (bind (_direction _open) (`Timeline|Open` :!via `PlayFromStart`)
    (:`Update`
      (`SceneComponent.K2_SetRelativeRotation` (`self.PlugHole`) (`KismetMathLibrary.MakeRotator` 0.0 0.0 _open) false false))))

(event `self.Azr_Touch.OnTouched`
  (`/Engine/EditorBlueprintResources/StandardMacros.DoOnce` false
    (:`Completed`
      (`/Game/Test_Chapter/GM_C1.Sub 7-2-1` (`self.GM_C1`)))))

(event `CloseKnob`
  (bind (_direction _close) (`Timeline|Close` :!via `PlayFromStart`)
    (:`Update`
      (`SceneComponent.K2_SetRelativeRotation` (`self.PlugHole`) (`KismetMathLibrary.MakeRotator` 0.0 0.0 _close) false false))))

(event `Set 7-4-2 Explain Visible`
  (`Azr_Explain.EnableExplain` (`self.Azr_Explain`)))

(event `Set 7-4-2 Explain Hidden`
  (`Azr_Explain.DisableExplain` (`self.Azr_Explain`)))

(event `self.Azr_Explain.OnExplainCompleted`
  (`/Engine/EditorBlueprintResources/StandardMacros.DoOnce` false
    (:`Completed`
      (`/Game/Test_Chapter/GM_C1.Sub 7-4-2` (`self.GM_C1`)))))

(fn `UserConstructionScript`)
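; BP_C1_Step1_Widg is a chapter 1, step 1 actor that controls an explanation component or widget and advances the chapter flow when it completes.
; On BeginPlay it waits briefly, then finds and caches the GM_C1 actor.
; Custom events enable and disable the AzrExplain explanation.
; When the explanation completes, a DoOnce guard calls Sub111 on GM_C1 a single time.
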(event `self.ReceiveBeginPlay`
  (`KismetSystemLibrary.Delay` 0.2)
  (bind _returnvalue (`GameplayStatics.GetActorOfClass` "/Game/Test_Chapter/GM_C1.GM_C1_C"))
  (set `self.GM_C1` _returnvalue))

(event `Set 1-1-1 Explain Enable`
  (`Azr_Explain.EnableExplain` (`self.Azr_Explain`)))

(event `Set 1-1-1 Explain Disable`
  (`Azr_Explain.DisableExplain` (`self.Azr_Explain`)))

(event `self.Azr_Explain.OnExplainCompleted`
  (`/Engine/EditorBlueprintResources/StandardMacros.DoOnce` false
    (:`Completed`
      (`/Game/Test_Chapter/GM_C1.Sub 1-1-1` (`self.GM_C1`)))))

(fn `UserConstructionScript`)
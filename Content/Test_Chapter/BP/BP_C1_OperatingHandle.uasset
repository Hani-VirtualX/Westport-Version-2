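; BP_C1_OperatingHandle is a Chapter 1 handle actor that can be grabbed, attached, removed and rotated to advance numbered steps in GM_C1.
; External events arm step flags and toggle its AzrGrab attach/remove and AzrLatch rotation.
; Grab and latch callbacks call the matching GM_C1 Sub functions, with attach steps firing once.
; Step 4-3-1 waits for full latch travel, while 7-4-1 fires on any value change.
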(event `self.ReceiveBeginPlay`
  (`KismetSystemLibrary.Delay` 0.2)
  (bind _returnvalue (`GameplayStatics.GetActorOfClass` "/Game/Test_Chapter/GM_C1.GM_C1_C"))
  (set `self.GM_C1` _returnvalue))

(event `Enable 4-2-1`
  (set `self.4-2-1` true))

(event `Disable 4-2-1`
  (set `self.4-2-1` false))

(event `Enable 4-3-1`
  (set `self.4-3-1` true))

(event `Disable 4-3-1`
  (set `self.4-3-1` false))

(event `Set Rotate Clock`
  (`KismetSystemLibrary.PrintString` "LATCH")
  (`Azr_Latch.SetLatchConfig` (`self.Azr_Latch`) "Rotation" "X_Axis" 0.0 -180.0 0.0)
  (`Azr_Latch.EnableLatch` (`self.Azr_Latch`)))

(event `Set Grab Attach 4-2-1 Enable`
  ;[1 1 1 0.5] Grab Attach Enable/Disable
  (`Azr_Grab.EnableGrabAttach` (`self.Azr_Grab`) 1))

(event `Set Grab Attach 4-2-1 Disable`
  ;[1 1 1 0.5] Grab Attach Enable/Disable
  (`Azr_Grab.DisableGrabAttach` (`self.Azr_Grab`)))

(event `Enable 4-4-1`
  (set `self.4-4-1` true))

(event `Disable 4-4-1`
  (set `self.4-4-1` false))

(event `Enable 7-3-1`
  (set `self.7-3-1` true))

(event `Disable 7-3-1`
  (set `self.7-3-1` false))

(event `Set Grab Attach 7-3-1 Enable`
  ;[1 1 1 0.5] Grab Attach Enable/Disable
  (`Azr_Grab.EnableGrabAttach` (`self.Azr_Grab`) 2))

(event `Set Grab Attach 7-3-1 Disable`
  ;[1 1 1 0.5] Grab Attach Enable/Disable
  (`Azr_Grab.DisableGrabAttach` (`self.Azr_Grab`)))

(event `Enable 7-4-1`
  (set `self.7-4-1` true))

(event `Disable 7-4-1`
  (set `self.7-4-1` false))

(event `Enable 7-5-1`
  (set `self.7-5-1` true))

(event `Disable 7-5-1`
  (set `self.7-5-1` false))

(event `Enable Grab Remove`
  (`Azr_Grab.EnableGrabRemove` (`self.Azr_Grab`)))

(event `Disable Grab Remove`
  (`Azr_Grab.DisableGrabRemove` (`self.Azr_Grab`) true))

(event `Set Latch Enable`
  (`Azr_Latch.EnableLatch` (`self.Azr_Latch`)))

(event `Set Latch Disable`
  (`Azr_Latch.DisableLatch` (`self.Azr_Latch`)))

(event `self.Azr_Grab.OnGrabRemoved`
  ; Grab Event
  (`|ExecutionSequence`
    (:`then_0`
      (if (`self.4-4-1`)
        (`/Game/Test_Chapter/GM_C1.Sub 4-4-1` (`self.GM_C1`))))
    (:`then_1`
      (if (`self.7-5-1`)
        (`/Game/Test_Chapter/GM_C1.Sub 7-5-1` (`self.GM_C1`))))))

(event `self.Azr_Grab.OnGrabAttached`
  (params (SequenceID :type Integer) (Target :type "Azr_AttachTarget Object Reference"))
  ; Grab Event
  (switch `int` SequenceID
    (:`1`
      (`/Engine/EditorBlueprintResources/StandardMacros.DoOnce` false
        (:`Completed`
          (`/Game/Test_Chapter/GM_C1.Sub 4-2-1` (`self.GM_C1`)))))
    (:`2`
      (`/Engine/EditorBlueprintResources/StandardMacros.DoOnce` false
        (:`Completed`
          (`/Game/Test_Chapter/GM_C1.Sub 7-3-1` (`self.GM_C1`)))))))

(event `self.Azr_Latch.OnValueChanged`
  (params (Value :type "Float (single-precision)"))
  (`|ExecutionSequence`
    (:`then_0`
      (if (`self.4-3-1`)
        (if (>= Value 1.0)
          (`/Game/Test_Chapter/GM_C1.Sub 4-3-1` (`self.GM_C1`)))))
    (:`then_1`
      (if (`self.7-4-1`)
        (if true
          (`/Game/Test_Chapter/GM_C1.Sub 7-4-1` (`self.GM_C1`))
          (`KismetSystemLibrary.PrintString` "DONE LATCH"))))))

(event `self.ReceiveTick`
  (params (DeltaSeconds :type "Float (single-precision)")))

(fn `UserConstructionScript`)